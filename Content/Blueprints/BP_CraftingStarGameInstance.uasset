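; Game instance for Crafting Star that handles host/guest session hosting and single-slot save data.
; Hosting creates an Advanced Session and opens MatchingMenu as a listen server; accepted invites join it, and network errors are printed.
; Save copies both players' PlayerState data and GameState progress into BP_SaveGame.
; Load restores player data and positions, then passes map and progress to the GameMode and calls InitGame; helpers check or create saves.
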(event Custom|Host
  (params (PlayerController :type Player%20Controller%20Object%20Reference))
  (|AdvancedSession 0 PlayerController 100 100 false true false true true true false false false true
    (:then
      (Development|PrintString "Host Create Session")
      (Game|OpenLevel(byName) "MatchingMenu" true "listen"))))

(event EventHandleNetworkError
  (params (FailureType :type ENetworkFailure%20Enum :default "NetDriverAlreadyExists") (bIsServer :type Boolean))
  (Development|PrintString (Utilities|String|EnumtoString FailureType)))

(event EventOnSessionInviteAccepted
  (params (LocalPlayerNum :type Integer) (PersonInvited :type BP%20Unique%20Net%20Id%20Structure) (SessionToJoin :type Blueprint%20Session%20Result%20Structure%20%28by%20ref%29))
  (|JoinSession (Game|GetPlayerController 0) SessionToJoin))

(event EventOnSessionInviteReceived
  (params (LocalPlayerNum :type Integer) (PersonInviting :type BP%20Unique%20Net%20Id%20Structure) (AppId :type String) (SessionToJoin :type Blueprint%20Session%20Result%20Structure%20%28by%20ref%29)))

(fn Save
  (bind _returnvalue (Game|GetGameState))
  (Utilities|IsValid (Variables|Default|GetSaveGame)
    (:Is%20Valid
      ;[1 1 1] 기존 게임 데이터 저장
      (for _array_element (Variables|/Script/Engine.GameStateBase|GetPlayerArray _returnvalue)
        (bind _returnvalue_2 (Class|UtilityFunction|IsHost (.AsController (Utilities|Casting|CastToController (Components|GetOwner _array_element)))))
        (if _returnvalue_2
          (Variables|/Game/Blueprints/InGameMenu/SaveSystem/BP_SaveGame.BP_SaveGame_C|SetHostData (Variables|Default|GetSaveGame) (Variables|/Script/CraftingStar.CraftingStarPS|GetPlayerData (.AsCrafting%20Star%20PS (Utilities|Casting|CastToCraftingStarPS _array_element))))
          (Variables|/Game/Blueprints/InGameMenu/SaveSystem/BP_SaveGame.BP_SaveGame_C|SetProgressData (Variables|Default|GetSaveGame) (Variables|/Script/CraftingStar.CraftingStarGS|GetProgressData (.AsCrafting%20Star%20GS (Utilities|Casting|CastToCraftingStarGS _returnvalue))))
          (else
            (Variables|/Game/Blueprints/InGameMenu/SaveSystem/BP_SaveGame.BP_SaveGame_C|SetGuestData (Variables|Default|GetSaveGame) (Variables|/Script/CraftingStar.CraftingStarPS|GetPlayerData (.AsCrafting%20Star%20PS (Utilities|Casting|CastToCraftingStarPS _array_element))))))))
    (:Is%20Not%20Valid
      ;[1 1 1] 새 게임 데이터 생성
      (bind _returnvalue_3 (SaveGame|CreateSaveGameObject "/Game/Blueprints/InGameMenu/SaveSystem/BP_SaveGame.BP_SaveGame_C"))
      (bind _output_get (Variables|Default|SetSaveGame _returnvalue_3))
      (Variables|/Game/Blueprints/InGameMenu/SaveSystem/BP_SaveGame.BP_SaveGame_C|SetHostData _output_get (Utilities|Struct|MakePlayerData "EDark"))
      (Variables|/Game/Blueprints/InGameMenu/SaveSystem/BP_SaveGame.BP_SaveGame_C|SetGuestData _output_get (Utilities|Struct|MakePlayerData "EDark"))))
  (SaveGame|SaveGametoSlot (Variables|Default|GetSaveGame) "CraftingStarGame")
  ;[1 1 1] 디버그
  (Development|PrintString (Utilities|String|ToString(Text) (Utilities|Text|FormatText (Utilities|Text|ToText(String) (.PlayerName (Utilities|Struct|BreakPlayerData (Variables|/Game/Blueprints/InGameMenu/SaveSystem/BP_SaveGame.BP_SaveGame_C|GetHostData (Variables|Default|GetSaveGame))))))))
  (Development|PrintString (Utilities|String|ToString(Text) (Utilities|Text|FormatText (Utilities|Text|ToText(String) (.PlayerName (Utilities|Struct|BreakPlayerData (Variables|/Game/Blueprints/InGameMenu/SaveSystem/BP_SaveGame.BP_SaveGame_C|GetGuestData (Variables|Default|GetSaveGame)))))))))

(fn Load
  (bind _returnvalue (Game|GetGameMode))
  (bind _ascrafting_star_game_mode (Utilities|Casting|CastToCraftingStarGameMode _returnvalue))
  (bind _returnvalue_2 (SaveGame|LoadGamefromSlot "CraftingStarGame"))
  (bind _asbp_save_game (Utilities|Casting|CastToBP_SaveGame _returnvalue_2))
  (for _array_element (Variables|/Script/Engine.GameStateBase|GetPlayerArray (Game|GetGameState))
    (bind _returnvalue_3 (Class|UtilityFunction|IsHost (.AsController (Utilities|Casting|CastToController (Components|GetOwner _array_element)))))
    (if _returnvalue_3
      ;[1 1 1] Host/Guest 구분에 따라 달라지는 Load 로직
      (Transformation|SetWorldTransform (Variables|/Script/Engine.Character|GetCapsuleComponent (.AsCrafting%20Star%20Character (Utilities|Casting|CastToCraftingStarCharacter (Pawn|GetControlledPawn (.AsController (Utilities|Casting|CastToController (Components|GetOwner _array_element))))))) (.HostPlayerPos (Utilities|Struct|BreakProgressData (Variables|/Game/Blueprints/InGameMenu/SaveSystem/BP_SaveGame.BP_SaveGame_C|GetProgressData _asbp_save_game))) false false)
      (Variables|/Script/CraftingStar.CraftingStarPS|SetPlayerData (.AsCrafting%20Star%20PS (Utilities|Casting|CastToCraftingStarPS _array_element)) (Variables|/Game/Blueprints/InGameMenu/SaveSystem/BP_SaveGame.BP_SaveGame_C|GetHostData _asbp_save_game))
      (else
        (Transformation|SetWorldTransform (Variables|/Script/Engine.Character|GetCapsuleComponent (.AsCrafting%20Star%20Character (Utilities|Casting|CastToCraftingStarCharacter (Pawn|GetControlledPawn (.AsController (Utilities|Casting|CastToController (Components|GetOwner _array_element))))))) (.GuestPlayerPos (Utilities|Struct|BreakProgressData (Variables|/Game/Blueprints/InGameMenu/SaveSystem/BP_SaveGame.BP_SaveGame_C|GetProgressData _asbp_save_game))) false false)
        (Variables|/Script/CraftingStar.CraftingStarPS|SetPlayerData (.AsCrafting%20Star%20PS (Utilities|Casting|CastToCraftingStarPS _array_element)) (Variables|/Game/Blueprints/InGameMenu/SaveSystem/BP_SaveGame.BP_SaveGame_C|GetGuestData _asbp_save_game)))))
  (Variables|/Script/CraftingStar.CraftingStarGameMode|SetNowMapName _ascrafting_star_game_mode (.NowMapName (Utilities|Struct|BreakProgressData (Variables|/Game/Blueprints/InGameMenu/SaveSystem/BP_SaveGame.BP_SaveGame_C|GetProgressData _asbp_save_game))))
  (Variables|/Script/CraftingStar.CraftingStarGameMode|SetProgressLevel _ascrafting_star_game_mode (.ProgressLevel (Utilities|Struct|BreakProgressData (Variables|/Game/Blueprints/InGameMenu/SaveSystem/BP_SaveGame.BP_SaveGame_C|GetProgressData _asbp_save_game))))
  (Development|PrintString "Hello")
  (Class|CraftingStarGameMode|InitGame _ascrafting_star_game_mode))

(fn CheckSaveData
  (bind _returnvalue (SaveGame|LoadGamefromSlot "CraftingStarGame"))
  (if (.bSuccess (Utilities|Casting|CastToBP_SaveGame _returnvalue))
    (Variables|Default|SetSaveGame (.AsBP%20Save%20Game (Utilities|Casting|CastToBP_SaveGame _returnvalue))))
  (return (.bSuccess (Utilities|Casting|CastToBP_SaveGame _returnvalue))))

(fn CreateSaveData
  (params (ServerMode :type EPlayerRole%20Enum :default "EDark") (ClientMode :type EPlayerRole%20Enum :default "EDark"))
  (bind _returnvalue (SaveGame|CreateSaveGameObject "/Game/Blueprints/InGameMenu/SaveSystem/BP_SaveGame.BP_SaveGame_C"))
  (bind _output_get (Variables|Default|SetSaveGame _returnvalue))
  ;[1 1 1] 초기 데이터 생성
  (Variables|/Game/Blueprints/InGameMenu/SaveSystem/BP_SaveGame.BP_SaveGame_C|SetHostData _output_get (Utilities|Struct|MakePlayerData ServerMode "" (LocalVariables|GetInitAbilityArray)))
  (Variables|/Game/Blueprints/InGameMenu/SaveSystem/BP_SaveGame.BP_SaveGame_C|SetGuestData _output_get (Utilities|Struct|MakePlayerData ClientMode "" (LocalVariables|GetInitAbilityArray)))
  (Variables|/Game/Blueprints/InGameMenu/SaveSystem/BP_SaveGame.BP_SaveGame_C|SetProgressData _output_get (Utilities|Struct|MakeProgressData "EKeyStar" (Math|Transform|MakeTransform "250.000000,30.000000,90.000000" "0,180.000000, 0") (Math|Transform|MakeTransform "210.000000,30.000000,90.000000" "0,180.000000, 0")))
  (SaveGame|SaveGametoSlot _output_get "CraftingStarGame"))