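; BP_FireBowl_Obj is an interactable fire bowl puzzle object that opens two fences once fully lit.
; OnPerformed plays and OffPerformed reverses the TurnLight timeline, which drives Fade Amount on a dynamic fire material.
; Passing a playback threshold sets IsClear, blocking further toggling, and starts the OpenFense timeline.
; That timeline moves both fence meshes by additive relative offsets on each update.
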(event OnComponentBeginOverlap(Box)
  (params (OverlappedComponent :type Primitive%20Component%20Object%20Reference) (OtherActor :type Actor%20Object%20Reference) (OtherComp :type Primitive%20Component%20Object%20Reference) (OtherBodyIndex :type Integer) (bFromSweep :type Boolean) (SweepResult :type Hit%20Result%20Structure%20%28by%20ref%29)))

(event OnComponentEndOverlap(Box)
  (params (OverlappedComponent :type Primitive%20Component%20Object%20Reference) (OtherActor :type Actor%20Object%20Reference) (OtherComp :type Primitive%20Component%20Object%20Reference) (OtherBodyIndex :type Integer)))

(event Custom|OnLight
  (if (not (Variables|Default|GetisClear?))
    (bind _새_트랙_0 (Timeline|TurnLight Play)
      (:Update
        (Rendering|Material|SetScalarParameterValue (Variables|Default|GetMaterial%20Instance) "Fade Amount" _새_트랙_0 :!class /Script/Engine.MaterialInstanceDynamic)
        (if (> (Components|Timeline|GetPlaybackPosition (Variables|Default|GetTurnLight)) 2.8)
          (Variables|Default|SetisClear? true)
          (bind _새_트랙_0_2 (Timeline|OpenFense Play)
            (:Update
              (Transformation|AddRelativeLocation (Variables|/Script/Engine.StaticMeshActor|GetStaticMeshComponent (Variables|Default|Getfense_1)) _새_트랙_0_2 false false))))))))

(event Custom|OffLight
  (if (not (Variables|Default|GetisClear?))
    (bind _새_트랙_0 (Timeline|TurnLight Reverse)
      (:Update
        (Rendering|Material|SetScalarParameterValue (Variables|Default|GetMaterial%20Instance) "Fade Amount" _새_트랙_0 :!class /Script/Engine.MaterialInstanceDynamic)
        (if (> (Components|Timeline|GetPlaybackPosition (Variables|Default|GetTurnLight)) 2.8)
          (Variables|Default|SetisClear? true)
          (bind _새_트랙_0_2 (Timeline|OpenFense Play)
            (:Update
              (Transformation|AddRelativeLocation (Variables|/Script/Engine.StaticMeshActor|GetStaticMeshComponent (Variables|Default|Getfense_1)) _새_트랙_0_2 false false))))))))

(event Collision|EventActorBeginOverlap
  (params (OtherActor :type Actor%20Object%20Reference)))

(event EventBeginPlay
  (bind _returnvalue (Rendering|Material|CreateDynamicMaterialInstance (Variables|Default|GetFire) 0 (Variables|Default|GetMaterial) "None" :!class /Script/Engine.PrimitiveComponent))
  (bind _output_get (Variables|Default|SetMaterial%20Instance _returnvalue))
  (Rendering|Material|SetScalarParameterValue _output_get "Fade Amount" 1.0 :!class /Script/Engine.MaterialInstanceDynamic))

(fn ConstructionScript)

(fn OnPerformed
  (CallFunction|OnLight))

(fn OffPerformed
  (CallFunction|OffLight))