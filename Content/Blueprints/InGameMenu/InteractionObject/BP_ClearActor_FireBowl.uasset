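; BP_ClearActor_FireBowl is a puzzle-clear actor that moves two fences, Fense1 and Fense2, once both the LightClear and DarkClear flags are true.
; Tick polls the flags, and a DoOnce lets the first success print "Clear" and start a timeline.
; Each timeline update adds the track's value to both fence meshes' relative location without sweep, so the offset accumulates per frame.
; Nothing in this graph sets the flags.
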(event EventBeginPlay)

(event Collision|EventActorBeginOverlap
  (params (OtherActor :type Actor%20Object%20Reference)))

(event EventTick
  (params (DeltaSeconds :type Float%20%28single-precision%29))
  (if (and (Variables|Default|GetLightClear) (Variables|Default|GetDarkClear))
    (Utilities|FlowControl|DoOnce false
      (:Completed
        (Development|PrintString "Clear")
        (bind _새_트랙_0 (Timeline|타임라인_0 Play)
          (:Update
            (Transformation|AddRelativeLocation (Variables|/Script/Engine.StaticMeshActor|GetStaticMeshComponent (Variables|Default|Getfense_1)) _새_트랙_0 false false)))))))

(fn ConstructionScript)