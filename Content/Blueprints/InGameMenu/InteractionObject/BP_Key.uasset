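; BP_Key is a collectible key pickup that counts toward level progression in CraftingStar.
; A Bounce timeline animates the mesh around the world location it had at BeginPlay.
; When a CraftingStarCharacter overlaps the box, the authority increments KeyNum on the game state and destroys the key.
; The fourth key also raises the progress level through UpdateProgressLevel, with debug prints reporting either count or level.
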(event OnComponentBeginOverlap(Box)
  (params (OverlappedComponent :type Primitive%20Component%20Object%20Reference) (OtherActor :type Actor%20Object%20Reference) (OtherComp :type Primitive%20Component%20Object%20Reference) (OtherBodyIndex :type Integer) (bFromSweep :type Boolean) (SweepResult :type Hit%20Result%20Structure%20%28by%20ref%29))
  (Networking|SwitchHasAuthority
    (:Authority
      (Utilities|Casting|CastToCraftingStarCharacter OtherActor)
      (bind _ascrafting_star_gs (Utilities|Casting|CastToCraftingStarGS (Game|GetGameState)))
      (if (== (Variables|/Script/CraftingStar.CraftingStarGS|GetKeyNum _ascrafting_star_gs) 3)
        (Variables|/Script/CraftingStar.CraftingStarGS|SetKeyNum _ascrafting_star_gs (+ (Variables|/Script/CraftingStar.CraftingStarGS|GetKeyNum _ascrafting_star_gs) 1))
        (Class|CraftingStarGS|UpdateProgressLevel _ascrafting_star_gs (+ (.ProgressLevel (Utilities|Struct|BreakProgressData (Variables|/Script/CraftingStar.CraftingStarGS|GetProgressData _ascrafting_star_gs))) 1))
        (Development|PrintString (Utilities|String|Append "Progress Level Update :" (Utilities|String|ToString(Integer) (.ProgressLevel (Utilities|Struct|BreakProgressData (Variables|/Script/CraftingStar.CraftingStarGS|GetProgressData _ascrafting_star_gs))))))
        (Actor|DestroyActor)
        (else
          (bind _output_get (Variables|/Script/CraftingStar.CraftingStarGS|SetKeyNum _ascrafting_star_gs (+ (Variables|/Script/CraftingStar.CraftingStarGS|GetKeyNum _ascrafting_star_gs) 1)))
          (Development|PrintString (Utilities|String|Append "Now Key Num :" (Utilities|String|ToString(Integer) _output_get)))
          (Actor|DestroyActor))))))

(event EventBeginPlay
  (bind _staticmeshcomponent (Variables|Debug|GetStaticMeshComponent))
  (Variables|Default|SetBeginOffset (Transformation|GetWorldLocation _staticmeshcomponent))
  (bind _새_트랙_0 (Timeline|Bounce Play)
    (:Update
      (Transformation|SetWorldLocation _staticmeshcomponent (+ _새_트랙_0 (Variables|Default|GetBeginOffset)) false false))))

(event Collision|EventActorBeginOverlap
  (params (OtherActor :type Actor%20Object%20Reference)))

(event EventTick
  (params (DeltaSeconds :type Float%20%28single-precision%29)))

(fn ConstructionScript)