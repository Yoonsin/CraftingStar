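; Game instance Blueprint that saves and restores host and guest player data in a single "GrabGame" slot.
; Save copies PlayerData from the player states of characters 0 and 1 into a BP_SaveGame and writes it.
; Load walks the game state's PlayerArray, treats the local authority controller as host, and passes the matching data to each GrabTestCharacter.
; CheckSaveData reports whether a valid save exists and caches it.
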(fn Save
  (Utilities|IsValid (Variables|Default|GetSaveGame)
    (:Is%20Valid
      _)
    (:Is%20Not%20Valid
      (bind _returnvalue (SaveGame|CreateSaveGameObject "/Game/ThirdPersonCPP/Blueprints/SaveSystem/BP_SaveGame.BP_SaveGame_C"))
      (bind _output_get (Variables|Default|SetSaveGame _returnvalue))))
  (bind _output_get_2 (Variables|/Game/ThirdPersonCPP/Blueprints/SaveSystem/BP_SaveGame.BP_SaveGame_C|SetHostData _output_get (Variables|/Game/ThirdPersonCPP/Blueprints/Player/BP_PlayerState.BP_PlayerState_C|GetPlayerData (.AsBP%20Player%20State (Utilities|Casting|CastToBP_PlayerState (Variables|/Script/Engine.Pawn|GetPlayerState (Game|GetPlayerCharacter 0)))))))
  (bind _output_get_3 (Variables|/Game/ThirdPersonCPP/Blueprints/SaveSystem/BP_SaveGame.BP_SaveGame_C|SetGuestData _output_get (Variables|/Game/ThirdPersonCPP/Blueprints/Player/BP_PlayerState.BP_PlayerState_C|GetPlayerData (.AsBP%20Player%20State (Utilities|Casting|CastToBP_PlayerState (Variables|/Script/Engine.Pawn|GetPlayerState (Game|GetPlayerCharacter 1)))))))
  (SaveGame|SaveGametoSlot _output_get "GrabGame")
  (Development|PrintString (Utilities|String|ToString(Text) (Utilities|Text|FormatText "Guest transporm {t} name {n} mode {m}" (Utilities|String|ToString(Transform) (.Pos (Utilities|Struct|BreakPlayerData _output_get_3))) (.PlayerName (Utilities|Struct|BreakPlayerData _output_get_3)) (Utilities|String|EnumtoString (.Mode (Utilities|Struct|BreakPlayerData _output_get_3))))))
  (Development|PrintString (Utilities|String|ToString(Text) (Utilities|Text|FormatText "Host transporm {t} name {n} mode {m}" (Utilities|String|ToString(Transform) (.Pos (Utilities|Struct|BreakPlayerData _output_get_2))) (.PlayerName (Utilities|Struct|BreakPlayerData _output_get_2)) (Utilities|String|EnumtoString (.Mode (Utilities|Struct|BreakPlayerData _output_get_2)))))))

(fn Load
  (bind _returnvalue (SaveGame|LoadGamefromSlot "GrabGame"))
  (bind _asbp_save_game (Utilities|Casting|CastToBP_SaveGame _returnvalue))
  (for _array_element (Variables|/Script/Engine.GameStateBase|GetPlayerArray (.AsBP%20Game%20State (Utilities|Casting|CastToBP_GameState (Game|GetGameState))))
    (bind _ishost (CallFunction|IsHost (.AsBP%20Player%20Controller (Utilities|Casting|CastToBP_PlayerController (Components|GetOwner _array_element)))))
    (if _ishost
      (Default|Load (.AsGrab%20Test%20Character (Utilities|Casting|CastToGrabTestCharacter (Pawn|GetControlledPawn (.AsBP%20Player%20Controller (Utilities|Casting|CastToBP_PlayerController (Components|GetOwner _array_element)))))) (Variables|/Game/ThirdPersonCPP/Blueprints/SaveSystem/BP_SaveGame.BP_SaveGame_C|GetHostData _asbp_save_game))
      (Development|PrintString (Utilities|String|ToString(Text) (Utilities|Text|FormatText "HOST transporm {t} name {n} mode {m}" (Utilities|String|ToString(Transform) (.Pos (Utilities|Struct|BreakPlayerData (Variables|/Game/ThirdPersonCPP/Blueprints/SaveSystem/BP_SaveGame.BP_SaveGame_C|GetHostData _asbp_save_game)))) (.PlayerName (Utilities|Struct|BreakPlayerData (Variables|/Game/ThirdPersonCPP/Blueprints/SaveSystem/BP_SaveGame.BP_SaveGame_C|GetHostData _asbp_save_game))))))
      (else
        (Default|Load (.AsGrab%20Test%20Character (Utilities|Casting|CastToGrabTestCharacter (Pawn|GetControlledPawn (.AsBP%20Player%20Controller (Utilities|Casting|CastToBP_PlayerController (Components|GetOwner _array_element)))))) (Variables|/Game/ThirdPersonCPP/Blueprints/SaveSystem/BP_SaveGame.BP_SaveGame_C|GetGuestData _asbp_save_game))
        (Development|PrintString (Utilities|String|ToString(Text) (Utilities|Text|FormatText "GUEST transporm {t} name {n} mode {m}" (Utilities|String|ToString(Transform) (.Pos (Utilities|Struct|BreakPlayerData (Variables|/Game/ThirdPersonCPP/Blueprints/SaveSystem/BP_SaveGame.BP_SaveGame_C|GetGuestData _asbp_save_game)))) (.PlayerName (Utilities|Struct|BreakPlayerData (Variables|/Game/ThirdPersonCPP/Blueprints/SaveSystem/BP_SaveGame.BP_SaveGame_C|GetGuestData _asbp_save_game))))))))))

(fn IsHost
  (params (Controller :type Controller%20Object%20Reference))
  (return (and (Pawn|IsLocalPlayerController Controller) (Ability|HasAuthority Controller))))

(fn CheckSaveData
  (bind _returnvalue (SaveGame|LoadGamefromSlot "GrabGame"))
  (if (.bSuccess (Utilities|Casting|CastToBP_SaveGame _returnvalue))
    (Variables|Default|SetSaveGame (.AsBP%20Save%20Game (Utilities|Casting|CastToBP_SaveGame _returnvalue))))
  (return (.bSuccess (Utilities|Casting|CastToBP_SaveGame _returnvalue))))