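; BP_CraftingStarPS, apparently the CraftingStar player state, holds a player's transform for save data.
; UpdateSaveData copies the given character's capsule world transform into Transform, whose RepNotify is an empty stub.
; PlayerData assignment and a debug print of player name and mode are disconnected and never run.
; BeginPlay, Tick and the construction script contain no logic.
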(event EventBeginPlay)

(event EventTick
  (params (DeltaSeconds :type Float%20%28single-precision%29)))

(fn ConstructionScript)

(fn UpdateSaveData
  (params (playerCharacter :type BP%20Crafting%20Star%20Character%20Object%20Reference))
  (bind _output_get (Variables|Default|SetTransform (Transformation|GetWorldTransform (Variables|/Script/Engine.Character|GetCapsuleComponent playerCharacter)))))

(fn OnRepTransform)