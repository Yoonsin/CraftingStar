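; Game state for the two-player CraftingStar game, coordinating cutscenes, ability pickups and quest-driven world changes.
; PlaySequence runs a level sequence while hiding the host or client dialog widget, then restores it on finish and flags completion on the server.
; ActiveObject maps Megeton quest IDs to destroying and saving walls or activating end-gate portals.
; Server Tick clears the current ability once host and guest both obtain it; dialog OnRep handlers are empty.
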(event Custom|ActiveObject
  (params (NowQuestID :type EQuestID%20Enum%20%28by%20ref%29 :default "EMegetonNotMeet"))
  (switch Utilities|FlowControl|Switch|SwitchonEQuestID NowQuestID
    (:EMegetonMeet
      (bind _outactors (Actor|GetAllActorsOfClass "/Game/Object/Blueprints/Megeton/BP_Wall.BP_Wall_C"))
      (for _array_element _outactors
        (Utilities|Array|AddUnique (.DestoryActors (Utilities|Struct|BreakProgressData (Variables|Default|GetProgressData))) (Variables|/Game/Object/Blueprints/Megeton/BP_Wall.BP_Wall_C|GetID _array_element))
        (Default|Save (.AsBP%20Crafting%20Star%20Game%20Instance (Utilities|Casting|CastToBP_CraftingStarGameInstance (Game|GetGameInstance))))
        (Actor|DestroyActor _array_element)))
    (:EMegetonClear
      (bind _outactors_2 (Actor|GetAllActorsOfClass "/Game/Object/Blueprints/Megeton/BP_Gate.BP_Gate_C"))
      (for _array_element_2 _outactors_2
        (if (Utilities|String|Contains (Utilities|GetDisplayName _array_element_2) "BP_EndGate")
          (Default|SetActivePortal _array_element_2 true))))))

(event Custom|PlaySequence
  (params (Sequence :type Level%20Sequence%20Object%20Reference))
  (Variables|Default|SetisPlayed false)
  (bind _returnvalue (Sequencer|Player|CreateLevelSequencePlayer Sequence))
  (EventDispatchers|BindEventtoOnFinished _returnvalue (delegate Custom|Finished))
  (bind _asbp_crafting_star_character (Utilities|Casting|CastToBP_CraftingStarCharacter (Game|GetPlayerCharacter 0)))
  (if (Networking|IsServer)
    (bind _asdialog_widget (Utilities|Casting|CastToDialogWidget (Variables|/Game/Blueprints/InGameMenu/Player/BP_CraftingStarCharacter.BP_CraftingStarCharacter_C|GetDialogWidget _asbp_crafting_star_character)))
    (Default|Disappeartemporarily _asdialog_widget)
    (else
      (bind _asdialog_widget_client (Utilities|Casting|CastToDialogWidget_client (Variables|/Game/Blueprints/InGameMenu/Player/BP_CraftingStarCharacter.BP_CraftingStarCharacter_C|GetDialogWidget _asbp_crafting_star_character)))
      (Default|Disappeartemporarily _asdialog_widget_client)))
  (Sequencer|Player|Play _returnvalue :!class /Script/MovieScene.MovieSceneSequencePlayer)
  (Development|PrintString "Play" false))

(event Custom|Finished
  (bind _asbp_crafting_star_character (Utilities|Casting|CastToBP_CraftingStarCharacter (Game|GetPlayerCharacter 0)))
  (if (Networking|IsServer)
    (bind _asdialog_widget (Utilities|Casting|CastToDialogWidget (Variables|/Game/Blueprints/InGameMenu/Player/BP_CraftingStarCharacter.BP_CraftingStarCharacter_C|GetDialogWidget _asbp_crafting_star_character)))
    (Default|Appear _asdialog_widget)
    (Variables|Default|SetisPlayed true)
    (else
      (bind _asdialog_widget_client (Utilities|Casting|CastToDialogWidget_client (Variables|/Game/Blueprints/InGameMenu/Player/BP_CraftingStarCharacter.BP_CraftingStarCharacter_C|GetDialogWidget _asbp_crafting_star_character)))
      (Default|Appear _asdialog_widget_client))))

(event EventBeginPlay)

(event EventTick
  (params (DeltaSeconds :type Float%20%28single-precision%29))
  (if (Math|Boolean|ANDBoolean (Variables|Default|GetisHostObtain) (Variables|Default|GetisGuestObtain) (Networking|IsServer))
    (Variables|Default|SetisHostObtain false)
    (Variables|Default|SetisGuestObtain false)
    (Variables|Default|SetnowObtainingAbility "ENone")))

(fn ConstructionScript)

(fn OnRepDialogTextReplicates)

(fn OnRepIsSpeak?)

(fn OnRepDialogSpeakTextReplicates)

(fn OnRepSelectRepliesNum)

(fn OnRepIsHoveredReply)

(fn OnRepSelectReplies)

(fn OnRepIsPlayed)

(fn OnRepIsPlaying)