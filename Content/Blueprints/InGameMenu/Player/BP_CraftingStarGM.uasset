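; Game mode for a two-player CraftingStar session that starts play once host and guest are ready and keeps their save data updated.
; Tick polls the game state's success, host and guest flags, then applies outfits by mode, stores both characters and generates the first player's UI.
; Afterwards, Tick calls UpdateSaveData on each PlayerState every frame; its trailing Delay throttles nothing.
; SetPlayerData offers the same update on demand, reporting whether both succeeded.
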(event EventTick
  (params (DeltaSeconds :type Float%20%28single-precision%29))
  (bind _returnvalue (Game|GetPlayerCharacter 1))
  (bind _returnvalue_2 (Game|GetGameState))
  (bind (_asbp_crafting_star_gs _bsuccess) (Utilities|Casting|CastToBP_CraftingStarGS _returnvalue_2))
  (if (Variables|Default|GetStartFlag)
    (bind _asbp_crafting_star_character (Utilities|Casting|CastToBP_CraftingStarCharacter (Game|GetPlayerCharacter 0)))
    (bind _asbp_crafting_star_ps (Utilities|Casting|CastToBP_CraftingStarPS (Variables|/Script/Engine.Pawn|GetPlayerState _asbp_crafting_star_character)))
    (Default|UpdateSaveData _asbp_crafting_star_ps _asbp_crafting_star_character)
    (if (Utilities|IsValid _returnvalue)
      (bind _asbp_crafting_star_character_2 (Utilities|Casting|CastToBP_CraftingStarCharacter _returnvalue))
      (bind _asbp_crafting_star_ps_2 (Utilities|Casting|CastToBP_CraftingStarPS (Variables|/Script/Engine.Pawn|GetPlayerState _returnvalue)))
      (Default|UpdateSaveData _asbp_crafting_star_ps_2 _asbp_crafting_star_character_2)
      (Utilities|FlowControl|Delay 0.5))
    (elif (Math|Boolean|ANDBoolean _bsuccess (Variables|/Game/Blueprints/InGameMenu/Player/BP_CraftingStarGS.BP_CraftingStarGS_C|GetGuestFlag _asbp_crafting_star_gs) (Variables|/Game/Blueprints/InGameMenu/Player/BP_CraftingStarGS.BP_CraftingStarGS_C|GetHostFlag _asbp_crafting_star_gs))
      (bind _asbp_crafting_star_character_3 (Utilities|Casting|CastToBP_CraftingStarCharacter (Game|GetPlayerCharacter 0)))
      (bind _asbp_crafting_star_ps_3 (Utilities|Casting|CastToBP_CraftingStarPS (Variables|/Script/Engine.Pawn|GetPlayerState _asbp_crafting_star_character_3)))
      (Default|PlayerOutfit _asbp_crafting_star_character_3 _asbp_crafting_star_character_3 (.mode (Variables|/Script/CraftingStar.CraftingStarPS|GetPlayerData _asbp_crafting_star_ps_3)))
      (bind _returnvalue_3 (Utilities|Array|Add (Variables|Default|GetPlayerCharacterArr) _asbp_crafting_star_character_3))
      (Development|PrintString (Utilities|String|ToString(Integer) _returnvalue_3))
      (bind _asbp_crafting_star_character_4 (Utilities|Casting|CastToBP_CraftingStarCharacter (Game|GetPlayerCharacter 1)))
      (bind _asbp_crafting_star_ps_4 (Utilities|Casting|CastToBP_CraftingStarPS (Variables|/Script/Engine.Pawn|GetPlayerState _asbp_crafting_star_character_4)))
      (Default|PlayerOutfit _asbp_crafting_star_character_4 _asbp_crafting_star_character_4 (.mode (Variables|/Script/CraftingStar.CraftingStarPS|GetPlayerData _asbp_crafting_star_ps_4)))
      (bind _returnvalue_4 (Utilities|Array|Add (Variables|Default|GetPlayerCharacterArr) _asbp_crafting_star_character_4))
      (Development|PrintString (Utilities|String|ToString(Integer) _returnvalue_4))
      (Variables|Default|SetStartFlag true)
      (Default|PlayerUIGenerate _asbp_crafting_star_character_3))))

(event EventBeginPlay
  (Variables|Default|SetStartFlag false))

(fn ConstructionScript)

(fn SetPlayerData
  (bind _returnvalue (Game|GetPlayerCharacter 1))
  (bind _asbp_crafting_star_character (Utilities|Casting|CastToBP_CraftingStarCharacter (Game|GetPlayerCharacter 0))
    (:then
      (bind _asbp_crafting_star_ps (Utilities|Casting|CastToBP_CraftingStarPS (Variables|/Script/Engine.Pawn|GetPlayerState _asbp_crafting_star_character))
        (:then
          (Default|UpdateSaveData _asbp_crafting_star_ps _asbp_crafting_star_character)
          (if (Utilities|IsValid _returnvalue)
            (bind _asbp_crafting_star_character_2 (Utilities|Casting|CastToBP_CraftingStarCharacter _returnvalue)
              (:then
                (bind _asbp_crafting_star_ps_2 (Utilities|Casting|CastToBP_CraftingStarPS (Variables|/Script/Engine.Pawn|GetPlayerState _returnvalue))
                  (:then
                    (Default|UpdateSaveData _asbp_crafting_star_ps_2 _asbp_crafting_star_character_2)
                    (bind _output_get (Variables|Default|SetFlag true))
                    (return _output_get))
                  (:CastFailed
                    (Variables|Default|SetFlag false))))
              (:CastFailed
                (Variables|Default|SetFlag false)))
            (else
              (Variables|Default|SetFlag false))))
        (:CastFailed
          (Variables|Default|SetFlag false))))
    (:CastFailed
      (Variables|Default|SetFlag false))))