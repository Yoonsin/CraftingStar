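; Player character Blueprint for CraftingStar that handles proximity interaction, a fire-bowl ray ability and debug hotkeys.
; InteractionSphere overlaps collect InteractionInterface actors or components and respawn the player on death triggers.
; The interaction input starts dialog on the first entry, blocking multi dialogs while any player is already interacting.
; Holding G line-traces each tick to toggle fire bowls, alongside debug drawing and keys for health, respawn and save.
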(event OnComponentBeginOverlap(InteractionSphere)
  (params (OverlappedComponent :type Primitive%20Component%20Object%20Reference) (OtherActor :type Actor%20Object%20Reference) (OtherComp :type Primitive%20Component%20Object%20Reference) (OtherBodyIndex :type Integer) (bFromSweep :type Boolean) (SweepResult :type Hit%20Result%20Structure%20%28by%20ref%29))
  ;[1 1 1] 상호작용 물체 체크
  (bind _asinteraction_interface (Utilities|Casting|CastToInteractionInterface OtherActor)
    (:then
      (Utilities|Array|AddUnique (Variables|Default|GetInteractables%20in%20Range) _asinteraction_interface))
    (:CastFailed
      (for _array_element (Class|Actor|GetComponentsbyInterface OtherActor "/Game/Blueprints/InGameMenu/DialogSystem/DialogSystem/InteractionInterface.InteractionInterface_C")
        (bind _asinteraction_interface_2 (Utilities|Casting|CastToInteractionInterface _array_element))
        (Utilities|Array|AddUnique (Variables|Default|GetInteractables%20in%20Range) _asinteraction_interface_2))))
  (Utilities|Casting|CastToBP_DeathTriggerBox OtherActor)
  (Class|CraftingStarCharacter|CallRespawnPlayer))

(event OnComponentEndOverlap(InteractionSphere)
  (params (OverlappedComponent :type Primitive%20Component%20Object%20Reference) (OtherActor :type Actor%20Object%20Reference) (OtherComp :type Primitive%20Component%20Object%20Reference) (OtherBodyIndex :type Integer))
  ;[1 1 1] 상호작용 물체 체크
  (bind _asinteraction_interface (Utilities|Casting|CastToInteractionInterface OtherActor)
    (:then
      (Utilities|Array|RemoveItem (Variables|Default|GetInteractables%20In%20Range) _asinteraction_interface))
    (:CastFailed
      (for _array_element (Class|Actor|GetComponentsbyInterface OtherActor "/Game/Blueprints/InGameMenu/DialogSystem/DialogSystem/InteractionInterface.InteractionInterface_C")
        (bind _asinteraction_interface_2 (Utilities|Casting|CastToInteractionInterface _array_element))
        (Utilities|Array|RemoveItem (Variables|Default|GetInteractables%20In%20Range) _asinteraction_interface_2)))))

(event Custom|RequestServerOffRay
  ;[1 1 1] 레이 트레이싱
  (Utilities|IsValid (Variables|Default|GetAs%20BP%20Fire%20Bowl)
    (:Is%20Valid
      (Default|OffPerformed (Variables|Default|GetAs%20BP%20Fire%20Bowl))
      (Variables|Default|SetAs%20BP%20Fire%20Bowl 0))))

(event Custom|OnMulti
  ;[1 1 1] 상호작용 시작 (State에 따라 멀티/싱글 구분)
  (Variables|Default|SetisSomeInteract? false)
  (bind _array_element (Utilities|Array|ForEachLoopwithBreak (Variables|/Script/Engine.GameStateBase|GetPlayerArray (.AsCrafting%20Star%20GS (Utilities|Casting|CastToCraftingStarGS (Game|GetGameState)))))
    (:LoopBody
      (if (Utilities|Enum|Equal(Enum) (Variables|/Script/CraftingStar.CraftingStarPS|GetNowDisplayState (.AsCrafting%20Star%20PS (Utilities|Casting|CastToCraftingStarPS _array_element))) "EInteraction")
        (Variables|Default|SetisSomeInteract? true)))
    (:Completed
      (if (Variables|Default|GetisSomeInteract?)
        (Development|PrintString "이미 다른 누군가가 상호작용 중입니다!")
        (else
          (Default|OnInteraction (Utilities|Array|Get(acopy) (Variables|Default|GetInteractables%20In%20Range)) (.AsCrafting%20Star%20Character (Utilities|Casting|CastToCraftingStarCharacter (Game|GetPlayerCharacter 0)))))))))

(event Custom|RequestServerOnRay
  (bind _raycast (Variables|Default|GetRayCast))
  (bind _returnvalue (Transformation|GetWorldLocation _raycast))
  ;[1 1 1] 레이 트레이싱
  (bind _outhit (Collision|LineTraceByChannel _returnvalue (+ _returnvalue (* (Math|Vector|GetForwardVector (Transformation|GetWorldRotation _raycast)) 1.5e+03)) "TraceTypeQuery1" false 0 "None"))
  (bind _asbp_fire_bowl_obj (Utilities|Casting|CastToBP_FireBowl_Obj (.HitActor (Collision|BreakHitResult _outhit)))
    (:then
      (Default|OnPerformed _asbp_fire_bowl_obj)
      (Variables|Default|SetAs%20BP%20Fire%20Bowl _asbp_fire_bowl_obj))
    (:CastFailed
      (Utilities|IsValid (Variables|Default|GetAs%20BP%20Fire%20Bowl)
        (:Is%20Valid
          (Default|OffPerformed (Variables|Default|GetAs%20BP%20Fire%20Bowl)))))))

(event Custom|SetInteractionVisibility
  (params (isVisibility :type Boolean))
  ;[1 1 1] 상호작용 마크 활성화/비활성화
  (Rendering|SetVisibility (Variables|Default|GetInteractionTag) isVisibility false))

(event Collision|EventActorBeginOverlap
  (params (OtherActor :type Actor%20Object%20Reference)))

(event EventTick
  (params (DeltaSeconds :type Float%20%28single-precision%29))
  (bind _raycast (Variables|Default|GetRayCast))
  (bind _interactionsphere (Variables|Default|GetInteractionSphere))
  (bind _returnvalue (Transformation|GetWorldLocation _raycast))
  ;[1 1 1] 상호작용 범위 디버그
  (Rendering|Debug|DrawDebugSphere (Transformation|GetWorldLocation _interactionsphere) (Variables|/Script/Engine.SphereComponent|GetSphereRadius _interactionsphere) 15 "(R=0.000000,G=1.000000,B=0.035105,A=0.500000)" 0.0)
  (if (Variables|Default|GetisRay?)
    (Rendering|Debug|DrawDebugLine _returnvalue (+ _returnvalue (* (Math|Vector|GetForwardVector (Transformation|GetWorldRotation _raycast)) 1.5e+03)) "(R=1.000000,G=0.137786,B=0.000000,A=1.000000)" 0.0 0.0)
    (CallFunction|RequestServeronRay)))

(event Input|ActionEvents|InputActionInteraction
  (params (Key :type Key%20Structure))
  (bind _interactables_in_range (Variables|Default|GetInteractables%20In%20Range))
  (bind _output (Utilities|Array|Get(acopy) _interactables_in_range))
  ;[1 1 1] 상호작용 시작 (State에 따라 멀티/싱글 구분)
  (:Pressed
    (if (> (Utilities|Array|Length (Variables|Default|GetInteractables%20In%20Range)) 0)
      (bind _state (Default|GetMultiState (.AsDialog%20Component (Utilities|Casting|CastToDialogComponent _output))))
      (Development|PrintString (Utilities|String|EnumtoString _state))
      (switch Utilities|FlowControl|Switch|SwitchonEInteractionMultiState _state
        (:NewEnumerator0
          (CallFunction|OnMulti))
        (:NewEnumerator1
          (Default|OnInteraction _output self))))))

(event Input|KeyboardEvents|G
  (params (Key :type Key%20Structure))
  ;[1 1 1] 레이 트레이싱
  (:Pressed
    (Variables|Default|SetisRay? true))
  (:Released
    (Variables|Default|SetisRay? false)
    (CallFunction|RequestServerOffRay)))

(event Input|KeyboardEvents|Y
  (params (Key :type Key%20Structure))
  (bind _playerstate (Variables|Default|GetPlayerState))
  (bind _ascrafting_star_ps (Utilities|Casting|CastToCraftingStarPS _playerstate))
  ;[1 1 1] 상호작용 범위 디버그
  ;;[1 1 1] HP 깎임 디버그
  (:Pressed
    (Utilities|IsValid _ascrafting_star_ps
      (:Is%20Valid
        (Class|CraftingStarPS|RequestHealth _ascrafting_star_ps 1e+01)))))

(event Input|KeyboardEvents|V
  (params (Key :type Key%20Structure))
  ;[1 1 1] 리스폰 디버그
  (:Pressed
    (Class|CraftingStarCharacter|CallRespawnPlayer)))

(event Input|KeyboardEvents|B
  (params (Key :type Key%20Structure))
  ;[1 1 1] 세이브 디버그
  (:Pressed
    (Class|CraftingStarPS|RequestSave (.AsCrafting%20Star%20PS (Utilities|Casting|CastToCraftingStarPS (Variables|Default|GetPlayerState))))
    (Default|Save (.AsBP%20Crafting%20Star%20Game%20Instance (Utilities|Casting|CastToBP_CraftingStarGameInstance (Game|GetGameInstance))))))

(fn ConstructionScript)