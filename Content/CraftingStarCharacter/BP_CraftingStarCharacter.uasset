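; Player character Blueprint for a two-player co-op game, handling world interaction, reviving knocked-down teammates, death-trigger respawns and replicated aim offset/visibility.
; Capsule overlaps maintain an interactables list that drives the dialog UI and, on authority, host/guest in-range flags in GameState.
; The Interaction input attempts a revive, then dispatches by multi/single state and interaction type.
; Shared dialog requires both players in range; guest actions often route through OnMulti.
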(event OnComponentEndOverlap(CapsuleComponent)
  (params (OverlappedComponent :type Primitive%20Component%20Object%20Reference) (OtherActor :type Actor%20Object%20Reference) (OtherComp :type Primitive%20Component%20Object%20Reference) (OtherBodyIndex :type Integer))
  ;[1 1 1] 상호작용 물체 체크
  (CallFunction|RemoveInteractables OtherActor)
  (CallFunction|SetUIInteractable))

(event OnComponentBeginOverlap(CapsuleComponent)
  (params (OverlappedComponent :type Primitive%20Component%20Object%20Reference) (OtherActor :type Actor%20Object%20Reference) (OtherComp :type Primitive%20Component%20Object%20Reference) (OtherBodyIndex :type Integer) (bFromSweep :type Boolean) (SweepResult :type Hit%20Result%20Structure%20%28by%20ref%29))
  ;[1 1 1] 상호작용 물체 체크
  (CallFunction|AddInteractables OtherActor)
  (CallFunction|SetUIInteractable)
  (Utilities|Casting|CastToBP_DeathTriggerBox OtherActor)
  (Class|CraftingStarCharacter|CallRespawnPlayer))

(event Custom|ServerSetVisible
  (params (isVisible :type Boolean))
  ;[1 1 1] 캐릭터 Visible
  (CallFunction|MultiSetVisible isVisible))

(event Custom|OnMulti
  ;[1 1 1] 상호작용 시작 (State에 따라 멀티/싱글 구분)
  ;;[1 1 1] Object 상호작용
  (CallFunction|MultiInteractive))

(event Custom|MultiSetVisible
  (params (isVisible :type Boolean%20%28by%20ref%29))
  ;[1 1 1] 캐릭터 Visible
  (Development|PrintString "Hello")
  (for _array_element (Variables|/Script/Engine.GameStateBase|GetPlayerArray (Game|GetGameState))
    (bind _asbp_crafting_star_character (Utilities|Casting|CastToBP_CraftingStarCharacter (Variables|/Script/Engine.PlayerState|GetPawnPrivate _array_element)))
    (Rendering|SetVisibility (Variables|/Script/Engine.Character|GetMesh _asbp_crafting_star_character) isVisible true)
    (Rendering|SetVisibility (Variables|/Script/CraftingStar.CraftingStarCharacter|GetComp_LaserNiagara _asbp_crafting_star_character) false true)
    (Rendering|SetVisibility (Variables|/Script/CraftingStar.CraftingStarCharacter|GetinteractTag _asbp_crafting_star_character) false false)))

(event Custom|MultiNotifiyUIInteractable
  (params (isInRange :type Boolean) (Type :type EInteractionType%20Enum :default "NewEnumerator0"))
  ;[1 1 1] 상호작용 물체 체크
  (Networking|SwitchHasAuthority
    (:Authority
      _)
    (:Remote
      _))
  (bind _asbp_crafting_star_character (Utilities|Casting|CastToBP_CraftingStarCharacter (Game|GetPlayerCharacter 0)))
  (bind _aswbp_game (Utilities|Casting|CastToWBP_Game (Variables|/Script/CraftingStar.CraftingStarCharacter|GetGameWidgetRef _asbp_crafting_star_character)))
  (Default|SetHeadcount _aswbp_game isInRange Type))

(event Custom|SetVisibleUIInteractable
  (params (Visibility :type ESlateVisibility%20Enum :default "Visible") (Character :type BP%20Crafting%20Star%20Character%20Object%20Reference%20%28by%20ref%29))
  ;[1 1 1] 상호작용 물체 체크
  (bind _aswbp_game (Utilities|Casting|CastToWBP_Game (Variables|/Script/CraftingStar.CraftingStarCharacter|GetGameWidgetRef Character)))
  (Default|SetVisibilityDialogBox _aswbp_game Visibility))

(event Custom|MultiSetVisibleUIInteractable
  (params (Visibility :type ESlateVisibility%20Enum :default "Visible"))
  ;[1 1 1] 상호작용 물체 체크
  (Networking|SwitchHasAuthority
    (:Authority
      _)
    (:Remote
      _))
  (bind _asbp_crafting_star_character (Utilities|Casting|CastToBP_CraftingStarCharacter (Game|GetPlayerCharacter 0)))
  (CallFunction|SetVisibleUIInteractable _asbp_crafting_star_character Visibility _asbp_crafting_star_character))

(event Custom|Server_ReviveInteraction
  ;[1 1 1] 상호작용 시작 (State에 따라 멀티/싱글 구분)
  ;;[0.2431 0.5094 0] Incendie: 쓰러진 플레이어 부활
  ;;;[1 1 1] Replicate Revival
  (CallFunction|ClientReviveInteraciton))

(event Custom|Client_ReviveInteraciton
  (bind _audiocomp (Variables|Default|GetaudioComp))
  ;[1 1 1] 상호작용 시작 (State에 따라 멀티/싱글 구분)
  ;;[0.2431 0.5094 0] Incendie: 쓰러진 플레이어 부활
  ;;;[1 1 1] Player doing Revival
  (bind _array_element (Utilities|Array|ForEachLoopwithBreak (Collision|GetOverlappingActors "BP_CraftingStarCharacter_C" :!class /Script/Engine.Actor) :!label _label)
    (:LoopBody
      (if (Utilities|DoesObjectImplementInterface _array_element "/Game/CraftingStarCharacter/RevivalInteractionInterface.RevivalInteractionInterface_C")
        (Class|RevivalInteractionInterface|OnReviveInteraction(Message) _array_element)
        (Audio|Components|Audio|SetSound _audiocomp "/Game/SFX/heal.heal")
        (Audio|Components|Audio|Play _audiocomp 0.0)
        (goto _label Break)))))

(event Custom|Server_SetArmVertical
  (params (New%20Value :type Float%20%28single-precision%29))
  ;[1 1 1] AimOffset 값 전달
  (CallFunction|MulticastSetArmVertical New%20Value))

(event Custom|Multicast_SetArmVertical
  (params (New%20Value :type Float%20%28single-precision%29))
  ;[1 1 1] AimOffset 값 전달
  (Variables|Animation|SetArmVertical New%20Value))

(event EventOnReviveInteraction
  (bind _audiocomp (Variables|Default|GetaudioComp))
  ;[1 1 1] 상호작용 시작 (State에 따라 멀티/싱글 구분)
  ;;[0.2431 0.5094 0] Incendie: 쓰러진 플레이어 부활
  ;;;[1 1 1] Player being Revived
  (if (Variables|Default|GetisKnockedDown)
    (Class|CraftingStarCharacter|OnRevivePopo)
    (Audio|Components|Audio|SetSound _audiocomp "/Game/SFX/heal.heal")
    (Audio|Components|Audio|Play _audiocomp 0.0)))

(event Collision|EventActorBeginOverlap
  (params (OtherActor :type Actor%20Object%20Reference)))

(event Input|ActionEvents|InputActionInteraction
  (params (Key :type Key%20Structure :default "None"))
  ;[1 1 1] 상호작용 시작 (State에 따라 멀티/싱글 구분)
  (:Pressed
    (Utilities|FlowControl|Sequence
      (:then_0
        ;;[0.2431 0.5094 0] Incendie: 쓰러진 플레이어 부활
        ;;;[1 1 1] Replicate Revival
        (CallFunction|ServerReviveInteraction))
      (:then_1
        ;;[1 1 1] Object 상호작용
        ;;;[1 1 1] 상호작용 모드 확인
        (CallFunction|CheckInteractiveMode)))))

(event Input|KeyboardEvents|Hyphen
  (params (Key :type Key%20Structure :default "None")))

(event Input|KeyboardEvents|Y
  (params (Key :type Key%20Structure :default "None"))
  (bind _playerstate (Variables|Default|GetPlayerState))
  (bind _ascrafting_star_ps (Utilities|Casting|CastToCraftingStarPS _playerstate))
  ;[1 1 1] HP 깎임 디버그
  (:Pressed
    (Utilities|IsValid _ascrafting_star_ps
      (:Is%20Valid
        (Class|CraftingStarPS|RequestHealth _ascrafting_star_ps 1e+01)))))

(event Input|KeyboardEvents|V
  (params (Key :type Key%20Structure :default "None"))
  ;[1 1 1] 리스폰 디버그
)

(event Input|KeyboardEvents|B
  (params (Key :type Key%20Structure :default "None"))
  ;[1 1 1] 죽음 디버그
)

(fn ConstructionScript)

(fn AddInteractables
  (params (Actor :type Actor%20Object%20Reference))
  (bind _returnvalue (Game|GetGameState))
  (bind _asinteraction_interface (Utilities|Casting|CastToInteractionInterface Actor)
    (:then
      (bind _returnvalue_2 (Utilities|Array|AddUnique (Variables|Default|GetInteractables%20in%20Range) _asinteraction_interface))
      (LocalVariables|SetIdx _returnvalue_2)
      (Networking|SwitchHasAuthority :!label _label
        (:Authority
          (bind _type (Default|GetInteractionType (Utilities|Array|Get(acopy) (Variables|Default|GetInteractables%20in%20Range) (LocalVariables|GetIdx))))
          (CallFunction|MultiNotifiyUIInteractable true _type)
          (bind _returnvalue_3 (Class|UtilityFunction|IsHost (Pawn|GetController self)))
          (if _returnvalue_3
            (bind _ascrafting_star_gs (Utilities|Casting|CastToCraftingStarGS _returnvalue))
            (Variables|/Script/CraftingStar.CraftingStarGS|SetisHostInInteractionRange _ascrafting_star_gs true)
            (Class|CraftingStarGS|InteractChange _ascrafting_star_gs true true)
            (else
              (bind _ascrafting_star_gs_2 (Utilities|Casting|CastToCraftingStarGS _returnvalue))
              (Variables|/Script/CraftingStar.CraftingStarGS|SetisGuestInInteractionRange _ascrafting_star_gs_2 true)
              (Class|CraftingStarGS|InteractChange _ascrafting_star_gs_2 false true))))))
    (:CastFailed
      (for _array_element (Class|Actor|GetComponentsbyInterface Actor "/Game/Object/Blueprints/Interaction/InteractionInterface.InteractionInterface_C")
        (bind _asinteraction_interface_2 (Utilities|Casting|CastToInteractionInterface _array_element))
        (bind _returnvalue_4 (Utilities|Array|AddUnique (Variables|Default|GetInteractables%20in%20Range) _asinteraction_interface_2))
        (LocalVariables|SetIdx _returnvalue_4)
        (goto _label)))))

(fn RemoveInteractables
  (params (Actor :type Actor%20Object%20Reference))
  (bind _returnvalue (Game|GetGameState))
  (bind _asinteraction_interface (Utilities|Casting|CastToInteractionInterface Actor)
    (:then
      (Utilities|Array|RemoveItem (Variables|상호작용|GetInteractables%20In%20Range) _asinteraction_interface)
      (LocalVariables|SetInterface _asinteraction_interface)
      (Networking|SwitchHasAuthority :!label _label
        (:Authority
          (bind _type (Default|GetInteractionType (LocalVariables|GetInterface)))
          (CallFunction|MultiNotifiyUIInteractable false _type)
          (bind _returnvalue_2 (Class|UtilityFunction|IsHost (Pawn|GetController self)))
          (if _returnvalue_2
            (bind _ascrafting_star_gs (Utilities|Casting|CastToCraftingStarGS _returnvalue))
            (Variables|/Script/CraftingStar.CraftingStarGS|SetisHostInInteractionRange _ascrafting_star_gs false)
            (Class|CraftingStarGS|InteractChange _ascrafting_star_gs true false)
            (else
              (bind _ascrafting_star_gs_2 (Utilities|Casting|CastToCraftingStarGS _returnvalue))
              (Variables|/Script/CraftingStar.CraftingStarGS|SetisGuestInInteractionRange _ascrafting_star_gs_2 false)
              (Class|CraftingStarGS|InteractChange _ascrafting_star_gs_2 false false))))))
    (:CastFailed
      (for _array_element (Class|Actor|GetComponentsbyInterface Actor "/Game/Object/Blueprints/Interaction/InteractionInterface.InteractionInterface_C")
        (bind _asinteraction_interface_2 (Utilities|Casting|CastToInteractionInterface _array_element))
        (Utilities|Array|RemoveItem (Variables|상호작용|GetInteractables%20In%20Range) _asinteraction_interface_2)
        (LocalVariables|SetInterface _asinteraction_interface_2)
        (goto _label)))))

(fn SetUIInteractable
  (bind _returnvalue (Pawn|IsLocallyControlled))
  (bind _interactables_in_range (Variables|상호작용|GetInteractables%20In%20Range))
  (bind _gamewidgetref (Variables|Default|GetGameWidgetRef))
  (Networking|SwitchHasAuthority
    (:Authority
      (if _returnvalue
        (if (> (Utilities|Array|Length _interactables_in_range) 0) :!label _label
          (bind _type (Default|GetInteractionType (Utilities|Array|Get(acopy) _interactables_in_range)))
          (if (!= _type (Utilities|Enum|LiteralenumEInteractionType "NewEnumerator3"))
            (Utilities|IsValid _gamewidgetref
              (:Is%20Valid
                (bind _aswbp_game (Utilities|Casting|CastToWBP_Game _gamewidgetref)
                  (:then
                    (Default|SetVisibilityDialogBox _aswbp_game "HitTestInvisible")
                    (Default|SetDialogText _aswbp_game _type))
                  (:CastFailed
                    (Development|PrintString "fail"))))
              (:Is%20Not%20Valid
                (Development|PrintString "isNotVaild"))))
          (else
            (bind _aswbp_game_2 (Utilities|Casting|CastToWBP_Game (Variables|Default|GetGameWidgetRef)))
            (Default|SetVisibilityDialogBox _aswbp_game_2 "Collapsed")))))
    (:Remote
      (if _returnvalue
        (goto _label)))))

(fn MultiInteractive
  (bind _returnvalue (Game|GetPlayerCharacter 0))
  (bind _interactables_in_range (Variables|상호작용|GetInteractables%20In%20Range))
  (bind _ascrafting_star_character (Utilities|Casting|CastToCraftingStarCharacter _returnvalue))
  (bind _output (Utilities|Array|Get(acopy) _interactables_in_range))
  (Variables|상호작용|SetisSomeInteract? false)
  (bind _array_element (Utilities|Array|ForEachLoopwithBreak (Variables|/Script/Engine.GameStateBase|GetPlayerArray (.AsCrafting%20Star%20GS (Utilities|Casting|CastToCraftingStarGS (Game|GetGameState)))))
    (:LoopBody
      (if (Utilities|Enum|Equal(Enum) (Variables|/Script/CraftingStar.CraftingStarPS|GetNowDisplayState (.AsCrafting%20Star%20PS (Utilities|Casting|CastToCraftingStarPS _array_element))) "EInteraction")
        (Variables|상호작용|SetisSomeInteract? true)))
    (:Completed
      (if (Variables|상호작용|GetisSomeInteract?)
        (Development|PrintString "이미 다른 누군가가 상호작용 중입니다!" false)
        (else
          (bind _type (Default|GetInteractionType _output))
          (switch Utilities|FlowControl|Switch|SwitchonEInteractionType _type
            (:NewEnumerator0
              (Default|OnInteraction _output _ascrafting_star_character :!label _label))
            (:NewEnumerator2
              (bind _asdialog_component (Utilities|Casting|CastToDialogComponent _output))
              (if (== (Utilities|GetClass (Components|GetOwner _asdialog_component)) "/Game/Object/Blueprints/Megeton/BP_MessageTriger.BP_MessageTriger_C")
                (if (Utilities|Enum|Equal(Enum) (.questid (Variables|/Script/CraftingStar.CraftingStarGS|GetProgressData (.AsCrafting%20Star%20GS (Utilities|Casting|CastToCraftingStarGS (Game|GetGameState))))) "EMegetonMeet")
                  (Default|OnInteraction _asdialog_component _ascrafting_star_character :!label _label_2))
                (else
                  (goto _label_2))))
            (:NewEnumerator1
              (goto _label))
            (:NewEnumerator4
              (Default|OnInteraction _output (.AsCrafting%20Star%20Character (Utilities|Casting|CastToCraftingStarCharacter (Game|GetPlayerCharacter 0))) :!label _label_3))
            (:NewEnumerator5
              (goto _label_3))))))))

(fn CheckInteractiveMode
  (bind _interactables_in_range (Variables|상호작용|GetInteractables%20In%20Range))
  (bind _output (Utilities|Array|Get(acopy) _interactables_in_range))
  (if (> (Utilities|Array|Length (Variables|상호작용|GetInteractables%20In%20Range)) 0)
    (bind _state (Default|GetMultiState _output))
    (switch Utilities|FlowControl|Switch|SwitchonEInteractionMultiState _state
      (:NewEnumerator0
        (|MultiDialog))
      (:NewEnumerator1
        (bind _type (Default|GetInteractionType _output))
        (switch Utilities|FlowControl|Switch|SwitchonEInteractionType _type
          (:NewEnumerator0
            (|Read _output))
          (:NewEnumerator2
            (|Dialog _output))
          (:NewEnumerator1
            (|OpenDoor _output))
          (:NewEnumerator4
            (|Item _output))
          (:NewEnumerator5
            (|Resque _output)))))))

(fn GetInteractionType
  (return "NewEnumerator0"))

(fn GetMultiState
  (return "NewEnumerator0"))