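; BP_NightmareDragon is a dragon monster Blueprint with a cooldown-gated attack.
; Attack plays the dragon attack montage, prints a debug hit message naming itself and the target player, and resets the cooldown; it applies no damage.
; Tick counts the cooldown down toward zero, and GetAttackable reports when it has expired, leaving callers to check it because Attack does not.
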(event EventBeginPlay)

(event Collision|EventActorBeginOverlap
  (params (OtherActor :type Actor%20Object%20Reference)))

(event EventTick
  (params (DeltaSeconds :type Float%20%28single-precision%29))
  (if (> (Variables|Default|GetAttackCurrentCooldown) 0.0)
    (Variables|Default|SetAttackCurrentCooldown (- (Variables|Default|GetAttackCurrentCooldown) DeltaSeconds))
    (else
      (Variables|Default|SetAttackCurrentCooldown 0.0))))

(fn ConstructionScript)

(fn Attack
  (params (Target%20Player :type Pawn%20Object%20Reference))
  (Animation|PlayAnimMontage "/Game/Monster/Animation/AM_DragonAttack.AM_DragonAttack" 1.0 "None")
  (Development|PrintString (Utilities|String|Append (Utilities|GetObjectName self) " hit " (Utilities|GetObjectName Target%20Player)))
  (Variables|Default|SetAttackCurrentCooldown (Variables|Default|GetAttackMaxCooldown)))

(fn GetAttackable
  (return (<= (Variables|Default|GetAttackCurrentCooldown) 0.0)))