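; BP_Laser is an actor that projects a Niagara laser beam along its forward vector.
; Each tick it line traces on the Camera channel up to Distance, with debug drawing, and sets the beam's LaserEnd to the hit location or trace end.
; The impact effect follows the hit location and shows only on a blocking hit.
; BeginPlay sets both effects' Color parameter to black.
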(event EventBeginPlay
  (Effects|Components|ParticleSystem|SetColorParameter (Variables|Default|GetNiagaraLaser) "Color" "(R=0.000000,G=0.000000,B=0.000000,A=1.000000)"))

(event Collision|EventActorBeginOverlap
  (params (OtherActor :type Actor%20Object%20Reference)))

(event EventTick
  (params (DeltaSeconds :type Float%20%28single-precision%29))
  (bind _returnvalue (Transformation|GetActorLocation))
  (bind _returnvalue_2 (Transformation|GetActorForwardVector))
  (bind _distance (Variables|디폴트|GetDistance))
  (bind _returnvalue_3 (* _returnvalue_2 _distance))
  (bind _returnvalue_4 (+ _returnvalue _returnvalue_3))
  (Variables|디폴트|SetTraceEnd _returnvalue_4)
  (bind _outhit (Collision|LineTraceByChannel _returnvalue _returnvalue_4 "TraceTypeQuery2" false 0 "ForOneFrame"))
  (Variables|Default|SetbHit (.bBlockingHit (Collision|BreakHitResult _outhit)))
  (Variables|Default|SetHitLocation (.Location (Collision|BreakHitResult _outhit)))
  (Effects|Components|ParticleSystem|SetVectorParameter (Variables|Default|GetNiagaraLaser) "LaserEnd" (select (Variables|Default|GetbHit) (Variables|Default|GetHitLocation) (Variables|디폴트|GetTraceEnd)))
  (Rendering|SetVisibility (Variables|Default|GetNiagaraLaserImpact) (Variables|Default|GetbHit) false)
  (Transformation|SetWorldLocation (Variables|Default|GetNiagaraLaserImpact) (Variables|Default|GetHitLocation) false false))

(fn ConstructionScript)