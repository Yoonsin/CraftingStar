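; BP_NPC_Glacier is an NPC Blueprint with an interaction radius and a persistent ID for saving world state.
; Its construction script sizes the trigger sphere and radius mesh from the square root of InteractionSquared, and generates a GUID when ID is empty.
; SaveState adds that ID uniquely to the CraftingStarGS WorldObjects progress data and saves through the game instance, while LoadState is empty.
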(event EventBeginPlay
  (|CallParentFunction) ; 지금 이 노드는 비활성 상태입니다. \n핀을 끌어서 다른 노드를 연결하면 활성화됩니다.
)

(event Collision|EventActorBeginOverlap
  (params (OtherActor :type Actor%20Object%20Reference))
  (|CallParentFunction OtherActor) ; 지금 이 노드는 비활성 상태입니다. \n핀을 끌어서 다른 노드를 연결하면 활성화됩니다.
)

(event EventTick
  (params (DeltaSeconds :type Float%20%28single-precision%29))
  (|CallParentFunction DeltaSeconds) ; 지금 이 노드는 비활성 상태입니다. \n핀을 끌어서 다른 노드를 연결하면 활성화됩니다.
)

(event EventSaveState
  (bind _ascrafting_star_gs (Utilities|Casting|CastToCraftingStarGS (Game|GetGameState)))
  (Utilities|Array|AddUnique (.WorldObjects (Utilities|Struct|BreakProgressData (Variables|/Script/CraftingStar.CraftingStarGS|GetProgressData _ascrafting_star_gs))) (Variables|세이브|GetID))
  (Class|UtilityFunction|Save (Game|GetGameInstance)))

(event EventLoadState)

(fn ConstructionScript
  (bind _interactionsquared (Variables|Default|GetInteractionSquared))
  (bind _returnvalue (Math|Float|Sqrt _interactionsquared))
  (bind _returnvalue_2 (/ _returnvalue 5e+01))
  (|CallParentFunction)
  (Transformation|SetWorldScale3D (Variables|Default|GetInteractionRadiusMesh) (Math|Vector|MakeVector _returnvalue_2 _returnvalue_2 1.0))
  (Components|Sphere|SetSphereRadius (Variables|Default|GetSphere) _returnvalue true)
  (if (Utilities|Enum|Equal(Enum) (Variables|세이브|GetID) "")
    (Variables|세이브|SetID (Guid|ToString(Guid) (Guid|NewGuid)))))

(fn GetObjectID
  (return (Variables|세이브|GetID)))