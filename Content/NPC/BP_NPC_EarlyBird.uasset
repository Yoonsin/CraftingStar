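; BP_NPC_EarlyBird is an interactable NPC actor that can be shown or hidden as a whole.
; Show and Hide events toggle its tick, collision and visibility together.
; The construction script sizes a radius mesh and sphere component from the square root of InteractionSquared, and assigns a new GUID string to ID when it is empty.
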(event Custom|Show
  (Actor|Tick|SetActorTickEnabled true)
  (Collision|SetActorEnableCollision true)
  (Rendering|SetActorHiddenInGame false))

(event Custom|Hide
  (Actor|Tick|SetActorTickEnabled false)
  (Collision|SetActorEnableCollision false)
  (Rendering|SetActorHiddenInGame true))

(event EventBeginPlay
  (|CallParentFunction) ; 지금 이 노드는 비활성 상태입니다. \n핀을 끌어서 다른 노드를 연결하면 활성화됩니다.
)

(event Collision|EventActorBeginOverlap
  (params (OtherActor :type Actor%20Object%20Reference))
  (|CallParentFunction OtherActor) ; 지금 이 노드는 비활성 상태입니다. \n핀을 끌어서 다른 노드를 연결하면 활성화됩니다.
)

(event EventTick
  (params (DeltaSeconds :type Float%20%28single-precision%29))
  (|CallParentFunction DeltaSeconds) ; 지금 이 노드는 비활성 상태입니다. \n핀을 끌어서 다른 노드를 연결하면 활성화됩니다.
)

(fn ConstructionScript
  (bind _interactionsquared (Variables|Default|GetInteractionSquared))
  (bind _returnvalue (Math|Float|Sqrt _interactionsquared))
  (bind _returnvalue_2 (/ _returnvalue 5e+01))
  (|CallParentFunction)
  (Transformation|SetWorldScale3D (Variables|Default|GetInteractionRadiusMesh) (Math|Vector|MakeVector _returnvalue_2 _returnvalue_2 1.0))
  (Components|Sphere|SetSphereRadius (Variables|Default|GetSphere) _returnvalue true)
  (if (Utilities|Enum|Equal(Enum) (Variables|Default|GetID) "")
    (Variables|Default|SetID (Guid|ToString(Guid) (Guid|NewGuid)))))