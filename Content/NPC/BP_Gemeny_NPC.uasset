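; BP_Gemeny_NPC is a modular NPC with two looks selected by IsLight: a light female-headed variant or a darker male-headed one.
; The construction script swaps head, hair, eye and mouth static meshes, body and cape skeletal meshes, and hair, cape and body materials.
; The Eye component receives the Mouth meshes and vice versa.
; Event graph stubs are empty, so the Blueprint's graphs only handle appearance.
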(event EventBeginPlay)

(event Collision|EventActorBeginOverlap
  (params (OtherActor :type Actor%20Object%20Reference)))

(event EventTick
  (params (DeltaSeconds :type Float%20%28single-precision%29)))

(fn ConstructionScript
  (Utilities|FlowControl|Sequence
    (:then_0
      ;[1 1 1] Head
      (Components|StaticMesh|SetStaticMesh (Variables|Default|GetHead) (select (Variables|Default|GetbIsLight) "/Game/Assets/BaseContent/RPGTinyHeroWavePolyart/Mesh/HeadPart/Head02_Female_SM.Head02_Female_SM" "/Game/Assets/BaseContent/RPGTinyHeroWavePolyart/Mesh/HeadPart/Head01_Male_SM.Head01_Male_SM"))
      ;[1 1 1] Hair
      (Components|StaticMesh|SetStaticMesh (Variables|Default|GetHair) (select (Variables|Default|GetbIsLight) "/Game/Assets/BaseContent/RPGTinyHeroWavePolyart/Mesh/HeadPart/Hair09_SM.Hair09_SM" "/Game/Assets/BaseContent/RPGTinyHeroWavePolyart/Mesh/HeadPart/Hair02_SM.Hair02_SM"))
      (Rendering|Material|SetMaterial (Variables|Default|GetHair) 0 (select (Variables|Default|GetbIsLight) "/Game/Assets/PlayerMaterial/Material/Light/MaskTintPolyart_Light_Hair.MaskTintPolyart_Light_Hair" "/Game/Assets/PlayerMaterial/Material/Dark/MaskTintPolyart_Dark_hair_notTh.MaskTintPolyart_Dark_hair_notTh"))
      ;[1 1 1] Eye & Mouth
      (Components|StaticMesh|SetStaticMesh (Variables|Default|GetEye) (select (Variables|Default|GetbIsLight) "/Game/Assets/BaseContent/RPGTinyHeroWavePolyart/Mesh/HeadPart/Mouth02_SM.Mouth02_SM" "/Game/Assets/BaseContent/RPGTinyHeroWavePolyart/Mesh/HeadPart/Mouth01_SM.Mouth01_SM"))
      (Components|StaticMesh|SetStaticMesh (Variables|Default|GetMouth) (select (Variables|Default|GetbIsLight) "/Game/Assets/BaseContent/RPGTinyHeroWavePolyart/Mesh/HeadPart/Eye08_SM.Eye08_SM" "/Game/Assets/BaseContent/RPGTinyHeroWavePolyart/Mesh/HeadPart/Eye01_SM.Eye01_SM")))
    (:then_1
      ;[1 1 1] Cape
      (Class|SkinnedMeshComponent|SetSkeletalMesh (Variables|Default|GetCape) (select (Variables|Default|GetbIsLight) "/Game/Assets/BaseContent/RPGTinyHeroWavePolyart/Mesh/BodyPart/Cloak02_SK.Cloak02_SK" "/Game/Assets/BaseContent/RPGTinyHeroWavePolyart/Mesh/BodyPart/Cloak03_SK.Cloak03_SK") true)
      (Rendering|Material|SetMaterial (Variables|Default|GetCape) 0 (select (Variables|Default|GetbIsLight) "/Game/Assets/PlayerMaterial/Material/Light/MaskTintPolyart_Light_Cape.MaskTintPolyart_Light_Cape" "/Game/Assets/PlayerMaterial/Material/Dark/MaskTintPolyart_cape.MaskTintPolyart_cape"))
      ;[1 1 1] Body
      (Class|SkinnedMeshComponent|SetSkeletalMesh (Variables|Character|GetMesh) (select (Variables|Default|GetbIsLight) "/Game/Assets/BaseContent/RPGTinyHeroWavePolyart/Mesh/BodyPart/Body10_SK.Body10_SK" "/Game/Assets/BaseContent/RPGTinyHeroWavePolyart/Mesh/BodyPart/Body09_SK.Body09_SK") true)
      (Rendering|Material|SetMaterial (Variables|Character|GetMesh) 0 (select (Variables|Default|GetbIsLight) "/Game/Assets/PlayerMaterial/Material/Light/MaskTintPolyart_Light_Body.MaskTintPolyart_Light_Body" "/Game/Assets/PlayerMaterial/Material/Dark/MaskTintPolyart_suit.MaskTintPolyart_suit")))))