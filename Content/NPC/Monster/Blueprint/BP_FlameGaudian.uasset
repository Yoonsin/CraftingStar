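; Flame guardian monster that is driven by an AI controller to follow an assigned spline route.
; On BeginPlay it cross-links the route and its BP_FGAIController, then runs a hard-coded delayed on, off, on sequence.
; The authority-only trigger events set the blackboard's ShouldFollow flag and the route's IsOn state together.
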(event EventBeginPlay
  (bind _splineroute (Variables|Default|GetSplineRoute))
  (Utilities|IsValid (Variables|Default|GetSplineRoute)
    (:Is%20Valid
      (bind _asbp_fgaicontroller (Utilities|Casting|CastToBP_FGAIController (Pawn|GetController)))
      (Variables|/Game/NPC/Monster/Blueprint/BP_FGAIController.BP_FGAIController_C|SetChasingRouteSpline _asbp_fgaicontroller _splineroute)
      (Variables|/Game/Object/Blueprints/Incendies/BP_Route_Guadian.BP_Route_Guadian_C|SetGuadianController _splineroute _asbp_fgaicontroller)
      (Utilities|FlowControl|Delay 1e+01)
      (CallFunction|Trigeron)
      (Utilities|FlowControl|Delay 3.0)
      (CallFunction|TrigerOff)
      (Utilities|FlowControl|Delay 3.0)
      (CallFunction|Trigeron))))

(event Collision|EventActorBeginOverlap
  (params (OtherActor :type Actor%20Object%20Reference)))

(event EventTrigeron
  (Networking|SwitchHasAuthority
    (:Authority
      (AI|Components|Blackboard|SetValueasBool (AI|GetBlackboard (Pawn|GetController)) (Utilities|Name|MakeLiteralName "ShouldFollow") true)
      (Variables|/Game/Object/Blueprints/Incendies/BP_Route_Guadian.BP_Route_Guadian_C|SetbIsOn (Variables|Default|GetSplineRoute) true))))

(event EventTrigerOff
  (Networking|SwitchHasAuthority
    (:Authority
      (AI|Components|Blackboard|SetValueasBool (AI|GetBlackboard (Pawn|GetController)) (Utilities|Name|MakeLiteralName "ShouldFollow") false)
      (Variables|/Game/Object/Blueprints/Incendies/BP_Route_Guadian.BP_Route_Guadian_C|SetbIsOn (Variables|Default|GetSplineRoute) false))))

(fn ConstructionScript)