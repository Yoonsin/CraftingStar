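; AI controller for the FlameGuard monster NPC that runs its behavior tree on BeginPlay and tells it when to follow players.
; AI perception updates set the ShouldFollow blackboard key to true whenever a stimulus is successfully sensed.
; On a lost stimulus, it counts the CraftingStar characters among sight-perceived actors and clears the key only when none remain.
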(event OnTargetPerceptionUpdated(AIPerception)
  (params (Actor :type Actor%20Object%20Reference) (Stimulus :type AI%20Stimulus%20Structure))
  (CallFunction|CheckPlayerforSight (.bSuccessfullySensed (Utilities|Struct|BreakAIStimulus Stimulus))))

(event EventBeginPlay
  (AI|RunBehaviorTree "/Game/NPC/Monster/AI/BT_FlameGuard.BT_FlameGuard"))

(event EventTick
  (params (DeltaSeconds :type Float%20%28single-precision%29)))

(fn ConstructionScript)

(fn CheckPlayerforSight
  (params (Condition :type Boolean))
  (if Condition
    (AI|Components|Blackboard|SetValueasBool (Variables|Default|GetBlackboard) (Utilities|Name|MakeLiteralName "ShouldFollow") true)
    (else
      (Variables|Default|SetPerceptedCount 0)
      (for _array_element (Class|AIPerceptionComponent|GetPerceivedActors (Variables|Default|GetAIPerception) "/Script/AIModule.AISense_Sight")
        (Utilities|Casting|CastToBP_CraftingStarCharacter _array_element)
        (Math|Integer|IncrementInt (Variables|Default|GetPerceptedCount)))
      (if (<= (Variables|Default|GetPerceptedCount) 0)
        (AI|Components|Blackboard|SetValueasBool (Variables|Default|GetBlackboard) (Utilities|Name|MakeLiteralName "ShouldFollow") false)))))