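; AI controller for monsters that picks the nearest perceived player character as its target.
; Perception updates for BP_CraftingStarCharacter actors add to the RecognizedPlayers set when sensed, or call Remove on it otherwise.
; Each such update then finds the set's nearest actor to the controller's location and writes it and its distance to the Target and TargetDistance Blackboard keys.
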(event OnTargetPerceptionUpdated(AIPerception)
  (params (Actor :type Actor%20Object%20Reference) (Stimulus :type AI%20Stimulus%20Structure))
  (bind _recognizedplayers (Variables|Default|GetRecognizedPlayers))
  (bind _blackboard (Variables|Default|GetBlackboard))
  (bind _asbp_crafting_star_character (Utilities|Casting|CastToBP_CraftingStarCharacter Actor))
  (if (.bSuccessfullySensed (Utilities|Struct|BreakAIStimulus Stimulus))
    (Utilities|Set|Add _recognizedplayers _asbp_crafting_star_character)
    (else
      (Utilities|Set|Remove _recognizedplayers 0)))
  (bind _result (Utilities|Set|ToArray (Variables|Default|GetRecognizedPlayers)))
  (AI|Components|Blackboard|SetValueasObject _blackboard (Utilities|Name|MakeLiteralName "Target") (.ReturnValue (Actor|FindNearestActor (Transformation|GetActorLocation) _result)))
  (AI|Components|Blackboard|SetValueasFloat _blackboard (Utilities|Name|MakeLiteralName "TargetDistance") (.Distance (Actor|FindNearestActor (Transformation|GetActorLocation) _result))))

(event EventBeginPlay)

(event EventTick
  (params (DeltaSeconds :type Float%20%28single-precision%29)))

(fn ConstructionScript)