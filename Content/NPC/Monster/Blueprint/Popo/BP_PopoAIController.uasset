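; AI controller for the Popo monster NPC that runs BT_Popo and shows or hides its pawn on activation and deactivation.
; Perception updates pick a non-collapsed player as the blackboard FollowCharacter, refresh Destination from its location, and clear it when that player collapses.
; Check functions copy follow, sight and attack-range state onto BP_Popo.
; The sight check also updates patrol and follow keys but is not called within this graph.
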(event OnPerceptionUpdated(AIPerception)
  (params (UpdatedActors :type Array%20of%20Actor%20Object%20References))
  (CallFunction|CheckPlayerforActors UpdatedActors)
  (CallFunction|CheckPlayerinAttackRange)
  (CallFunction|CheckHasPopoFollowCharacter))

(event Custom|ActivatePopo
  (Rendering|SetActorHiddenInGame (Pawn|GetControlledPawn) false)
  (AI|RunBehaviorTree "/Game/NPC/Monster/AI/Popo/BT_Popo.BT_Popo"))

(event Custom|deactivatePopo
  (Rendering|SetActorHiddenInGame (Pawn|GetControlledPawn) true))

(event EventPossess
  (params (PossessedPawn :type Pawn%20Object%20Reference))
  (CallFunction|DeactivatePopo))

(event EventTick
  (params (DeltaSeconds :type Float%20%28single-precision%29)))

(event EventBeginPlay
  (CallFunction|ActivatePopo))

(fn ConstructionScript)

(fn CheckPlayerforActors
  (params (Actors :type Array%20of%20Actor%20Object%20References))
  (bind _array_element (Utilities|Array|ForEachLoopwithBreak Actors :!label _label)
    (:LoopBody
      (bind _asbp_crafting_star_character (Utilities|Casting|CastToBP_CraftingStarCharacter _array_element))
      (if (Variables|/Script/CraftingStar.CraftingStarCharacter|GetisCollapsed _asbp_crafting_star_character)
        ;[1 1 1] 감지된 쓰러진 캐릭터가 FollowCharacter인지 확인
        (if (== _asbp_crafting_star_character (AI|Components|Blackboard|GetValueasObject (Variables|Default|GetBlackboard) (Utilities|Name|MakeLiteralName "FollowCharacter")))
          (AI|Components|Blackboard|SetValueasObject (Variables|Default|GetBlackboard) (Utilities|Name|MakeLiteralName "FollowCharacter") 0))
        (else
          ;[1 1 1] 이미 따라가고 있는 캐릭터가 있는가?
          (if (Utilities|IsValid (AI|Components|Blackboard|GetValueasObject (Variables|Default|GetBlackboard) (Utilities|Name|MakeLiteralName "FollowCharacter")))
            ;[1 1 1] 있음: FollowCharacter 위치 업데이트
            (bind _asbp_crafting_star_character_2 (Utilities|Casting|CastToBP_CraftingStarCharacter (AI|Components|Blackboard|GetValueasObject (Variables|Default|GetBlackboard) (Utilities|Name|MakeLiteralName "FollowCharacter"))))
            (AI|Components|Blackboard|SetValueasVector (Variables|Default|GetBlackboard) (Utilities|Name|MakeLiteralName "Destination") (Transformation|GetActorLocation _asbp_crafting_star_character_2))
            (goto _label Break)
            (else
              ;[1 1 1] 없음: FollowCharacter 업데이트
              (AI|Components|Blackboard|SetValueasObject (Variables|Default|GetBlackboard) (Utilities|Name|MakeLiteralName "FollowCharacter") _asbp_crafting_star_character))))))))

(fn CheckPlayerinSight
  ;[1 1 1] 포포의 AI Perception에 Player 캐릭터가 감지되고 있는지 검사
  (bind _asbp_crafting_star_character (Utilities|Casting|CastToBP_CraftingStarCharacter (AI|Components|Blackboard|GetValueasObject (Variables|Default|GetBlackboard) (Utilities|Name|MakeLiteralName "FollowCharacter")))
    (:then
      (bind _info (Class|AIPerceptionComponent|GetActorsPerception (Variables|Default|GetAIPerception) _asbp_crafting_star_character))
      (if (.bSuccessfullySensed (Utilities|Struct|BreakAIStimulus (Utilities|Array|Get(acopy) (.LastSensedStimuli (Utilities|Struct|BreakActorPerceptionBlueprintInfo _info)))))
        _
        (else
          ;[1 1 1] 포포 정찰 설정
          (AI|Components|Blackboard|SetValueasBool (Variables|Default|GetBlackboard) (Utilities|Name|MakeLiteralName "IsPatrolling") false)))
      (bind _asbp_popo (Utilities|Casting|CastToBP_Popo (Pawn|GetControlledPawn)))
      (Variables|/Game/NPC/Monster/Blueprint/Popo/BP_Popo.BP_Popo_C|SetPlayerInSight _asbp_popo (and (.bSuccessfullySensed (Utilities|Struct|BreakAIStimulus (Utilities|Array|Get(acopy) (.LastSensedStimuli (Utilities|Struct|BreakActorPerceptionBlueprintInfo _info))))) (not (Variables|/Script/CraftingStar.CraftingStarCharacter|GetisCollapsed _asbp_crafting_star_character)))))
    (:CastFailed
      (AI|Components|Blackboard|SetValueasBool (Variables|Default|GetBlackboard) (Utilities|Name|MakeLiteralName "ShouldFollow") false))))

(fn CheckPlayerinAttackRange
  (bind _asbp_crafting_star_character (Utilities|Casting|CastToBP_CraftingStarCharacter (AI|Components|Blackboard|GetValueasObject (Variables|Default|GetBlackboard) (Utilities|Name|MakeLiteralName "FollowCharacter"))))
  (bind _asbp_popo (Utilities|Casting|CastToBP_Popo (Pawn|GetControlledPawn)))
  (Variables|/Game/NPC/Monster/Blueprint/Popo/BP_Popo.BP_Popo_C|SetPlayerInAttackRange _asbp_popo (and (not (Variables|/Script/CraftingStar.CraftingStarCharacter|GetisCollapsed _asbp_crafting_star_character)) (<= (Class|BlackboardComponent|GetValueasFloat (Variables|Default|GetBlackboard) (Utilities|Name|MakeLiteralName "DistanceFromTarget")) (Variables|Default|GetAttackDistance)))))

(fn CheckHasPopoFollowCharacter
  (bind _asbp_popo (Utilities|Casting|CastToBP_Popo (Pawn|GetControlledPawn)))
  (Variables|/Game/NPC/Monster/Blueprint/Popo/BP_Popo.BP_Popo_C|SetHasPopoFollowCharacter _asbp_popo (Utilities|IsValid (AI|Components|Blackboard|GetValueasObject (Variables|Default|GetBlackboard) (Utilities|Name|MakeLiteralName "FollowCharacter")))))