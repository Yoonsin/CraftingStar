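; BP_Popo is the Popo monster NPC that can attack players when berserk and resets the encounter once two are caught.
; Each tick derives the attack flag from visibility, sight, range, follow and berserk state, and has the server check catches, playing the GetKey sequence, teleporting Popo and reviving players at respawn points.
; Multicast show/hide toggles mesh, movement and blackboard pause.
; A construction-time GUID supports saving, and loading deactivates Popo through its AI controller.
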(event Custom|Server_HidePopo
  (CallFunction|MulticastHidePopo))

(event Custom|Multicast_ShowPopo
  (Development|PrintString "Show")
  (if (Networking|IsServer)
    (AI|Components|Blackboard|SetValueasBool (AI|GetBlackboard 0) (Utilities|Name|MakeLiteralName "PauseMovement") false))
  (Pawn|Components|CharacterMovement|SetMovementMode (Variables|Character|GetCharacterMovement) "MOVE_Walking" 0)
  (Rendering|SetVisibility (Variables|Character|GetMesh) true false)
  (Variables|AI|SetIsPopoHidden false))

(event Custom|Server_ShowPopo
  (CallFunction|MulticastShowPopo))

(event Custom|Multicast_HidePopo
  (Development|PrintString "Hide")
  (if (Networking|IsServer)
    (AI|Components|Blackboard|SetValueasBool (AI|GetBlackboard 0) (Utilities|Name|MakeLiteralName "PauseMovement") true))
  (Pawn|Components|CharacterMovement|DisableMovement (Variables|Character|GetCharacterMovement))
  (Rendering|SetVisibility (Variables|Character|GetMesh) false false)
  (Variables|AI|SetIsPopoHidden true))

(event EventBeginPlay)

(event Collision|EventActorBeginOverlap
  (params (OtherActor :type Actor%20Object%20Reference)))

(event EventTick
  (params (DeltaSeconds :type Float%20%28single-precision%29))
  (CallFunction|UpdateAttackCondition)
  (CallFunction|CheckCatchedAll))

(event EventLoadState
  (bind _asbp_popo_aicontroller (Utilities|Casting|CastToBP_PopoAIController (Pawn|GetController)))
  (Default|DeactivatePopo _asbp_popo_aicontroller))

(event EventSaveState
  (bind _ascrafting_star_gs (Utilities|Casting|CastToCraftingStarGS (Game|GetGameState)))
  (Utilities|Array|AddUnique (.WorldObjects (Utilities|Struct|BreakProgressData (Variables|/Script/CraftingStar.CraftingStarGS|GetProgressData _ascrafting_star_gs))) (Variables|세이브|GetID))
  (Class|UtilityFunction|Save (Game|GetGameInstance)))

(fn ConstructionScript
  (if (Utilities|Enum|Equal(Enum) (Variables|세이브|GetID) "")
    (Variables|세이브|SetID (Guid|ToString(Guid) (Guid|NewGuid)))))

(fn SetMaxWalkSpeed
  (params (newSpeed :type Float%20%28single-precision%29))
  (Variables|/Script/Engine.CharacterMovementComponent|SetMaxWalkSpeed (Variables|Character|GetCharacterMovement) newSpeed))

(fn UpdateAttackCondition
  (Variables|Attack|SetOnAttack (and (not (Variables|AI|GetIsPopoHidden)) (and (and (and (Variables|Attack|GetPlayerInSight) (Variables|Attack|GetPlayerInAttackRange)) (Variables|Attack|GetHasPopoFollowCharacter)) (Variables|AI|GetIsBerserk)))))

(fn CheckCatchedAll
  (if (Networking|IsServer)
    (bind _returnvalue (Class|Popo|CheckCatchedPlayerCnt))
    (if (== _returnvalue 2)
      ;[1 1 1] 포포 GetKey 시퀀스 재생
      (Networking|SwitchHasAuthority
        (:Authority
          (bind _asbp_crafting_star_gs (Utilities|Casting|CastToBP_CraftingStarGS (Game|GetGameState)))
          (Default|MultiCastPlaySequence _asbp_crafting_star_gs "/Game/Cinematics/Incendies/GetKey.GetKey")
          ;[1 1 1] 포포 위치 이동
          (Transformation|SetActorRelativeLocation (Variables|Incendie|GetBerserkPos) false true)
          ;[1 1 1] 플레이어 부활 및 위치 이동
          (bind _outactors (Actor|GetAllActorsOfClass "/Game/CraftingStarCharacter/BP_CraftingStarCharacter.BP_CraftingStarCharacter_C"))
          (bind _array_element (Utilities|Array|ForEachLoopwithBreak _outactors)
            (:LoopBody
              (Class|CraftingStarCharacter|OnRevivePopo _array_element)
              (Transformation|SetActorRelativeLocation _array_element (Variables|/Game/CraftingStarCharacter/BP_CraftingStarCharacter.BP_CraftingStarCharacter_C|GetRespawnPos_Popo _array_element) false true))))))))

(fn GetObjectID
  (return (Variables|세이브|GetID)))