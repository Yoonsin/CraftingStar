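; Sequencer director Blueprint holding the event-track handlers for the boss cinematic BossCinematics4.
; One event calls BreakWall on the bound BP_Broken_Main actor to break a wall during the sequence.
; Three others each activate a bound assimilation plate (L2, Last_L, Last_D) by unhiding its Niagara and spline Niagara effects and enabling query-only collision on its trigger.
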(event Custom|BP_Broken_Main_Event_0
  (params (BP_Broken_Main :type BP%20Broken%20Wall%20Object%20Reference))
  (Default|BreakWall BP_Broken_Main))

(event Custom|BP_AssimilationPlate_L2_Event_0
  (params (BP_AssimilationPlate_L2 :type BP%20Assimilation%20Plate%20Object%20Reference))
  (Development|SetHiddeninGame (Variables|/Game/Object/Blueprints/BP_AssimilationPlate.BP_AssimilationPlate_C|GetNiagara BP_AssimilationPlate_L2) false false)
  (Collision|SetCollisionEnabled (Variables|/Script/CraftingStar.AssimilationObject|GetTrigerComponent BP_AssimilationPlate_L2) "QueryOnly"))

(event Custom|BP_AssimilationPlate_Last_L_Event_0
  (params (BP_AssimilationPlate_Last_L :type BP%20Assimilation%20Plate%20Object%20Reference))
  (Development|SetHiddeninGame (Variables|/Game/Object/Blueprints/BP_AssimilationPlate.BP_AssimilationPlate_C|GetNiagara BP_AssimilationPlate_Last_L) false false)
  (Collision|SetCollisionEnabled (Variables|/Script/CraftingStar.AssimilationObject|GetTrigerComponent BP_AssimilationPlate_Last_L) "QueryOnly"))

(event Custom|BP_AssimilationPlate_Last_D_Event_0
  (params (BP_AssimilationPlate_Last_D :type BP%20Assimilation%20Plate%20Object%20Reference))
  (Development|SetHiddeninGame (Variables|/Game/Object/Blueprints/BP_AssimilationPlate.BP_AssimilationPlate_C|GetNiagara BP_AssimilationPlate_Last_D) false false)
  (Collision|SetCollisionEnabled (Variables|/Script/CraftingStar.AssimilationObject|GetTrigerComponent BP_AssimilationPlate_Last_D) "QueryOnly"))