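; Multiplayer boss character with falling-stone, knockback swing and stone-wall shield attacks, plus its widget and animation helpers.
; Authority-gated hits use a grace timer; every third makes it groggy and invincible via Blackboard until StoneShield spawns walls and clears invincibility.
; A hit while groggy destroys walls, plays a sequence and hides the boss.
; ProgressPhase updates the Blackboard pattern, rebinds sequence-end callbacks and plays cinematics or triggers the ending.
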(event Custom|PlaySequence
  (params (MultiLevelSequence :type Level%20Sequence%20Object%20Reference))
  ;[1 1 1] 시퀀서 재생
  (if (not (Variables|Default|GetbIsPlayingSequencer))
    (bind _returnvalue (Sequencer|Player|CreateLevelSequencePlayer MultiLevelSequence (Utilities|Struct|MakeMovieSceneSequencePlaybackSettings false "(Value=0)" 1.0 0.0 false false true true true true)))
    (EventDispatchers|BindEventtoOnFinished _returnvalue (delegate Custom|Play%20End))
    (Variables|Default|SetbIsPlayingSequencer true)
    (Sequencer|Player|Play _returnvalue :!class /Script/MovieScene.MovieSceneSequencePlayer)))

(event Custom|Groggy
  ;[1 1 1] 그로기
  (Networking|SwitchHasAuthority
    (:Authority
      (bind _output_get (Variables|Default|SetbIsGroggy true))
      (Variables|Default|SetbInvincible true)
      (AI|Components|Blackboard|SetValueasBool (AI|GetBlackboard (Pawn|GetController)) (Utilities|Name|MakeLiteralName "IsGroggy") _output_get))))

(event Custom|Play%20End
  ;[1 1 1] 시퀀서 재생
  (Variables|Default|SetbIsPlayingSequencer false)
  (Default|CallSequencerEndEvent))

(event Custom|Make%20Widget
  (Utilities|FlowControl|Delay 0.5)
  (UserInterface|Viewport|AddtoViewport (Variables|Widget|GetBossWidget) 0))

(event Custom|SequncerEndEvent_Event
  (Development|PrintString "End Boss Sequnece"))

(event Custom|Boss%20Die
  (Widget|RemovefromParent (Variables|Widget|GetBossWidget)))

(event Custom|ServerHit
  ;[0.1649 0.1649 0.1649] is Attacked
  (if (and (Variables|Damage|GetbCanDamage) (not (Variables|Default|GetbInvincible)))
    (if (Variables|Default|GetbIsGroggy)
      (CallFunction|HitatGroggy)
      (Variables|Damage|SetbCanDamage false)
      (Variables|Damage|SetRemainDamageTime (Variables|Damage|GetGracePeriod))
      (else
        (Variables|Damage|SetbCanDamage false)
        (Variables|Damage|SetRemainDamageTime (Variables|Damage|GetGracePeriod))
        (Development|PrintString "보스 Hit")
        (CallFunction|Damage)
        (bind _result (Math|Integer|IncrementInt (Variables|Damage|GetGroggyCount))
          (:%20%20
            (if (>= _result 3)
              (CallFunction|Groggy))))))))

(event Custom|Damage
  ;[1 0.2135 0.2135] Damage
  (if (Math|Random|RandomBool)
    (Animation|PlayAnimMontage "/Game/NPC/Monster/Blueprint/Boss/Animations/AM_Hit_Left_Boss.AM_Hit_Left_Boss" 1.0 "None")
    (else
      (Animation|PlayAnimMontage "/Game/NPC/Monster/Blueprint/Boss/Animations/AM_Hit_Right_Boss.AM_Hit_Right_Boss" 1.0 "None")))
  (Networking|SwitchHasAuthority
    (:Authority
      (Math|Float|DecrementFloat (Variables|Damage|GetHP)))))

(event EventBeginPlay
  (bind _returnvalue (UserInterface|CreateWidget "/Game/NPC/Monster/Blueprint/Boss/WBP_Boss.WBP_Boss_C" (Game|GetPlayerController 0) self))
  (Variables|Widget|SetBossWidget _returnvalue)
  (EventDispatchers|BindEventtoSequencerEndEvent (delegate Custom|SequncerEndEvent_Event)))

(event Collision|EventActorBeginOverlap
  (params (OtherActor :type Actor%20Object%20Reference)))

(event EventTick
  (params (DeltaSeconds :type Float%20%28single-precision%29))
  ;[1 1 1] 판정
  (if (not (Variables|Damage|GetbCanDamage))
    (bind _output_get (Variables|Damage|SetRemainDamageTime (- (Variables|Damage|GetRemainDamageTime) DeltaSeconds)))
    (if (< _output_get 0.0)
      (Variables|Damage|SetbCanDamage true))))

(event EventAttackbyTwoHanded
  (params (bLightCharacter :type Boolean))
  ;[0.1649 0.1649 0.1649] is Attacked
  (|SpawnParticle)
  (Networking|SwitchHasAuthority
    (:Authority
      (CallFunction|ServerHit))))

(event Custom|Spawn%20Stone
  (params (SpawnTransform :type Transform))
  ;[1 1 1] 멀티캐스트용
  (Game|SpawnActorfromClass "/Game/NPC/Monster/Blueprint/Boss/BP_FallingStone_Boss.BP_FallingStone_Boss_C" SpawnTransform "Undefined" 0 0))

(event Custom|Call%20Stone%20Attack
  ;[1 0.7299 0.277] 멀티캐스트용
  (bind _outactors (Actor|GetAllActorsOfClass "/Game/CraftingStarCharacter/BP_CraftingStarCharacter.BP_CraftingStarCharacter_C"))
  (bind _point (CallFunction|GetRandomCircle (Math|Vector|MakeVector (.X (Math|Vector|BreakVector (Transformation|GetActorLocation (.ReturnValue (Actor|FindNearestActor (Transformation|GetActorLocation) _outactors))))) (.Y (Math|Vector|BreakVector (Transformation|GetActorLocation (.ReturnValue (Actor|FindNearestActor (Transformation|GetActorLocation) _outactors))))) (+ (.Z (Math|Vector|BreakVector (Transformation|GetActorLocation (.ReturnValue (Actor|FindNearestActor (Transformation|GetActorLocation) _outactors))))) (Variables|Default|GetSpawnHeight))) 2e+02))
  (CallFunction|SpawnStone (Math|Transform|MakeTransform _point (Math|Random|RandomRotator false))))

(event Custom|Phase1
  (CallFunction|ShowBoss)
  (CallFunction|Ungroggy)
  (EventDispatchers|UnbindallEventsfromSequencerEndEvent))

(event Custom|Swing%20Attack
  (bind _returnvalue (Transformation|GetActorLocation))
  (bind _swinghitactorset (Variables|Default|GetSwingHitActorSet))
  (bind (_x _y _z) (Math|Vector|BreakVector _returnvalue))
  (bind _returnvalue_2 (- _z 2e+02))
  (bind _returnvalue_3 (Math|Vector|MakeVector _x _y _returnvalue_2))
  ;[1 0.7299 0.277] Swing Attack
  (bind _outhits (Collision|MultiSphereTraceForObjects _returnvalue_3 _returnvalue_3 5e+02 (Utilities|Array|MakeArray "ObjectTypeQuery3") false 0 "ForDuration" true "(R=1.000000,G=0.000000,B=0.904409,A=1.000000)" "(R=0.014835,G=0.000000,B=1.000000,A=1.000000)"))
  (for _array_element _outhits
    (Utilities|Set|Add (Variables|Default|GetSwingHitActorSet) (.HitActor (Collision|BreakHitResult _array_element))))
  (bind _result (Utilities|Set|ToArray _swinghitactorset))
  (for _array_element_2 _result
    (bind _ascrafting_star_character (Utilities|Casting|CastToCraftingStarCharacter _array_element_2))
    (bind _asbp_crafting_star_ps (Utilities|Casting|CastToBP_CraftingStarPS (Variables|/Script/Engine.Pawn|GetPlayerState _ascrafting_star_character)))
    (Class|CraftingStarPS|RequestHealth _asbp_crafting_star_ps 1e+01)
    (Character|LaunchCharacter _ascrafting_star_character (* (Math|Vector|MakeVector (.X (Math|Vector|BreakVector (- (Transformation|GetActorLocation _ascrafting_star_character) (Transformation|GetActorLocation)))) (.Y (Math|Vector|BreakVector (- (Transformation|GetActorLocation _ascrafting_star_character) (Transformation|GetActorLocation)))) 4e+02) (Variables|Default|GetSwingPower)) false false)
    (Animation|PlayAnimMontage _ascrafting_star_character (Variables|/Script/CraftingStar.CraftingStarCharacter|GetHitMontage_Popo _ascrafting_star_character) 1.0 "None"))
  (Utilities|Set|Clear _swinghitactorset))

(event Custom|Phase2)

(event Custom|Ungroggy
  ;[1 1 1] 그로기 해제
  (bind _output_get (Variables|Default|SetbIsGroggy false))
  (AI|Components|Blackboard|SetValueasBool (AI|GetBlackboard (AI|GetAIController self)) (Utilities|Name|MakeLiteralName "isGroggy") _output_get)
  (Variables|Damage|SetGroggyCount 0))

(event Custom|Multicast%20SequencerEnd%20Bind
  (params (Phase :type Integer))
  (EventDispatchers|UnbindallEventsfromSequencerEndEvent)
  (EventDispatchers|BindEventtoSequencerEndEvent (Utilities|Select :Index (- Phase 1) :Option%200 (delegate Custom|Phase1) :Option%201 (delegate Custom|Phase2) :Option%202 (delegate Custom|Phase2))))

(event Custom|StoneShield
  (bind _self self)
  ;[1 0.7299 0.277] Stone Shield
  ;;[1 1 1] 주변 캐릭터 날리기
  (CallFunction|SwingAttack)
  (Utilities|FlowControl|Delay 1.0)
  (bind _vector (CallFunction|GetCirclePoints (Transformation|GetActorLocation) 5e+02 10))
  (for _array_element _vector
    (bind _returnvalue (Game|SpawnActorfromClass "/Game/NPC/Monster/Blueprint/Boss/BP_StoneWall.BP_StoneWall_C" _array_element "AlwaysSpawn" _self _self 0))
    (bind _asbp_boss_controller_boss (Utilities|Casting|CastToBP_BossController_Boss (Pawn|GetController)))
    (Default|AddStoneWall _asbp_boss_controller_boss _returnvalue)
    (Variables|Default|SetbInvincible false)))

(event Custom|Call%20Line%20Attack
  ;[1 0.7299 0.277] 코멘트
  (for _index (range 1 10)
    (CallFunction|SpawnStone (Math|Transform|MakeTransform (Math|Vector|MakeVector (.X (Math|Vector|BreakVector (+ (Transformation|GetActorLocation) (* (Transformation|GetActorForwardVector) (* _index 3e+02))))) (.Y (Math|Vector|BreakVector (+ (Transformation|GetActorLocation) (* (Transformation|GetActorForwardVector) (* _index 3e+02))))) (+ (.Z (Math|Vector|BreakVector (+ (Transformation|GetActorLocation) (* (Transformation|GetActorForwardVector) (* _index 3e+02))))) (Variables|Default|GetSpawnHeight))) (Math|Random|RandomRotator false)))))

(event Custom|ProgressPhase
  ;[0.6927 0.7265 1] 다음 페이즈
  (Networking|SwitchHasAuthority
    (:Authority
      (bind _result (Math|Integer|IncrementInt (Variables|Default|GetBossPhase))
        (:%20%20
          (Class|BlackboardComponent|SetValueasInt (AI|GetBlackboard (AI|GetAIController self)) (Utilities|Name|MakeLiteralName "BossPattern") _result)
          (CallFunction|MulticastSequencerEndBind _result)
          (Development|PrintString (Utilities|String|ToString(Integer) _result))
          (switch int _result
            (:Default
              (Development|PrintString "WTF" true true "(R=1.000000,G=0.047707,B=0.000000,A=1.000000)" 1e+01))
            (:1
              (CallFunction|PlaySequence "/Game/NPC/Monster/Blueprint/Boss/BossCinematics2.BossCinematics2"))
            (:2
              (CallFunction|PlaySequence "/Game/Cinematics/Boss/DongHwaBoth.DongHwaBoth"))
            (:3
              (bind _returnvalue (Actor|GetActorOfClass "/Game/SFX/BGM/BGM_Director.BGM_Director_C"))
              (Default|StopMusic _returnvalue)
              (bind _asbp_crafting_star_gs (Utilities|Casting|CastToBP_CraftingStarGS (Game|GetGameState)))
              (Default|Ending _asbp_crafting_star_gs))))))))

(event Custom|HitAtGroggy
  ;[0.6927 0.7265 1] 다음 패턴
  (Networking|SwitchHasAuthority
    (:Authority
      (bind _asbp_boss_controller_boss (Utilities|Casting|CastToBP_BossController_Boss (AI|GetAIController self)))
      (for _array_element (Variables|/Game/NPC/Monster/Blueprint/Boss/BP_BossController_Boss.BP_BossController_Boss_C|GetRecognizedWalls _asbp_boss_controller_boss)
        (Utilities|IsValid _array_element
          (:Is%20Valid
            (Actor|DestroyActor _array_element))))
      (Utilities|FlowControl|Delay 0.5)
      (CallFunction|PlaySequence (Utilities|Select :Index (Variables|Default|GetBossPhase) :Option%200 "/Game/Cinematics/Boss/DongHwaDark.DongHwaDark" :Option%201 "/Game/Cinematics/Boss/DongHwaLight.DongHwaLight"))
      (Development|PrintString "보스 이동 로직" true true "(R=1.000000,G=0.853274,B=0.000000,A=1.000000)" 1e+01)
      (CallFunction|HideBoss))))

(event Custom|HideBoss
  ;[1 1 1] 코멘트
  (Rendering|SetVisibility (Variables|Character|GetMesh) false false)
  (Collision|SetCollisionEnabled (Variables|Collision|GetCapsuleComponent) "NoCollision"))

(event Custom|ShowBoss
  ;[1 1 1] 코멘트
  (Rendering|SetVisibility (Variables|Character|GetMesh) true false)
  (Collision|SetCollisionEnabled (Variables|Collision|GetCapsuleComponent) "QueryAndPhysics"))

(event Custom|StopAnimation
  (params (AnimMontage :type Anim%20Montage%20Object%20Reference))
  (Animation|StopAnimMontage AnimMontage))

(event Custom|PlayAnimation
  (params (AnimMontage :type Anim%20Montage%20Object%20Reference))
  (Animation|PlayAnimMontage AnimMontage 1.0 "None"))

(fn ConstructionScript)

(fn GetRandomCircle
  (params (Center :type Vector) (Radius :type Float%20%28single-precision%29))
  (bind _returnvalue (Math|Trig|GetPI))
  (bind _returnvalue_2 (Math|Random|RandomFloatinRange 0.0 1.0))
  (bind (_x _y _z) (Math|Vector|BreakVector Center))
  (bind _returnvalue_3 (Math|Float|Sqrt _returnvalue_2))
  (bind _returnvalue_4 (* 2.0 _returnvalue))
  (bind _returnvalue_5 (Math|Random|RandomFloatinRange 0.0 _returnvalue_4))
  (bind _returnvalue_6 (* Radius _returnvalue_3))
  (return (Math|Vector|MakeVector (+ _x (* (Math|Trig|Cos(Radians) _returnvalue_5) _returnvalue_6)) (+ _y (* (Math|Trig|Sin(Radians) _returnvalue_5) _returnvalue_6)) _z)))

(fn GetCirclePoints
  (params (Center :type Vector) (Radius :type Float%20%28single-precision%29) (Amount :type Integer))
  (Utilities|Array|Clear (LocalVariables|GetPointsTransform))
  (for _index (range 0 (- Amount 1))
    (Utilities|Array|Add (LocalVariables|GetPointsTransform) (Math|Transform|MakeTransform (+ Center (Math|Vector|MakeVector (* Radius (Math|Trig|Cos(Radians) (Math|Trig|DegreesToRadians (* _index (/ 3.6e+02 (Math|Conversions|ToFloat(Integer) Amount)))))) (* Radius (Math|Trig|Sin(Radians) (Math|Trig|DegreesToRadians (* _index (/ 3.6e+02 (Math|Conversions|ToFloat(Integer) Amount)))))) 0.0)) (Math|Rotator|MakeRotator 0.0 0.0 (+ (Math|Trig|RadiansToDegrees (Math|Trig|DegreesToRadians (* _index (/ 3.6e+02 (Math|Conversions|ToFloat(Integer) Amount))))) 2.7e+02)) "2.000000,2.000000,2.000000")))
  (return (LocalVariables|GetPointsTransform)))