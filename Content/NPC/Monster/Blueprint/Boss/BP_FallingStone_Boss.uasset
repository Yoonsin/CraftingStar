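; BP_FallingStone_Boss is a falling-stone boss hazard that reacts when its static mesh hits something.
; On hitting a BP_CraftingStarCharacter, it calls RequestHealth on the player state, prints health before and after, and plays the character's hit montage through MulticastPlayAnim.
; It then destroys itself, as it does on hitting any non-character, and EndPlay spawns an explosion emitter at the mesh location.
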(event OnComponentHit(StaticMesh)
  (params (HitComponent :type Primitive%20Component%20Object%20Reference) (OtherActor :type Actor%20Object%20Reference) (OtherComp :type Primitive%20Component%20Object%20Reference) (NormalImpulse :type Vector :default "0, 0, 0") (Hit :type Hit%20Result%20Structure%20%28by%20ref%29))
  (bind _asbp_crafting_star_character (Utilities|Casting|CastToBP_CraftingStarCharacter OtherActor)
    (:then
      (bind _asbp_crafting_star_ps (Utilities|Casting|CastToBP_CraftingStarPS (Variables|/Script/Engine.Pawn|GetPlayerState _asbp_crafting_star_character)))
      (Development|PrintString (Utilities|String|ToString(Float) (Variables|/Script/CraftingStar.CraftingStarPS|GetHealth _asbp_crafting_star_ps)) true true "(R=1.000000,G=0.483506,B=0.000000,A=1.000000)")
      (Class|CraftingStarPS|RequestHealth _asbp_crafting_star_ps 1e+01)
      (CallFunction|MulticastPlayAnim _asbp_crafting_star_character (Variables|/Script/CraftingStar.CraftingStarCharacter|GetHitMontage_Popo _asbp_crafting_star_character))
      (Development|PrintString (Utilities|String|ToString(Float) (Variables|/Script/CraftingStar.CraftingStarPS|GetHealth _asbp_crafting_star_ps)) true true "(R=1.000000,G=0.483506,B=0.000000,A=1.000000)")
      (Actor|DestroyActor))
    (:CastFailed
      (Actor|DestroyActor))))

(event Custom|MulticastPlayAnim
  (params (Character :type Character%20Object%20Reference) (AnimMontage :type Anim%20Montage%20Object%20Reference))
  (Animation|PlayAnimMontage Character AnimMontage 1.0 "None"))

(event EventBeginPlay)

(event Collision|EventActorBeginOverlap
  (params (OtherActor :type Actor%20Object%20Reference)))

(event EventTick
  (params (DeltaSeconds :type Float%20%28single-precision%29)))

(event EventEndPlay
  (params (EndPlayReason :type EEndPlayReason%20Enum :default "Destroyed"))
  (Effects|SpawnEmitteratLocation "/Game/Assets/BaseContent/StarterContent/Particles/P_Explosion.P_Explosion" (Transformation|GetWorldLocation (Variables|Default|GetStaticMesh))))

(event EventDestroyed)

(fn ConstructionScript)