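; BP_StoneWall is a stone wall actor tied to a boss monster through its OwnerBoss reference.
; Each tick, the authority checks the wall's distance to that boss and destroys the wall once it exceeds MaxDistance.
; On destruction, it spawns an enlarged, randomly rotated explosion particle effect at the mesh's world location.
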(event EventBeginPlay)

(event Collision|EventActorBeginOverlap
  (params (OtherActor :type Actor%20Object%20Reference)))

(event EventTick
  (params (DeltaSeconds :type Float%20%28single-precision%29))
  (Networking|SwitchHasAuthority
    (:Authority
      (if (> (Transformation|GetDistanceTo (Variables|Default|GetOwnerBoss)) (Variables|Default|GetMaxDistance))
        (Actor|DestroyActor)))))

(event EventEndPlay
  (params (EndPlayReason :type EEndPlayReason%20Enum :default "Destroyed")))

(event EventDestroyed
  (Effects|SpawnEmitteratLocation "/Game/Assets/BaseContent/StarterContent/Particles/P_Explosion.P_Explosion" (Transformation|GetWorldLocation (Variables|Default|GetActorMesh)) (Math|Random|RandomRotator false) "1.500000,1.500000,1.500000"))

(fn ConstructionScript)