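; AI controller for the boss monster that starts the BT_Boss behavior tree on BeginPlay.
; GetRandomCircle returns a random point around a center at the same height, using a random angle and square-root-scaled radius to spread points over the disc.
; CallStoneAttack is an empty stub, and nothing in this file calls either function.
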(event EventBeginPlay
  (AI|RunBehaviorTree "/Game/NPC/Monster/Blueprint/Boss/BT_Boss.BT_Boss"))

(event EventTick
  (params (DeltaSeconds :type Float%20%28single-precision%29)))

(fn ConstructionScript)

(fn CallStoneAttack)

(fn GetRandomCircle
  (params (Center :type Vector) (Radius :type Float%20%28single-precision%29))
  (bind _returnvalue (Math|Trig|GetPI))
  (bind _returnvalue_2 (Math|Random|RandomFloatinRange 0.0 1.0))
  (bind (_x _y _z) (Math|Vector|BreakVector Center))
  (bind _returnvalue_3 (Math|Float|Sqrt _returnvalue_2))
  (bind _returnvalue_4 (* 2.0 _returnvalue))
  (bind _returnvalue_5 (Math|Random|RandomFloatinRange 0.0 _returnvalue_4))
  (bind _returnvalue_6 (* Radius _returnvalue_3))
  (return (Math|Vector|MakeVector (+ _x (* (Math|Trig|Cos(Radians) _returnvalue_5) _returnvalue_6)) (+ _y (* (Math|Trig|Sin(Radians) _returnvalue_5) _returnvalue_6)) _z)))