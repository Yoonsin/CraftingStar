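; BP_Popo is a monster NPC character driven by BP_PopoAIController, with persistent world-object state.
; Its construction script assigns a GUID as ID when none is set, exposed through GetObjectID.
; SaveState adds that ID to the game state's saved world objects and triggers a save, while LoadState tells the AI controller to deactivate Popo.
; A helper function sets max walk speed.
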(event EventBeginPlay)

(event Collision|EventActorBeginOverlap
  (params (OtherActor :type Actor%20Object%20Reference)))

(event EventTick
  (params (DeltaSeconds :type Float%20%28single-precision%29)))

(event EventLoadState
  (bind _asbp_popo_aicontroller (Utilities|Casting|CastToBP_PopoAIController (Pawn|GetController)))
  (Default|DeactivatePopo _asbp_popo_aicontroller))

(event EventSaveState
  (bind _ascrafting_star_gs (Utilities|Casting|CastToCraftingStarGS (Game|GetGameState)))
  (Utilities|Array|AddUnique (.WorldObjects (Utilities|Struct|BreakProgressData (Variables|/Script/CraftingStar.CraftingStarGS|GetProgressData _ascrafting_star_gs))) (Variables|세이브|GetID))
  (Class|UtilityFunction|Save (Game|GetGameInstance)))

(fn ConstructionScript
  (if (Utilities|Enum|Equal(Enum) (Variables|세이브|GetID) "")
    (Variables|세이브|SetID (Guid|ToString(Guid) (Guid|NewGuid)))))

(fn SetMaxWalkSpeed
  (params (newSpeed :type Float%20%28single-precision%29))
  (Variables|/Script/Engine.CharacterMovementComponent|SetMaxWalkSpeed (Variables|Character|GetCharacterMovement) newSpeed))

(fn GetObjectID
  (return (Variables|세이브|GetID)))