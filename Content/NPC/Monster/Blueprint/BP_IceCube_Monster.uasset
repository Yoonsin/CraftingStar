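; Ice cube monster character with a health bar widget, a knockback attack and death handling.
; Two-handed hits lower HP, play a hit montage and open a grace period that Tick counts down.
; Attack sphere-traces nearby pawns, deduplicates them in a set and launches CraftingStarCharacters away and upward.
; Tick also turns the widget toward the camera and checks HP; on death the authority notifies MonsterSpawner after a delay, then destroys the actor.
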(event Custom|Attack
  (bind _returnvalue (Transformation|GetActorLocation))
  (bind _swinghitactorset (Variables|Attack|GetSwingHitActorSet))
  (bind _outhits (Collision|MultiSphereTraceForObjects _returnvalue _returnvalue 5e+02 (Utilities|Array|MakeArray "ObjectTypeQuery3") false 0 "ForDuration" true "(R=1.000000,G=0.000000,B=0.904409,A=1.000000)" "(R=0.014835,G=0.000000,B=1.000000,A=1.000000)"))
  (for _array_element _outhits
    (Utilities|Set|Add (Variables|Attack|GetSwingHitActorSet) (.HitActor (Collision|BreakHitResult _array_element))))
  (bind _result (Utilities|Set|ToArray _swinghitactorset))
  (for _array_element_2 _result
    (bind _ascrafting_star_character (Utilities|Casting|CastToCraftingStarCharacter _array_element_2))
    (Character|LaunchCharacter _ascrafting_star_character (* (Math|Vector|MakeVector (.X (Math|Vector|BreakVector (- (Transformation|GetActorLocation _ascrafting_star_character) (Transformation|GetActorLocation)))) (.Y (Math|Vector|BreakVector (- (Transformation|GetActorLocation _ascrafting_star_character) (Transformation|GetActorLocation)))) 4e+02) (Variables|Attack|GetSwingPower)) false false)
    (Development|PrintString (Utilities|String|ToString(Vector) (* (Math|Vector|MakeVector (.X (Math|Vector|BreakVector (- (Transformation|GetActorLocation _ascrafting_star_character) (Transformation|GetActorLocation)))) (.Y (Math|Vector|BreakVector (- (Transformation|GetActorLocation _ascrafting_star_character) (Transformation|GetActorLocation)))) 4e+02) (Variables|Attack|GetSwingPower)))))
  (Utilities|Set|Clear _swinghitactorset))

(event Custom|PlayAnimation
  (Animation|PlayAnimMontage (Variables|Animation|GetAttackAnimMontage) 1.0 "None"))

(event EventBeginPlay
  (bind _widget (Variables|Default|GetWidget))
  (Rendering|SetCastShadow _widget false)
  (bind _aswbp_monster_health (Utilities|Casting|CastToWBP_MonsterHealth (UserInterface|GetWidget _widget)))
  (Variables|/Game/NPC/Monster/Blueprint/WBP_MonsterHealth.WBP_MonsterHealth_C|SetMonster _aswbp_monster_health self))

(event Collision|EventActorBeginOverlap
  (params (OtherActor :type Actor%20Object%20Reference)))

(event EventTick
  (params (DeltaSeconds :type Float%20%28single-precision%29))
  (Utilities|FlowControl|Sequence
    (:then_0
      (|Damage DeltaSeconds))
    (:then_1
      (|WidgetGraph))
    (:then_2
      (|DieCheckGraph))))

(event EventAttackbyTwoHanded
  (params (bLightCharacter :type Boolean))
  (if (Variables|Damage|GetbCanDamage)
    (bind _result (Math|Float|DecrementFloat (Variables|Damage|GetHP))
      (:%20%20
        (Development|PrintString (Utilities|String|Append "HP: " (Utilities|String|ToString(Float) _result)))
        (Animation|PlayAnimMontage (Variables|Animation|GetHit%20Anim%20Montage) 1.0 "None")
        (Variables|Damage|SetRemainDamageTime (Variables|Damage|GetGracePeriod))
        (Variables|Damage|SetbCanDamage false)))))

(fn ConstructionScript)