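; AI controller for the Popo monster NPC, which stays hidden and inactive from possession until activated.
; ActivatePopo unhides the pawn and runs BT_Popo, while deactivatePopo hides it and stops the brain logic.
; Perception updates write the nearest updated actor and its location to the FollowCharacter and Destination blackboard keys.
; Despite the CheckPlayerForActors name, that selection does not filter for players.
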(event OnPerceptionUpdated(AIPerception)
  (params (UpdatedActors :type Array%20of%20Actor%20Object%20References))
  (CallFunction|CheckPlayerforActors UpdatedActors))

(event Custom|ActivatePopo
  (Rendering|SetActorHiddenInGame (Pawn|GetControlledPawn) false)
  (AI|RunBehaviorTree "/Game/NPC/Monster/AI/BT_Popo.BT_Popo"))

(event Custom|deactivatePopo
  (Rendering|SetActorHiddenInGame (Pawn|GetControlledPawn) true)
  (AI|Logic|StopLogic (Variables|Default|GetBrainComponent) "Popo Deactivate"))

(event EventPossess
  (params (PossessedPawn :type Pawn%20Object%20Reference))
  (CallFunction|DeactivatePopo))

(event EventTick
  (params (DeltaSeconds :type Float%20%28single-precision%29)))

(fn ConstructionScript)

(fn CheckPlayerforActors
  (params (Actors :type Array%20of%20Actor%20Object%20References))
  (bind _returnvalue (Pawn|GetControlledPawn))
  (bind _returnvalue_2 (Transformation|GetActorLocation _returnvalue))
  (bind _returnvalue_3 (Actor|FindNearestActor _returnvalue_2 Actors))
  (AI|Components|Blackboard|SetValueasObject (Variables|Default|GetBlackboard) (Utilities|Name|MakeLiteralName "FollowCharacter") _returnvalue_3)
  (AI|Components|Blackboard|SetValueasVector (Variables|Default|GetBlackboard) (Utilities|Name|MakeLiteralName "Destination") (Transformation|GetActorLocation _returnvalue_3)))