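; AI controller for a prison monster NPC that chases the nearest player it currently perceives.
; AI Perception updates add a sensed BP_CraftingStarCharacter to a RecognizedPlayers set and remove it when sensing fails.
; Every tick it finds the closest recognized player to the controlled pawn and issues AI MoveTo toward them with an acceptance radius, without a behavior tree.
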(event OnTargetPerceptionUpdated(AIPerception)
  (params (Actor :type Actor%20Object%20Reference) (Stimulus :type AI%20Stimulus%20Structure))
  (bind _recognizedplayers (Variables|Default|GetRecognizedPlayers))
  (bind _asbp_crafting_star_character (Utilities|Casting|CastToBP_CraftingStarCharacter Actor))
  (if (.bSuccessfullySensed (Utilities|Struct|BreakAIStimulus Stimulus))
    (Utilities|Set|Add _recognizedplayers _asbp_crafting_star_character)
    (else
      (Utilities|Set|Remove _recognizedplayers 0))))

(event EventBeginPlay)

(event EventTick
  (params (DeltaSeconds :type Float%20%28single-precision%29))
  (bind _returnvalue (Pawn|GetControlledPawn))
  (bind _result (Utilities|Set|ToArray (Variables|Default|GetRecognizedPlayers)))
  (Utilities|IsValid (.ReturnValue (Actor|FindNearestActor (Transformation|GetActorLocation _returnvalue) _result))
    (:Is%20Valid
      (AI|AIMoveTo _returnvalue "0, 0, 0" (.ReturnValue (Actor|FindNearestActor (Transformation|GetActorLocation _returnvalue) _result)) 1.5e+02 false))))

(fn ConstructionScript)