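; BP_MainMenuPC is the player controller for the main menu.
; On BeginPlay it shows the mouse cursor, then creates the WBP_MainMenu widget and adds it to the viewport.
; Hosting is relayed from a client host event to a server host event, which asks BP_CraftingStarGameInstance to host with this controller and an empty server name.
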(event Custom|Client_HostGame
  (CallFunction|ServerHostGame))

(event Custom|Server_HostGame
  (bind _asbp_crafting_star_game_instance (Utilities|Casting|CastToBP_CraftingStarGameInstance (Game|GetGameInstance)))
  (Default|Host _asbp_crafting_star_game_instance self))

(event EventBeginPlay
  (Variables|Default|SetbShowMouseCursor true)
  (bind _returnvalue (UserInterface|CreateWidget "/Game/UI/Tutorial/MainMenu/WidgetBlueprints/WBP_MainMenu.WBP_MainMenu_C" (Game|GetPlayerController 0)))
  (UserInterface|Viewport|AddtoViewport _returnvalue 0))

(event EventTick
  (params (DeltaSeconds :type Float%20%28single-precision%29)))

(fn ConstructionScript)