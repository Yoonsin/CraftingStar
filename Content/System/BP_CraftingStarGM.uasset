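; Game mode for CraftingStar that restores saved world and quest progress and handles player login.
; World loading picks a class list by map name, then calls LoadState on NeedToSave actors whose IDs appear in the save.
; Quest loading matches the saved quest ID to play a Megeton, Incendie or boss sequence through a GameState multicast.
; PostLogin clears a reconnect timer when LogoutFlag is set; logout session teardown is unwired.
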(event EventOnLogout
  (params (ExitingController :type Controller%20Object%20Reference))
  ;[1 1 1] 로그아웃
  (bind _ascrafting_star_pc (Utilities|Casting|CastToCraftingStarPC ExitingController))
  (bind _returnvalue (Class|UtilityFunction|IsHost _ascrafting_star_pc))
  (if _returnvalue
    _))

(event EventPostLogin
  (params (NewPlayer :type Player%20Controller%20Object%20Reference))
  (bind _reconnecttimerhandle (Variables|접속|GetReconnectTimerHandle))
  ;[1 1 1] 로그인
  (if (Variables|접속|GetLogoutFlag)
    (Variables|접속|SetLogoutFlag true)
    (Development|PrintString "ReConnect")
    (if (Utilities|Time|IsValidTimerHandle _reconnecttimerhandle)
      (Utilities|Time|ClearandInvalidateTimerbyHandle _reconnecttimerhandle))))

(event EventLoadWorldData
  (params (saveGame :type Crafting%20Star%20Save%20Game%20Object%20Reference))
  (bind _progressdata (Variables|/Script/CraftingStar.CraftingStarSaveGame|GetProgressData saveGame))
  (bind _loadclassarr_megeton (Variables|로드데이터|GetLoadClassArr_Megeton))
  ;[1 1 1] 월드 상태 로드
  (for _array_element (Utilities|Select :Index (.nowmapname _progressdata) :EWorldMap _loadclassarr_megeton :EKeyStar _loadclassarr_megeton :EFlameAndIceStar (Variables|로드데이터|GetLoadClassArr_Incendie) :EBossMap 0)
    (로드데이터|ChangeStateObject (.worldobjects _progressdata) _array_element)
    (bind _asbp_crafting_star_character (Utilities|Casting|CastToBP_CraftingStarCharacter (Game|GetPlayerCharacter 0)))
    (Default|MultiSetVisibleUIInteractable _asbp_crafting_star_character "Collapsed")))

(event EventLoadQuestData
  (params (saveGame :type Crafting%20Star%20Save%20Game%20Object%20Reference))
  ;[1 1 1] 퀘스트 상태 로드
  (switch Utilities|FlowControl|Switch|SwitchonEQuestID (.questid (Variables|/Script/CraftingStar.CraftingStarSaveGame|GetProgressData saveGame))
    (:EMegetonNotMeet
      (|LoadQuestDataMegeton))
    (:EIncendieStartMovie
      (로드데이터|LoadQuestDataIncendie (Variables|/Script/CraftingStar.CraftingStarSaveGame|GetProgressData saveGame)))
    (:EBossInStart
      (|LoadQuestDataBoss))))

(fn ConstructionScript)

(fn LoadQuestDataIncendie
  (params (ProgressData :type Progress%20Data%20Structure%20%28by%20ref%29))
  (Utilities|Struct|SetmembersinProgressData ProgressData "EIncendiePengdoNotMeet")
  (bind _asbp_crafting_star_gs (Utilities|Casting|CastToBP_CraftingStarGS (Game|GetGameState)))
  (Utilities|Struct|SetmembersinProgressData (Variables|/Script/CraftingStar.CraftingStarGS|GetProgressData _asbp_crafting_star_gs) "EIncendiePengdoNotMeet")
  (Default|MultiCastPlaySequence _asbp_crafting_star_gs "/Game/Cinematics/Incendies/GameStart.GameStart"))

(fn ChangeStateObject
  (params (TargetArray :type Array%20of%20Strings) (ClassName :type Actor%20Class%20Reference))
  (bind _outactors (Actor|GetAllActorsOfClass ClassName))
  (for _array_element _outactors
    (bind _asneed_to_save (Utilities|Casting|CastToNeedToSave _array_element))
    (bind _id (Default|GetObjectID _asneed_to_save))
    (if (Utilities|Array|ContainsItem TargetArray _id)
      (Default|LoadState _asneed_to_save))))