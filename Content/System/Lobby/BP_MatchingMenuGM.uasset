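; Game mode for the matchmaking lobby menu, handling client joins and departures and moving the session to a level.
; PostLogin and OnLogout filter out the host and fire CallPostLogin or CallLogOut only for other players.
; TravelTo builds a servertravel console command with the Listen option to open the named level as a listen server.
; DestroySession chains remain in the graph but never run.
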(event Custom|Travel%20To
  (params (Level%20Name :type String))
  (Development|ExecuteConsoleCommand (Utilities|String|Append "servertravel " Level%20Name "?Listen") 0))

(event EventBeginPlay)

(event EventTick
  (params (DeltaSeconds :type Float%20%28single-precision%29)))

(event EventPostLogin
  (params (NewPlayer :type Player%20Controller%20Object%20Reference))
  (bind _returnvalue (Class|UtilityFunction|IsHost NewPlayer))
  (if (not _returnvalue)
    (Default|CallPostLogin)))

(event EventOnLogout
  (params (ExitingController :type Controller%20Object%20Reference))
  (bind _returnvalue (Class|UtilityFunction|IsHost ExitingController))
  (if (not _returnvalue)
    (Default|CallLogOut)))

(fn ConstructionScript)