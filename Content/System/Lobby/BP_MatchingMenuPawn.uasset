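; Pawn for the matchmaking menu that gives keyboard access to the friend list and invite UI.
; P uses a FlipFlop to create and show a new WBP_FriendList with the mouse cursor, then remove it, leaving the cursor visible.
; N passes the owning PlayerController to ShowInviteUI and prints placeholder debug text on success or failure.
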(event EventBeginPlay)

(event Collision|EventActorBeginOverlap
  (params (OtherActor :type Actor%20Object%20Reference)))

(event EventTick
  (params (DeltaSeconds :type Float%20%28single-precision%29)))

(event Input|KeyboardEvents|N
  (params (Key :type Key%20Structure :default "None"))
  (:Pressed
    (bind _asplayer_controller (Utilities|Casting|CastToPlayerController (Pawn|GetController)))
    (Class|AdvancedExternalUILibrary|ShowInviteUI _asplayer_controller
      (:OnSuccess
        (Development|PrintString "Hello"))
      (:OnFailure
        (Development|PrintString "Not Hello")))))

(event Input|KeyboardEvents|P
  (params (Key :type Key%20Structure :default "None"))
  (:Pressed
    (Utilities|FlowControl|FlipFlop
      (:A
        (bind _returnvalue (UserInterface|CreateWidget "/Game/UI/Lobby/WBP_FriendList.WBP_FriendList_C"))
        (Variables|Default|SetWB%20Friends%20List _returnvalue)
        (UserInterface|Viewport|AddtoViewport _returnvalue 0)
        (Variables|/Script/Engine.PlayerController|SetbShowMouseCursor (Game|GetPlayerController 0) true))
      (:B
        (Widget|RemovefromParent (Variables|Default|GetWB%20Friends%20List))))))

(fn ConstructionScript)