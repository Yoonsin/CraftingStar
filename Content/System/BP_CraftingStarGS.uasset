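; Game state for the two-player CraftingStar game, coordinating cutscenes, quest-driven world changes and map travel.
; Level sequences pause the local character and hide interaction and dialogue UI until finished, with separate server and client handling.
; Quest IDs trigger unlocking doors, activating portals, waking Popo or spawning guardians, finding actors by class and name substring.
; It also teleports host and guest, shows the ending, and saves progress before portal travel except in debug.
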(event Custom|ActiveObject
  (params (NowQuestID :type EQuestID%20Enum%20%28by%20ref%29 :default "EMegetonNotMeet"))
  ;[1 1 1] 퀘스트 라인에 따른 오브젝트 활성화
  (switch Utilities|FlowControl|Switch|SwitchonEQuestID NowQuestID
    (:EMegetonMeet
      (퀘스트오브젝트활성화|ActiveObjectMegetonMeet))
    (:EMegetonGetKey
      (퀘스트오브젝트활성화|ActiveObjectMegetonGetKey))
    (:EMegetonClear
      (퀘스트오브젝트활성화|ActiveObjectMegetonClear))
    (:EIncendiePengdoNotMeet
      (퀘스트오브젝트활성화|ActiveObjectPengdoNotMeet))
    (:EIncendieClacierNotMeetAndPopoBerserk
      (퀘스트오브젝트활성화|ActiveObjectClacierNotMeet))
    (:EIncendieRescueFrameGuardian
      (퀘스트오브젝트활성화|ActiveObjectResqueFrame))
    (:EIncendieRescueIncendie
      (CallFunction|ActiveObjectResqueIncendie))))

(event Custom|BP_MultiCastPlaySequence
  (params (Sequence :type Level%20Sequence%20Object%20Reference))
  ;[1 1 1] 시퀀스 재생
  (Variables|시퀀스|SetisPlayed false)
  (bind _returnvalue (Sequencer|Player|CreateLevelSequencePlayer Sequence))
  (EventDispatchers|BindEventtoOnFinished _returnvalue (delegate Custom|Finished))
  (bind _asbp_crafting_star_character (Utilities|Casting|CastToBP_CraftingStarCharacter (Game|GetPlayerCharacter 0)))
  (Default|SetVisibleUIInteractable _asbp_crafting_star_character "Collapsed" _asbp_crafting_star_character)
  (Class|CraftingStarCharacter|SetPause _asbp_crafting_star_character true)
  (if (Networking|IsServer)
    (Default|ServerSetVisible _asbp_crafting_star_character false)
    (bind _asdialog_widget (Utilities|Casting|CastToDialogWidget (Variables|/Game/CraftingStarCharacter/BP_CraftingStarCharacter.BP_CraftingStarCharacter_C|GetDialogWidget _asbp_crafting_star_character))
      (:then
        (Default|Disappeartemporarily _asdialog_widget))
      (:CastFailed
        _))
    (else
      (Variables|시퀀스|SetisPlayed_Client false)
      (bind _asdialog_widget_client (Utilities|Casting|CastToDialogWidget_client (Variables|/Game/CraftingStarCharacter/BP_CraftingStarCharacter.BP_CraftingStarCharacter_C|GetDialogWidget _asbp_crafting_star_character))
        (:then
          (Default|Disappeartemporarily _asdialog_widget_client))
        (:CastFailed
          _))))
  (Sequencer|Player|Play _returnvalue :!class /Script/MovieScene.MovieSceneSequencePlayer))

(event Custom|Finished
  ;[1 1 1] 시퀀스 재생
  (bind _asbp_crafting_star_character (Utilities|Casting|CastToBP_CraftingStarCharacter (Game|GetPlayerCharacter 0)))
  (Default|SetUIInteractable _asbp_crafting_star_character)
  (Class|CraftingStarCharacter|SetPause _asbp_crafting_star_character false)
  (if (Networking|IsServer)
    (bind _asdialog_widget (Utilities|Casting|CastToDialogWidget (Variables|/Game/CraftingStarCharacter/BP_CraftingStarCharacter.BP_CraftingStarCharacter_C|GetDialogWidget _asbp_crafting_star_character))
      (:then
        (Default|Appear _asdialog_widget))
      (:CastFailed
        _))
    (Variables|시퀀스|SetisPlayed true)
    (else
      (bind _asdialog_widget_client (Utilities|Casting|CastToDialogWidget_client (Variables|/Game/CraftingStarCharacter/BP_CraftingStarCharacter.BP_CraftingStarCharacter_C|GetDialogWidget _asbp_crafting_star_character))
        (:then
          (Default|Appear _asdialog_widget_client))
        (:CastFailed
          _))
      (Variables|시퀀스|SetisPlayed_Client true)
      (Default|ServerSetVisible _asbp_crafting_star_character true))))

(event Custom|MultiRemovePlayerWidget
  ;[1 1 1] 모든 플레이어 위젯 삭제
)

(event Custom|Ending
  ;[1 1 1] 시퀀스 재생
  (bind _returnvalue (UserInterface|CreateWidget "/Game/UI/Ending/WBP_Ending.WBP_Ending_C" (Game|GetPlayerController 0)))
  (UserInterface|Viewport|AddtoViewport _returnvalue 0)
  (Default|PlayEnding _returnvalue))

(event EventBeginPlay
  ;[1 1 1] 시퀀스 재생
)

(event EventTick
  (params (DeltaSeconds :type Float%20%28single-precision%29))
  ;[1 1 1] Tick
  (if (Networking|IsServer)
    (if (and (Variables|Default|GetisHostObtain) (Variables|Default|GetisGuestObtain))
      (Variables|Default|SetisHostObtain false)
      (Variables|Default|SetisGuestObtain false)
      (Variables|Default|SetnowObtainingAbility "ENone"))
    (elif (Variables|시퀀스|GetisPlayed_Client)
      (Variables|시퀀스|SetisPlayed_Client false))))

(event EventMultiCastPlaySequence
  (params (Sequence :type Level%20Sequence%20Object%20Reference))
  ;[1 1 1] 시퀀스 재생
  (CallFunction|MultiCastPlaySequence Sequence))

(fn ConstructionScript)

(fn OnRepDialogTextReplicates)

(fn OnRepIsSpeak?)

(fn OnRepDialogSpeakTextReplicates)

(fn OnRepSelectRepliesNum)

(fn OnRepIsHoveredReply)

(fn OnRepSelectReplies)

(fn OnRepIsPlayed)

(fn OnRepIsPlaying)

(fn ActiveObjectMegetonGetKey
  (bind _outactors (Actor|GetAllActorsOfClass "/Game/Object/Blueprints/BP_Gate.BP_Gate_C"))
  (for _array_element _outactors
    (if (Utilities|String|Contains (Utilities|GetDisplayName _array_element) "BP_EndGate")
      (Default|SaveState _array_element))))

(fn ActiveObjectMegetonMeet
  (bind _outactors (Actor|GetAllActorsOfClass "/Game/Object/Blueprints/Megeton/BP_Wall.BP_Wall_C"))
  (for _array_element _outactors
    (bind _asneed_to_save (Utilities|Casting|CastToNeedToSave _array_element))
    (if (Utilities|String|Contains (Utilities|GetDisplayName _array_element) "BP_Wall")
      (Default|SaveState _asneed_to_save))))

(fn ActiveObjectMegetonClear
  (bind _outactors (Actor|GetAllActorsOfClass "/Game/Object/Blueprints/Megeton/BP_Gate_MegetonPortal.BP_Gate_MegetonPortal_C"))
  (for _array_element _outactors
    (if (Utilities|String|Contains (Utilities|GetDisplayName _array_element) "BP_EndGate")
      (Default|SetActivePortal _array_element true))))

(fn ActiveObjectClacierNotMeet
  (bind _outactors (Actor|GetAllActorsOfClass "/Game/Object/Blueprints/Incendies/BP_Door_VillageHouse.BP_Door_VillageHouse_C"))
  (bind _array_element (Utilities|Array|ForEachLoopwithBreak _outactors :!label _label)
    (:LoopBody
      (if (Utilities|String|Contains (Utilities|GetObjectName _array_element) "BP_Door_VillageHouse_F")
        (Variables|/Game/Object/Blueprints/Incendies/BP_Door_VillageHouse.BP_Door_VillageHouse_C|SetbIsLocked _array_element false)
        (Default|SaveState _array_element)
        (goto _label Break)))
    (:Completed
      (Development|PrintString "파욱스 문 잠김 해제"))))

(fn ActiveObjectResqueFrame
  (bind _outactors (Actor|GetAllActorsOfClass "/Game/Object/Blueprints/Incendies/BP_Door_Fence.BP_Door_Fence_C"))
  (bind _array_element (Utilities|Array|ForEachLoopwithBreak _outactors :!label _label)
    (:LoopBody
      (if (Utilities|String|Contains (Utilities|GetObjectName _array_element) "SM_fence")
        (Variables|/Game/Object/Blueprints/Incendies/BP_Door_Fence.BP_Door_Fence_C|SetisLocked _array_element false)
        (Default|SaveState _array_element)
        (goto _label Break)))
    (:Completed
      (bind _outactors_2 (Actor|GetAllActorsOfClass "/Game/Object/Blueprints/Incendies/BP_FrameGaudianSpawner.BP_FrameGaudianSpawner_C"))
      (bind _array_element_2 (Utilities|Array|ForEachLoopwithBreak _outactors_2 :!label _label_2)
        (:LoopBody
          (if (Utilities|String|Contains (Utilities|GetObjectName _array_element_2) "BP_FGSpawner")
            (Default|SpawnFrameGaudian _array_element_2)
            (Default|SaveState _array_element_2)
            (goto _label_2 Break)))))))

(fn ActiveObjectPengdoNotMeet
  (bind _outactors (Actor|GetAllActorsOfClass "/Game/NPC/Monster/Blueprint/Popo/BP_Popo.BP_Popo_C"))
  (for _array_element _outactors
    (if (Utilities|String|Contains (Utilities|GetObjectName _array_element) "BP_Popo")
      (bind _asbp_popo_aicontroller (Utilities|Casting|CastToBP_PopoAIController (Pawn|GetController _array_element)))
      (Default|ActivatePopo _asbp_popo_aicontroller)
      (Default|SaveState _array_element))))

(fn MoveCharacter
  (params (Host%20Transform :type Transform) (GuestTransforl :type Transform))
  (LocalVariables|SetHost Host%20Transform)
  (LocalVariables|SetGuest GuestTransforl)
  (for _array_element (Variables|Default|GetPlayerArray)
    (bind _asplayer_controller (Utilities|Casting|CastToPlayerController (Components|GetOwner _array_element)))
    (bind _asbp_crafting_star_character (Utilities|Casting|CastToBP_CraftingStarCharacter (Pawn|GetControlledPawn _asplayer_controller)))
    (bind _returnvalue (Class|UtilityFunction|IsHost _asplayer_controller))
    (if _returnvalue
      (Transformation|SetWorldTransform (Variables|/Script/Engine.Character|GetCapsuleComponent _asbp_crafting_star_character) (LocalVariables|GetHost) false true)
      (else
        (Transformation|SetWorldTransform (Variables|/Script/Engine.Character|GetCapsuleComponent _asbp_crafting_star_character) (LocalVariables|GetGuest) false true)))))

(fn ActiveObjectResqueIncendie)

(fn OpenPortal
  (Variables|Default|SetNextMapName (Utilities|Select :Index (.nowmapname (Variables|Default|GetProgressData)) :EWorldMap "" :EKeyStar "L_Map_incendie" :EFlameAndIceStar "L_BossMap" :EBossMap "L_BossMap"))
  (bind _asbp_crafting_star_game_instance (Utilities|Casting|CastToBP_CraftingStarGameInstance (Game|GetGameInstance)))
  ;[1 1 1] 디버그 (인게임 맵에서 바로 시작) 시에는 세이브 파일 저장 x
  (Variables|Default|SetProgressData (Utilities|Struct|MakeProgressData (Utilities|Select :Index (.nowmapname (Variables|Default|GetProgressData)) :EWorldMap "EKeyStar" :EKeyStar "EFlameAndIceStar" :EFlameAndIceStar "EBossMap" :EBossMap "EWorldMap") (.HostPlayerPos (Utilities|Struct|BreakSpawnTransform (.Value (Utilities|Map|Find (Variables|/Script/CraftingStar.CraftingStarGameInstance|GetMapSpawnDict _asbp_crafting_star_game_instance) (Utilities|Select :Index (.nowmapname (Variables|Default|GetProgressData)) :EWorldMap "EKeyStar" :EKeyStar "EFlameAndIceStar" :EFlameAndIceStar "EBossMap" :EBossMap "EWorldMap"))))) (.GuestPlayerPos (Utilities|Struct|BreakSpawnTransform (.Value (Utilities|Map|Find (Variables|/Script/CraftingStar.CraftingStarGameInstance|GetMapSpawnDict _asbp_crafting_star_game_instance) (Utilities|Select :Index (.nowmapname (Variables|Default|GetProgressData)) :EWorldMap "EKeyStar" :EKeyStar "EFlameAndIceStar" :EFlameAndIceStar "EBossMap" :EBossMap "EWorldMap"))))) 0 (Utilities|Select :Index (.questid (Variables|Default|GetProgressData)) :EMegetonNotMeet "EMegetonNotMeet" :EMegetonMeet "EMegetonNotMeet" :EMegetonGetKey "EMegetonNotMeet" :EMegetonClear "EMegetonTransition" :EMegetonTransition "EMegetonTransition" :EIncendieStartMovie "EMegetonNotMeet" :EIncendiePengdoNotMeet "EMegetonNotMeet" :EIncendiePengdoMeet "EMegetonNotMeet" :EIncendieClacierNotMeetAndPopoBerserk "EMegetonNotMeet" :EIncendieClacierMeet "EMegetonNotMeet" :EIncendieRescueFrameGuardian "EMegetonNotMeet" :EIncendieExploreForest "EMegetonNotMeet" :EIncendieArriveTheEndOfForest "EMegetonNotMeet" :EIncendiePuzzleClear "EMegetonNotMeet" :EIncendieRescueIncendie "EIncendieTransition" :EIncendieTransition "EIncendieTransition" :EBossInStart "EBossInStart" :EBossInBattle "EBossInStart" :EBossInDefeated "EBossInStart") 0))
  (if (Variables|/Script/CraftingStar.CraftingStarGameInstance|GetisDebug _asbp_crafting_star_game_instance)
    (Default|Travelto _asbp_crafting_star_game_instance (Variables|Default|GetNextMapName) :!label _label)
    (else
      (bind _returnvalue (Class|UtilityFunction|Save _asbp_crafting_star_game_instance))
      (if _returnvalue
        (goto _label)))))