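; Game instance for CraftingStar, a two-player host/guest game, handling sessions, map travel and save data.
; Host, marked for deprecation, creates an Advanced Sessions LAN session and opens the matching menu as a listen server; TravelTo moves players via servertravel.
; SetDebugData seeds a missing save with dark host and light guest players at world-map spawns.
; Network-error and invite events are empty, their former logout-widget, friend and join logic left disconnected.
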(event Custom|Host
  (params (PlayerController :type Player%20Controller%20Object%20Reference) (ServerName :type String))
  ;[1 1 1] 폐기 예정
  (|AdvancedSession 0 PlayerController 100 100 true true false true true true false false false true
    (:OnSuccess
      (Development|PrintString "Host Create Session")
      (Game|OpenLevel(byObjectReference) "/Game/Maps/L_MatchingMenu.L_MatchingMenu" true "listen"))))

(event Custom|RemoveLogout
  (bind _logoutserverwidgetref (Variables|세이브|GetLogOutServerWidgetRef))
  ;[1 1 1] 서버가 나갔을 시 -> 클라이언트에서 불릴 함수
  (Utilities|IsValid _logoutserverwidgetref
    (:Is%20Valid
      (Widget|RemovefromParent _logoutserverwidgetref))))

(event EventHandleNetworkError
  (params (FailureType :type ENetworkFailure%20Enum :default "NetDriverAlreadyExists") (bIsServer :type Boolean))
  ;[1 1 1] 서버가 나갔을 시 -> 클라이언트에서 불릴 함수
)

(event EventOnSessionInviteAccepted
  (params (LocalPlayerNum :type Integer) (PersonInvited :type BP%20Unique%20Net%20Id%20Structure) (SessionToJoin :type Blueprint%20Session%20Result%20Structure%20%28by%20ref%29))
  ;[1 1 1] 폐기 예정
)

(event EventOnSessionInviteReceived
  (params (LocalPlayerNum :type Integer) (PersonInviting :type BP%20Unique%20Net%20Id%20Structure) (AppId :type String) (SessionToJoin :type Blueprint%20Session%20Result%20Structure%20%28by%20ref%29))
  ;[1 1 1] 폐기 예정
)

(fn SetDebugData
  (bind _mapspawndict (Variables|Default|GetMapSpawnDict))
  (bind _value (Utilities|Map|Find _mapspawndict "EWorldMap"))
  (bind (_hostplayerpos _guestplayerpos) (Utilities|Struct|BreakSpawnTransform _value))
  (Utilities|IsValid (Variables|Default|GetnowSaveGame)
    (:Is%20Not%20Valid
      (bind _returnvalue (SaveGame|CreateSaveGameObject "/Script/CraftingStar.CraftingStarSaveGame"))
      ;[1 1 1] 초기 데이터 생성
      (Variables|/Script/CraftingStar.CraftingStarSaveGame|SetHostData _returnvalue (Utilities|Struct|MakePlayerData "EDark" "" (LocalVariables|GetInitAbilityArray)))
      (Variables|/Script/CraftingStar.CraftingStarSaveGame|SetGuestData _returnvalue (Utilities|Struct|MakePlayerData "ELight" "" (LocalVariables|GetInitAbilityArray)))
      (Variables|/Script/CraftingStar.CraftingStarSaveGame|SetProgressData _returnvalue (Utilities|Struct|MakeProgressData "EWorldMap" _hostplayerpos _guestplayerpos))
      (Variables|Default|SetnowSaveGame _returnvalue))))

(fn Travelto
  (params (MapName :type String))
  (Development|PrintString MapName)
  (Development|ExecuteConsoleCommand (Utilities|String|Append "servertravel " MapName "?Listen") 0))