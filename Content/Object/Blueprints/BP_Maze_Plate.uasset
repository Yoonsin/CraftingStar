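; BP_Maze_Plate is a maze plate that responds to whether the light character triggers it.
; Its React event forwards the LightCharacter flag to LightCast, which swaps the mesh between light and dark fade materials and sets Activate.
; LightCast then lowers the mesh when lit or raises it otherwise, using a relative offset that accumulates on repeated calls with the same state.
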(event Custom|LightCast
  (params (light :type Boolean))
  (bind _mesh (Variables|Character|GetMesh))
  (if light
    (Rendering|Material|SetMaterial _mesh 0 "/Game/Assets/Sky_Dungeon/materials/props_materials/Fade_Inst_Light.Fade_Inst_Light")
    (Variables|Default|SetbActivate true)
    (else
      (Rendering|Material|SetMaterial _mesh 0 "/Game/Assets/Sky_Dungeon/materials/props_materials/Fade_Inst_Dark.Fade_Inst_Dark")
      (Variables|Default|SetbActivate false)))
  (Transformation|AddRelativeLocation (Variables|Character|GetMesh) (Math|Vector|MakeVector 0.0 0.0 (select (Variables|Default|GetbActivate) -1e+02 1e+02)) false false))

(event EventBeginPlay)

(event Collision|EventActorBeginOverlap
  (params (OtherActor :type Actor%20Object%20Reference)))

(event EventTick
  (params (DeltaSeconds :type Float%20%28single-precision%29)))

(event EventReact
  (params (bLightCharacter :type Boolean) (Location :type Vector :default "0, 0, 0"))
  (CallFunction|LightCast bLightCharacter))

(fn ConstructionScript)