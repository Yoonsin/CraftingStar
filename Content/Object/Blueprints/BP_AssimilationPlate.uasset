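; BP_AssimilationPlate is a plate that carries the owner of its trigger's assimilation component along a spline.
; While IsChasing is set, Tick advances Distance by Speed and places that actor at the trigger's location plus the local spline point, following only spline yaw.
; At the spline's end it resets and calls ChaseEnd on the trigger.
; The construction script passes the Light flag to the trigger and tints Niagara white or black accordingly.
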(event EventBeginPlay)

(event Collision|EventActorBeginOverlap
  (params (OtherActor :type Actor%20Object%20Reference)))

(event EventTick
  (params (DeltaSeconds :type Float%20%28single-precision%29))
  (Class|AssimilationObject|ChaseSpline DeltaSeconds))

(event EventChaseSpline
  (params (DeltaTime :type Float%20%28single-precision%29))
  (bind _trigercomponent (Variables|Default|GetTrigerComponent))
  (bind _trigercomponent_2 (Variables|Default|GetTrigerComponent))
  (if (Variables|Default|GetbIsChasing)
    (Variables|Default|SetDistance (+ (* DeltaTime (Variables|Default|GetSpeed)) (Variables|Default|GetDistance)))
    (Utilities|IsValid _trigercomponent_2
      (:Is%20Valid
        (bind _returnvalue (Class|AssimilationTrigerComponent|GetAssimilationComponent _trigercomponent_2))
        (Utilities|IsValid _returnvalue
          (:Is%20Valid
            (Transformation|SetActorTransform (Components|GetOwner _returnvalue) (Math|Transform|MakeTransform (+ (Transformation|GetWorldLocation (Variables|Default|GetTrigerComponent)) (.location (Spline|GetTransformatDistanceAlongSpline (Variables|Default|GetSpline) (Variables|Default|GetDistance) "Local" false))) (Math|Rotator|MakeRotator 0.0 0.0 (.Yaw (Math|Rotator|BreakRotator (.rotation (Spline|GetTransformatDistanceAlongSpline (Variables|Default|GetSpline) (Variables|Default|GetDistance) "Local" false))))) "1,1,1"))
            (if (> (Variables|Default|GetDistance) (Spline|GetSplineLength (Variables|Default|GetSpline)))
              (Variables|Default|SetbIsChasing false)
              (Variables|Default|SetDistance 0.0)
              (bind _returnvalue_2 (Class|AssimilationTrigerComponent|GetAssimilationComponent (Variables|Default|GetTrigerComponent)))
              (Utilities|IsValid _returnvalue_2
                (:Is%20Valid
                  (bind _returnvalue_3 (Class|AssimilationTrigerComponent|GetAssimilationComponent _trigercomponent))
                  (Class|SplineChasingInterface|ChaseEnd _trigercomponent _returnvalue_3)))))))
      (:Is%20Not%20Valid
        (Development|PrintString "NULL일수가 없는데")))))

(fn ConstructionScript
  (bind _output_get (Variables|/Script/CraftingStar.AssimilationTrigerComponent|SetbForLightCharacter (Variables|Default|GetTrigerComponent) (Variables|Default|GetbLight)))
  (Effects|Components|ParticleSystem|SetColorParameter (Variables|Default|GetNiagara) "Color" (select _output_get (Class|KismetMathLibrary|LinearColorWhite) (Class|KismetMathLibrary|LinearColorBlack))))