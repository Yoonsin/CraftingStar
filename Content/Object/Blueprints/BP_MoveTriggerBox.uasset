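; One-shot trigger box that moves the host and guest characters to the village when a CraftingStarCharacter overlaps it.
; On the server, it finds PlayerStarts named like "PlayerStart_Village", calls MoveCharacter on the game state, then saves.
; Saving sets quest progress to IncendieRescueFrameGuardian and records the box's construction-time GUID in WorldObjects.
; LoadState destroys the actor, so a used trigger stays gone in saved games.
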(event EventBeginPlay)

(event Collision|EventActorBeginOverlap
  (params (OtherActor :type Actor%20Object%20Reference))
  (Utilities|Casting|CastToCraftingStarCharacter OtherActor)
  (Networking|SwitchHasAuthority
    (:Authority
      (bind _outactors (Actor|GetAllActorsOfClass "/Script/Engine.PlayerStart"))
      (for _array_element _outactors
        (if (Utilities|String|Contains (Utilities|GetObjectName _array_element) "PlayerStart_Village")
          (bind _asbp_crafting_star_gs (Utilities|Casting|CastToBP_CraftingStarGS (Game|GetGameState)))
          (Default|MoveCharacter _asbp_crafting_star_gs (Transformation|GetActorTransform _array_element) (Transformation|GetActorTransform _array_element))
          (CallFunction|SaveState))))))

(event EventTick
  (params (DeltaSeconds :type Float%20%28single-precision%29)))

(event EventSaveState
  (bind _ascrafting_star_gs (Utilities|Casting|CastToCraftingStarGS (Game|GetGameState)))
  (Utilities|Struct|SetmembersinProgressData (Variables|/Script/CraftingStar.CraftingStarGS|GetProgressData _ascrafting_star_gs) "EIncendieRescueFrameGuardian")
  (Utilities|Array|AddUnique (.WorldObjects (Utilities|Struct|BreakProgressData (Variables|/Script/CraftingStar.CraftingStarGS|GetProgressData _ascrafting_star_gs))) (Variables|세이브|GetID))
  (Class|UtilityFunction|Save (Game|GetGameInstance)))

(event EventLoadState
  (Actor|DestroyActor))

(fn ConstructionScript
  (if (Utilities|Enum|Equal(Enum) (Variables|세이브|GetID) "")
    (Variables|세이브|SetID (Guid|ToString(Guid) (Guid|NewGuid)))))

(fn GetObjectID
  (return (Variables|세이브|GetID)))