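; Destructible bridge actor, named for a boss encounter, that collapses when its BreakBridge event is called.
; BreakBridge disables collision on the Destructible component and applies heavy damage with a downward impulse at the actor's location to shatter it.
; When the component fractures, the companion StaticMesh loses collision and the actor destroys itself after a short delay.
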(event OnComponentFracture(Destructible)
  (params (HitPoint :type Vector%20%28by%20ref%29 :default "0, 0, 0") (HitDirection :type Vector%20%28by%20ref%29 :default "0, 0, 0"))
  (Collision|SetCollisionEnabled (Variables|Default|GetStaticMesh) "NoCollision")
  (Utilities|FlowControl|Delay 3.0)
  (Actor|DestroyActor))

(event Custom|BreakBridge
  (Collision|SetCollisionEnabled (Variables|Default|GetDestructible) "NoCollision")
  (Class|DestructibleComponent|ApplyDamage (Variables|Default|GetDestructible) 3e+02 (Transformation|GetActorLocation) (Math|Vector|VectorDown) 1e+02))

(event EventBeginPlay)

(event Collision|EventActorBeginOverlap
  (params (OtherActor :type Actor%20Object%20Reference)))

(event EventTick
  (params (DeltaSeconds :type Float%20%28single-precision%29)))

(fn ConstructionScript)