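; Double-door gate that opens once when enough triggers are active, playing an optional level sequence, a sound and a timeline door swing.
; On authority, it then saves its construction-generated GUID to the game state's world objects.
; LoadState snaps the doors open without animation.
; A separate OpenPortal function, not called here, updates map and quest progress, saves unless in debug, then travels to the next map.
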(event Custom|OpenDoor
  (bind _level_sequence (Variables|Default|GetLevel%20Sequence))
  (if (not (Variables|Default|GetbIsPlayed))
    (Variables|Default|SetbIsPlayed true)
    (Utilities|IsValid _level_sequence
      (:Is%20Valid
        (bind _returnvalue (Sequencer|Player|CreateLevelSequencePlayer _level_sequence))
        (Sequencer|Player|Play _returnvalue :!class /Script/MovieScene.MovieSceneSequencePlayer))
      (:Is%20Not%20Valid
        _))
    (Audio|PlaySoundatLocation 0 (Transformation|GetActorLocation) "0, 0, 0" 1.0 1.0 0.0 0 0 0)
    (bind _curve (Timeline|Gate%20Open Play)
      (:Update
        (Transformation|SetRelativeRotation (Variables|Default|GetLeftDoor) (Math|Rotator|Lerp(Rotator) "0, 0, 0" "0,-90.000000,0.000000" _curve) false false)
        (Transformation|SetRelativeRotation (Variables|Default|GetRightDoor) (Math|Rotator|Lerp(Rotator) "0, 0, 0" "0,90.000000,0.000000" _curve) false false))
      (:Finished
        (Networking|SwitchHasAuthority
          (:Authority
            (CallFunction|SaveState)))))))

(event Custom|SetLocation
  (params (LeftDoorRotation :type Rotator) (RightDoorRotation :type Rotator))
  (Transformation|SetRelativeRotation (Variables|Default|GetLeftDoor) LeftDoorRotation false false)
  (Transformation|SetRelativeRotation (Variables|Default|GetRightDoor) RightDoorRotation false false)
  (Development|PrintString "Gate Load"))

(event Collision|EventActorBeginOverlap
  (params (OtherActor :type Actor%20Object%20Reference)))

(event EventTick
  (params (DeltaSeconds :type Float%20%28single-precision%29)))

(event EventTrigeron
  (bind _result (Math|Integer|IncrementInt (Variables|Default|GetTrigerCount))
    (:%20%20
      (if (>= _result (Variables|Default|GetTrigerObjectAmount))
        (CallFunction|OpenDoor)))))

(event EventTrigerOff
  (Math|Integer|DecrementInt (Variables|Default|GetTrigerCount)))

(event EventSaveState
  (bind _ascrafting_star_gs (Utilities|Casting|CastToCraftingStarGS (Game|GetGameState)))
  (Utilities|Array|AddUnique (.WorldObjects (Utilities|Struct|BreakProgressData (Variables|/Script/CraftingStar.CraftingStarGS|GetProgressData _ascrafting_star_gs))) (Variables|Default|GetID))
  (Class|UtilityFunction|Save (Game|GetGameInstance)))

(event EventLoadState
  (CallFunction|SetLocation "0,-90.000000, 0" "0,90.000000, 0"))

(fn ConstructionScript
  (if (Utilities|Enum|Equal(Enum) (Variables|Default|GetID) "")
    (Variables|Default|SetID (Guid|ToString(Guid) (Guid|NewGuid)))))

(fn OpenPortal
  (Development|PrintString "Open Portal")
  (bind _ascrafting_star_gs (Utilities|Casting|CastToCraftingStarGS (Game|GetGameState)))
  (bind _asbp_crafting_star_game_instance (Utilities|Casting|CastToBP_CraftingStarGameInstance (Game|GetGameInstance)))
  (bind _output_get (Variables|Default|SetNextMoveMap (Utilities|Select :Index (.nowmapname (Variables|/Script/CraftingStar.CraftingStarGS|GetProgressData _ascrafting_star_gs)) :EWorldMap "" :EKeyStar "L_Map_incendie" :EFlameAndIceStar "")))
  (Variables|/Script/CraftingStar.CraftingStarGS|SetProgressData _ascrafting_star_gs (Utilities|Struct|MakeProgressData (Utilities|Select :Index (.nowmapname (Variables|/Script/CraftingStar.CraftingStarGS|GetProgressData _ascrafting_star_gs)) :EWorldMap "EKeyStar" :EKeyStar "EFlameAndIceStar" :EFlameAndIceStar "EFlameAndIceStar") (.HostPlayerPos (Utilities|Struct|BreakSpawnTransform (.Value (Utilities|Map|Find (Variables|/Script/CraftingStar.CraftingStarGameInstance|GetMapSpawnDict _asbp_crafting_star_game_instance) "EFlameAndIceStar")))) (.GuestPlayerPos (Utilities|Struct|BreakSpawnTransform (.Value (Utilities|Map|Find (Variables|/Script/CraftingStar.CraftingStarGameInstance|GetMapSpawnDict _asbp_crafting_star_game_instance) "EFlameAndIceStar")))) (.progresslevel (Variables|/Script/CraftingStar.CraftingStarGS|GetProgressData _ascrafting_star_gs)) (Utilities|Select :Index (.questid (Variables|/Script/CraftingStar.CraftingStarGS|GetProgressData _ascrafting_star_gs)) :EMegetonNotMeet "EMegetonNotMeet" :EMegetonMeet "EMegetonNotMeet" :EMegetonGetKey "EMegetonNotMeet" :EMegetonClear "EMegetonTransition" :EMegetonTransition "EMegetonTransition" :EIncendieStartMovie "EMegetonNotMeet" :EIncendiePengdoNotMeet "EMegetonNotMeet" :EIncendiePengdoMeet "EMegetonNotMeet" :EIncendieClacierNotMeetAndPopoBerserk "EMegetonNotMeet" :EIncendieClacierMeet "EMegetonNotMeet") 0))
  (if (Variables|/Script/CraftingStar.CraftingStarGameInstance|GetisDebug _asbp_crafting_star_game_instance)
    (Development|PrintString (Utilities|String|EnumtoString (Utilities|Select :Index (.questid (Variables|/Script/CraftingStar.CraftingStarGS|GetProgressData _ascrafting_star_gs)) :EMegetonNotMeet "EMegetonNotMeet" :EMegetonMeet "EMegetonNotMeet" :EMegetonGetKey "EMegetonNotMeet" :EMegetonClear "EMegetonTransition" :EMegetonTransition "EMegetonTransition" :EIncendieStartMovie "EMegetonNotMeet" :EIncendiePengdoNotMeet "EMegetonNotMeet" :EIncendiePengdoMeet "EMegetonNotMeet" :EIncendieClacierNotMeetAndPopoBerserk "EMegetonNotMeet" :EIncendieClacierMeet "EMegetonNotMeet")) :!label _label)
    (Default|Travelto _asbp_crafting_star_game_instance _output_get)
    (else
      (bind _returnvalue (Class|UtilityFunction|Save _asbp_crafting_star_game_instance))
      (if _returnvalue
        (goto _label)))))

(fn GetObjectID
  (return (Variables|Default|GetID)))