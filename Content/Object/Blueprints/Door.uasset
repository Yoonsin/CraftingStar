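; Double door actor that swings open once both its left and right plates have been triggered.
; OpenTrigger latches a flag for the given side, but checks both flags and calls OpenDoor only on the left call, so a right trigger arriving last does not open it.
; OpenDoor plays a timeline whose curve lerps LeftDoor and RightDoor to opposite 90-degree relative rotations.
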(event Custom|OpenDoor
  (bind _curve (Timeline|타임라인_0 Play)
    (:Update
      (Transformation|SetRelativeRotation (Variables|Default|GetLeftDoor) (Math|Rotator|Lerp(Rotator) "0, 0, 0" "0,-90.000000,0.000000" _curve) false false)
      (Transformation|SetRelativeRotation (Variables|Default|GetRightDoor) (Math|Rotator|Lerp(Rotator) "0, 0, 0" "0,90.000000,0.000000" _curve) false false))))

(event EventBeginPlay)

(event Collision|EventActorBeginOverlap
  (params (OtherActor :type Actor%20Object%20Reference)))

(event EventTick
  (params (DeltaSeconds :type Float%20%28single-precision%29)))

(fn ConstructionScript)

(fn OpenTrigger
  (params (isLeft :type Boolean))
  (if isLeft
    (bind _output_get (Variables|Default|SetLeftPlate true))
    (if (and _output_get (stale _output_get_2))
      (CallFunction|OpenDoor))
    (else
      (bind _output_get_2 (Variables|Default|SetRightPlate true)))))