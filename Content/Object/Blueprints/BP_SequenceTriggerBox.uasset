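; A one-shot trigger box that plays its assigned Sequence when a CraftingStarCharacter overlaps it.
; The server has the game state multicast the sequence, then saves the box and disables its collision.
; SaveState adds the box's ID to the world-object progress data and saves through the game instance, while LoadState destroys the actor.
; The construction script assigns a GUID as the ID when it is empty.
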(event EventBeginPlay)

(event Collision|EventActorBeginOverlap
  (params (OtherActor :type Actor%20Object%20Reference))
  (Utilities|Casting|CastToCraftingStarCharacter OtherActor)
  (Networking|SwitchHasAuthority
    (:Authority
      (bind _asbp_crafting_star_gs (Utilities|Casting|CastToBP_CraftingStarGS (Game|GetGameState)))
      (Default|MultiCastPlaySequence _asbp_crafting_star_gs (Variables|시퀀스재생|GetSequence))
      (CallFunction|SaveState)
      (Collision|SetCollisionEnabled (Variables|Default|GetCollisionComponent) "NoCollision"))))

(event EventTick
  (params (DeltaSeconds :type Float%20%28single-precision%29)))

(event EventSaveState
  (bind _ascrafting_star_gs (Utilities|Casting|CastToCraftingStarGS (Game|GetGameState)))
  (Utilities|Array|AddUnique (.WorldObjects (Utilities|Struct|BreakProgressData (Variables|/Script/CraftingStar.CraftingStarGS|GetProgressData _ascrafting_star_gs))) (Variables|세이브|GetID))
  (Class|UtilityFunction|Save (Game|GetGameInstance)))

(event EventLoadState
  (Actor|DestroyActor))

(fn ConstructionScript
  (if (Utilities|Enum|Equal(Enum) (Variables|세이브|GetID) "")
    (Variables|세이브|SetID (Guid|ToString(Guid) (Guid|NewGuid)))))

(fn GetObjectID
  (return (Variables|세이브|GetID)))