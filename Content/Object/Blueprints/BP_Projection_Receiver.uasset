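; BP_Projection_Receiver is a trigger target that detects when the player character faces it, apparently an early stub.
; On Tick, each receiver casts a debug-drawn Visibility line trace forward from the player character's location along the pawn's rotation.
; It calls TriggerOn on whichever receiver is hit, not necessarily itself.
; TriggerOn only prints a debug string, and TriggerOff is empty.
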(event EventBeginPlay)

(event Collision|EventActorBeginOverlap
  (params (OtherActor :type Actor%20Object%20Reference)))

(event EventTick
  (params (DeltaSeconds :type Float%20%28single-precision%29))
  (bind _returnvalue (Game|Player|GetPlayerPawn 0))
  (bind _asbp_crafting_star_character (Utilities|Casting|CastToBP_CraftingStarCharacter _returnvalue))
  (bind (_outhit _returnvalue_2) (Collision|LineTraceByChannel (Transformation|GetActorLocation _asbp_crafting_star_character) (+ (Transformation|GetActorLocation _asbp_crafting_star_character) (* (Math|Vector|GetForwardVector (Transformation|GetActorRotation _returnvalue)) 1e+03)) "TraceTypeQuery1" false 0 "ForOneFrame" true "(R=0.000000,G=0.256177,B=1.000000,A=1.000000)"))
  (if _returnvalue_2
    (bind _asbp_projection_receiver (Utilities|Casting|CastToBP_Projection_Receiver (.HitActor (Collision|BreakHitResult _outhit))))
    (CallFunction|Triggeron _asbp_projection_receiver)))

(fn ConstructionScript)

(fn Triggeron
  (Development|PrintString "Hello"))

(fn TriggerOff)