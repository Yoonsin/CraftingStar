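; BP_ElementBowl is a composite actor that pairs a light sensor with an eject symbol through Child Actor components.
; Its construction script copies ForLight to both children and also passes TrigerObject to the BP_LightSensor.
; The symbol is only configured if the sensor cast succeeds, and the event graph holds no logic of its own.
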(event Collision|EventActorBeginOverlap
  (params (OtherActor :type Actor%20Object%20Reference)))

(event EventBeginPlay)

(fn ConstructionScript
  (bind _asbp_light_sensor (Utilities|Casting|CastToBP_LightSensor (Variables|/Script/Engine.ChildActorComponent|GetChildActor (Variables|Default|GetSensor))))
  (Variables|/Game/Object/Blueprints/Megeton/BP_LightSensor.BP_LightSensor_C|SetbForLight _asbp_light_sensor (Variables|Default|GetForLight))
  (Variables|/Game/Object/Blueprints/Megeton/BP_LightSensor.BP_LightSensor_C|SetTrigerObject _asbp_light_sensor (Variables|Default|GetTrigerObject))
  (bind _asbp_eject_symbol (Utilities|Casting|CastToBP_Eject_Symbol (Variables|/Script/Engine.ChildActorComponent|GetChildActor (Variables|Default|GetSymbol))))
  (Variables|/Game/Object/BP_Eject_Symbol.BP_Eject_Symbol_C|SetbForLight _asbp_eject_symbol (Variables|Default|GetForLight)))