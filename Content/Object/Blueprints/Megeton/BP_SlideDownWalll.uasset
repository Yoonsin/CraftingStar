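; BP_SlideDownWalll is a wall that slides down once enough triggers are active.
; Trigger on and off events adjust a counter; reaching the required count spawns a wall sound and plays a timeline that lowers the mesh by DownAmount.
; On finish, if the sound is still valid, it stops it, records the wall's construction-script GUID in the GameState's DestoryActors list and saves through the GameInstance.
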(event EventBeginPlay)

(event Collision|EventActorBeginOverlap
  (params (OtherActor :type Actor%20Object%20Reference)))

(event EventTick
  (params (DeltaSeconds :type Float%20%28single-precision%29)))

(event EventTrigeron
  (bind _result (Math|Integer|IncrementInt (Variables|Default|GetTrigerCount))
    (:%20%20
      (if (>= _result (Variables|Default|GetTrigerObjectCount))
        (bind _returnvalue (Audio|SpawnSoundatLocation "/Game/Assets/Sound/Wall.Wall" (Transformation|GetActorLocation) "0, 0, 0" 1.0 1.0 0.0 0 0))
        (bind _slidedown (Timeline|SlideDown Play)
          (:Update
            (Transformation|SetRelativeLocation (Variables|Default|GetStaticMesh) (Math|Vector|Lerp(Vector) "0, 0, 0" (Math|Vector|MakeVector 0.0 0.0 (* -1 (Variables|Default|GetDownAmount))) _slidedown) false false))
          (:Finished
            (Utilities|IsValid _returnvalue
              (:Is%20Valid
                (Audio|Components|Audio|Stop _returnvalue)
                (bind _ascrafting_star_gs (Utilities|Casting|CastToCraftingStarGS (Game|GetGameState)))
                (Utilities|Array|AddUnique (.DestoryActors (Utilities|Struct|BreakProgressData (Variables|/Script/CraftingStar.CraftingStarGS|GetProgressData _ascrafting_star_gs))) (Variables|Default|GetID))
                (Default|Save (.AsBP%20Crafting%20Star%20Game%20Instance (Utilities|Casting|CastToBP_CraftingStarGameInstance (Game|GetGameInstance))))))))))))

(event EventTrigerOff
  (Math|Integer|DecrementInt (Variables|Default|GetTrigerCount)))

(fn ConstructionScript
  (if (Utilities|Enum|Equal(Enum) (Variables|Default|GetID) "")
    (Variables|Default|SetID (Guid|ToString(Guid) (Guid|NewGuid)))))