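; BP_AbilitySphere is a pickup that grants its ObtainingAbility to a CraftingStar character on overlap, with a 2D sound.
; Authority and remote both set the game state's NowObtainingAbility; only authority calls ServerObtainAbility on the character and saves.
; SaveState records the sphere's ID in the game state's ProgressData, saves and destroys the actor.
; The construction script fills an empty ID with a GUID, and LoadState simply destroys the sphere.
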(event EventBeginPlay)

(event Collision|EventActorBeginOverlap
  (params (OtherActor :type Actor%20Object%20Reference))
  (bind _returnvalue (Game|GetGameState))
  (bind _obtainingability (Variables|Default|GetObtainingAbility))
  (bind _ascrafting_star_gs (Utilities|Casting|CastToCraftingStarGS _returnvalue))
  (bind _asbp_crafting_star_character (Utilities|Casting|CastToBP_CraftingStarCharacter OtherActor))
  (Audio|PlaySound2D "/Game/Assets/Sound/GetAbility.GetAbility" 1.0 1.0 0.0 0 0)
  (Networking|SwitchHasAuthority
    (:Authority
      (bind _output_get (Variables|/Script/CraftingStar.CraftingStarGS|SetnowObtainingAbility _ascrafting_star_gs _obtainingability))
      (Class|CraftingStarCharacter|ServerObtainAbility _asbp_crafting_star_character _output_get)
      (CallFunction|SaveState))
    (:Remote
      (Variables|/Script/CraftingStar.CraftingStarGS|SetnowObtainingAbility _ascrafting_star_gs _obtainingability))))

(event EventTick
  (params (DeltaSeconds :type Float%20%28single-precision%29)))

(event EventSaveState
  (bind _ascrafting_star_gs (Utilities|Casting|CastToCraftingStarGS (Game|GetGameState)))
  (Utilities|Array|AddUnique (.WorldObjects (Utilities|Struct|BreakProgressData (Variables|/Script/CraftingStar.CraftingStarGS|GetProgressData _ascrafting_star_gs))) (Variables|Default|GetID))
  (Class|UtilityFunction|Save (Game|GetGameInstance))
  (Actor|DestroyActor))

(event EventLoadState
  (Actor|DestroyActor))

(fn ConstructionScript
  (if (Utilities|Enum|Equal(Enum) (Variables|Default|GetID) "")
    (Variables|Default|SetID (Guid|ToString(Guid) (Guid|NewGuid)))))

(fn OnRepObtainingAbility)

(fn GetObjectID
  (return (Variables|Default|GetID)))