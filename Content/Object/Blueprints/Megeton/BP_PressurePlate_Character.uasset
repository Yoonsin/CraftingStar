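; A pressure plate actor that Characters press by standing on it to trigger a linked object, such as a gate.
; On the server, collision begin and end overlaps with Characters call PressOn and PressOff, guarded by an IsPressed flag.
; Each toggles the plate's height, plays a sound, and calls TrigerOn or TrigerOff on TrigerObject, printing a warning if none is set.
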(event OnComponentBeginOverlap(PlateCollision)
  (params (OverlappedComponent :type Primitive%20Component%20Object%20Reference) (OtherActor :type Actor%20Object%20Reference) (OtherComp :type Primitive%20Component%20Object%20Reference) (OtherBodyIndex :type Integer) (bFromSweep :type Boolean) (SweepResult :type Hit%20Result%20Structure%20%28by%20ref%29))
  (Networking|SwitchHasAuthority
    (:Authority
      (Utilities|Casting|CastToCharacter OtherActor)
      (Gate|Presson))))

(event OnComponentEndOverlap(PlateCollision)
  (params (OverlappedComponent :type Primitive%20Component%20Object%20Reference) (OtherActor :type Actor%20Object%20Reference) (OtherComp :type Primitive%20Component%20Object%20Reference) (OtherBodyIndex :type Integer))
  (Networking|SwitchHasAuthority
    (:Authority
      (Utilities|Casting|CastToCharacter OtherActor)
      (Gate|PressOff))))

(event EventBeginPlay)

(event Collision|EventActorBeginOverlap
  (params (OtherActor :type Actor%20Object%20Reference)))

(event EventTick
  (params (DeltaSeconds :type Float%20%28single-precision%29)))

(fn ConstructionScript)

(fn Presson
  (bind _returnvalue (Transformation|GetActorLocation))
  (bind _trigerobject (Variables|Gate|GetTrigerObject))
  (if (Variables|Default|GetbIsPressed)
    _
    (else
      (Audio|PlaySoundatLocation "/Game/Assets/Sound/ButtonOn.ButtonOn" _returnvalue "0, 0, 0" 1.0 1.0 0.0 0 0 0)
      (Transformation|SetActorLocation (+ _returnvalue "0,0.000000,-20.000000") false true)
      (Utilities|IsValid (Utilities|ToObject(Interface) _trigerobject)
        (:Is%20Valid
          (Default|Trigeron _trigerobject))
        (:Is%20Not%20Valid
          (Development|PrintString "Please Set Gate at Plate")))))
  (Variables|Default|SetbIsPressed true))

(fn PressOff
  (bind _returnvalue (Transformation|GetActorLocation))
  (bind _trigerobject (Variables|Gate|GetTrigerObject))
  (if (Variables|Default|GetbIsPressed)
    (Transformation|SetActorLocation (+ _returnvalue "0,0.000000,20.000000") false false)
    (Audio|PlaySoundatLocation "/Game/Assets/Sound/ButtonOff.ButtonOff" _returnvalue "0, 0, 0" 1.0 1.0 0.0 0 0 0)
    (Utilities|IsValid (Utilities|ToObject(Interface) _trigerobject)
      (:Is%20Valid
        (Default|TrigerOff _trigerobject))
      (:Is%20Not%20Valid
        (Development|PrintString "Pllease Set Gate at Plate"))))
  (Variables|Default|SetbIsPressed false))