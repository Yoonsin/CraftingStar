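; BP_Gate_MegetonPortal is a portal gate for Megeton that opens when a CraftingStarCharacter steps into it.
; The Portal component starts with collision off, and SetActivePortal enables it when passed true; false does nothing.
; A character overlap, handled only on the authority, disables the collision again so it cannot retrigger, then calls OpenPortal, whose logic lives outside this graph.
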(event OnComponentBeginOverlap(Portal)
  (params (OverlappedComponent :type Primitive%20Component%20Object%20Reference) (OtherActor :type Actor%20Object%20Reference) (OtherComp :type Primitive%20Component%20Object%20Reference) (OtherBodyIndex :type Integer) (bFromSweep :type Boolean) (SweepResult :type Hit%20Result%20Structure%20%28by%20ref%29))
  (Utilities|Casting|CastToCraftingStarCharacter OtherActor)
  (Networking|SwitchHasAuthority
    (:Authority
      (Collision|SetCollisionEnabled (Variables|Default|GetPortal) "NoCollision")
      (CallFunction|OpenPortal))))

(event Custom|SetActivePortal
  (params (Flag :type Boolean))
  (if Flag
    (Collision|SetCollisionEnabled (Variables|Default|GetPortal) "QueryAndPhysics")))

(event EventBeginPlay
  (Collision|SetCollisionEnabled (Variables|Default|GetPortal) "NoCollision"))

(fn ConstructionScript
  (|CallParentFunction))