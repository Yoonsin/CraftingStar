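; BP_BreableChain is a breakable chain that breaks when hit by a two-handed attack.
; On that event it spawns an explosion effect and sound, then hides its three meshes and disables their and the box's collision rather than destroying the actor.
; It records its construction-script GUID in the game state's destroyed-actor list and saves through the game instance, exposing the ID via GetID.
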(event EventBeginPlay)

(event Collision|EventActorBeginOverlap
  (params (OtherActor :type Actor%20Object%20Reference)))

(event EventTick
  (params (DeltaSeconds :type Float%20%28single-precision%29)))

(event EventAttackbyTwoHanded
  (params (bLightCharacter :type Boolean))
  (bind _returnvalue (Transformation|GetActorLocation))
  (Effects|SpawnEmitteratLocation "/Game/Assets/BaseContent/StarterContent/Particles/P_Explosion.P_Explosion" _returnvalue)
  (Audio|PlaySoundatLocation "/Game/Assets/Sound/BreakObject.BreakObject" _returnvalue "0, 0, 0" 1.0 1.0 0.0 0 0 0)
  (Rendering|SetVisibility (Variables|Default|GetStaticMesh) false false)
  (Rendering|SetVisibility (Variables|Default|GetStaticMesh1) false false)
  (Rendering|SetVisibility (Variables|Default|GetStaticMesh2) false false)
  (Collision|SetCollisionEnabled (Variables|Default|GetBox) "NoCollision")
  (bind _ascrafting_star_gs (Utilities|Casting|CastToCraftingStarGS (Game|GetGameState)))
  (Utilities|Array|AddUnique (.DestoryActors (Utilities|Struct|BreakProgressData (Variables|/Script/CraftingStar.CraftingStarGS|GetProgressData _ascrafting_star_gs))) (Variables|Default|GetID))
  (Default|Save (.AsBP%20Crafting%20Star%20Game%20Instance (Utilities|Casting|CastToBP_CraftingStarGameInstance (Game|GetGameInstance)))))

(fn ConstructionScript
  (if (Utilities|Enum|Equal(Enum) (Variables|Default|GetID) "")
    (Variables|Default|SetID (Guid|ToString(Guid) (Guid|NewGuid)))))

(fn GetID
  (return (Variables|Default|GetID)))