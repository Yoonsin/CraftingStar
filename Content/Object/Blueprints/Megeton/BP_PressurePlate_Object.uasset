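; BP_PressurePlate_Object is a pressure plate that switches a linked trigger object, such as a gate, on and off.
; Begin and end overlaps on PlateCollision from actors with the TrigerTag tag call PressOn and PressOff, guarded by an IsPressed flag rather than an occupant count.
; These move the whole actor down or back up, then call TrigerOn or TrigerOff on TrigerObject, printing a warning if it is unset.
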(event OnComponentBeginOverlap(PlateCollision)
  (params (OverlappedComponent :type Primitive%20Component%20Object%20Reference) (OtherActor :type Actor%20Object%20Reference) (OtherComp :type Primitive%20Component%20Object%20Reference) (OtherBodyIndex :type Integer) (bFromSweep :type Boolean) (SweepResult :type Hit%20Result%20Structure%20%28by%20ref%29))
  (if (Actor|ActorHasTag OtherActor (Variables|Default|GetTrigerTag))
    (Gate|Presson)))

(event OnComponentEndOverlap(PlateCollision)
  (params (OverlappedComponent :type Primitive%20Component%20Object%20Reference) (OtherActor :type Actor%20Object%20Reference) (OtherComp :type Primitive%20Component%20Object%20Reference) (OtherBodyIndex :type Integer))
  (if (Actor|ActorHasTag OtherActor (Variables|Default|GetTrigerTag))
    (Gate|PressOff)))

(event EventBeginPlay)

(event Collision|EventActorBeginOverlap
  (params (OtherActor :type Actor%20Object%20Reference)))

(event EventTick
  (params (DeltaSeconds :type Float%20%28single-precision%29)))

(fn ConstructionScript)

(fn Presson
  (bind _trigerobject (Variables|Gate|GetTrigerObject))
  (if (Variables|Default|GetbIsPressed)
    _
    (else
      (Transformation|SetActorLocation (+ (Transformation|GetActorLocation) "0,0.000000,-20.000000") false true)
      (Utilities|IsValid (Utilities|ToObject(Interface) _trigerobject)
        (:Is%20Valid
          (Default|Trigeron _trigerobject))
        (:Is%20Not%20Valid
          (Development|PrintString "Please Set Gate at Plate")))))
  (Variables|Default|SetbIsPressed true))

(fn PressOff
  (bind _trigerobject (Variables|Gate|GetTrigerObject))
  (if (Variables|Default|GetbIsPressed)
    (Transformation|SetActorLocation (+ (Transformation|GetActorLocation) "0,0.000000,20.000000") false false)
    (Utilities|IsValid (Utilities|ToObject(Interface) _trigerobject)
      (:Is%20Valid
        (Default|TrigerOff _trigerobject))
      (:Is%20Not%20Valid
        (Development|PrintString "Pllease Set Gate at Plate"))))
  (Variables|Default|SetbIsPressed false))