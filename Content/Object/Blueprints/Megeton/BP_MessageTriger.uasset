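; Overlap trigger for the Megeton area whose response depends on the quest ID in the game state.
; Before the Megeton meeting quest, an overlapping player pawn gets a message widget and a barrier sound, with the widget removed on end overlap.
; At the meeting quest, the host starts the dialog, flags the Megeton door open, records the trigger's ID in progress data and saves, disabling further triggering.
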(event OnComponentBeginOverlap(CollisionComponent)
  (params (OverlappedComponent :type Primitive%20Component%20Object%20Reference) (OtherActor :type Actor%20Object%20Reference) (OtherComp :type Primitive%20Component%20Object%20Reference) (OtherBodyIndex :type Integer) (bFromSweep :type Boolean) (SweepResult :type Hit%20Result%20Structure%20%28by%20ref%29))
  (if (not (Variables|Default|GetbDestroy))
    (if (not (Variables|Default|GetbActiveMessage))
      (if (Utilities|IsValidClass (Variables|Default|GetMessageAsset))
        (bind _aspawn (Utilities|Casting|CastToPawn OtherActor))
        (Utilities|Casting|CastToPlayerController (Pawn|GetController _aspawn))
        (bind _ascrafting_star_gs (Utilities|Casting|CastToCraftingStarGS (Game|GetGameState)))
        (if (Utilities|Enum|Equal(Enum) (.questid (Variables|/Script/CraftingStar.CraftingStarGS|GetProgressData _ascrafting_star_gs)) "EMegetonNotMeet")
          (bind _returnvalue (UserInterface|CreateWidget (Variables|Default|GetMessageAsset) 0 (Variables|Default|GetMessage)))
          (bind _output_get (Variables|Default|SetCurrent%20Widget _returnvalue))
          (UserInterface|Viewport|AddtoViewport _output_get 0)
          (Variables|Default|SetbActiveMessage true)
          (Audio|PlaySoundatLocation "/Game/Assets/Sound/Barrier.Barrier" (Transformation|GetActorLocation) "0, 0, 0" 1.0 1.0 0.0 0 0 0)
          (else
            (bind _ascrafting_star_character (Utilities|Casting|CastToCraftingStarCharacter (Game|GetPlayerCharacter 0)))
            (bind _returnvalue_2 (Class|UtilityFunction|IsHost (Pawn|GetController _ascrafting_star_character)))
            (if (Utilities|Enum|Equal(Enum) (.questid (Variables|/Script/CraftingStar.CraftingStarGS|GetProgressData _ascrafting_star_gs)) "EMegetonMeet")
              (if _returnvalue_2
                (Default|OnInteraction (Variables|Default|GetDialogComponent) _ascrafting_star_character)
                (Variables|Default|SetbDestroy true)
                (bind _asbp_crafting_star_gs (Utilities|Casting|CastToBP_CraftingStarGS (Game|GetGameState)))
                (Variables|/Script/CraftingStar.CraftingStarGS|SetisOpenMegetonDoor _asbp_crafting_star_gs true)
                (bind _ascrafting_star_gs_2 (Utilities|Casting|CastToCraftingStarGS (Game|GetGameState)))
                (Utilities|Array|AddUnique (.collectedkeysid (Variables|/Script/CraftingStar.CraftingStarGS|GetProgressData _ascrafting_star_gs_2)) (Variables|Default|GetID))
                (bind _asbp_crafting_star_game_instance (Utilities|Casting|CastToBP_CraftingStarGameInstance (Game|GetGameInstance)))
                (Default|Save _asbp_crafting_star_game_instance)))))
        (else
          (Development|PrintString "Message Object를 세팅하세요."))))))

(event OnComponentEndOverlap(CollisionComponent)
  (params (OverlappedComponent :type Primitive%20Component%20Object%20Reference) (OtherActor :type Actor%20Object%20Reference) (OtherComp :type Primitive%20Component%20Object%20Reference) (OtherBodyIndex :type Integer))
  (if (Variables|Default|GetbActiveMessage)
    (bind _aspawn (Utilities|Casting|CastToPawn OtherActor))
    (Utilities|Casting|CastToPlayerController (Pawn|GetController _aspawn))
    (Widget|RemovefromParent (Variables|Default|GetCurrent%20Widget))
    (Variables|Default|SetCurrent%20Widget 0)
    (Variables|Default|SetbActiveMessage false)))

(event Collision|EventActorBeginOverlap
  (params (OtherActor :type Actor%20Object%20Reference)))

(event EventTick
  (params (DeltaSeconds :type Float%20%28single-precision%29)))

(event EventTrigerOff
  (Actor|DestroyActor))

(event EventBeginPlay)

(fn ConstructionScript)

(fn GetID
  (return (Variables|Default|GetID)))