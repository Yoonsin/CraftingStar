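; BP_Door is a door that swings open once enough triggers are active.
; Trigeron prints a debug message, increments a counter and, when it reaches TrigerObjectAmount, plays the DoorOpen timeline to lerp the Door's relative rotation through 90 degrees.
; TrigerOff only decrements the counter, so nothing here closes the door again.
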(event EventBeginPlay)

(event Collision|EventActorBeginOverlap
  (params (OtherActor :type Actor%20Object%20Reference)))

(event EventTick
  (params (DeltaSeconds :type Float%20%28single-precision%29)))

(event EventTrigeron
  (Development|PrintString "Hello")
  (bind _result (Math|Integer|IncrementInt (Variables|Triger|GetTrigerCount))
    (:%20%20
      (if (>= _result (Variables|Triger|GetTrigerObjectAmount))
        (bind _새_트랙_0 (Timeline|DoorOpen Play)
          (:Update
            (Transformation|SetRelativeRotation (Variables|Default|GetDoor) (Math|Rotator|Lerp(Rotator) "0, 0, 0" "0,-90.000000,0.000000" _새_트랙_0) false false)))))))

(event EventTrigerOff
  (Math|Integer|DecrementInt (Variables|Triger|GetTrigerCount)))

(fn ConstructionScript)