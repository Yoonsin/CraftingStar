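; BP_LightSensor is a puzzle sensor that responds only to the matching light or dark character and fires an assigned trigger object.
; React sets it active, refreshes a short timer and plays the TurnLight timeline, which fades the Fire dynamic material.
; When the timer expires, Tick deactivates it and reverses the fade.
; Reaching near the timeline's end while active triggers the object and locks the sensor as cleared.
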(event Custom|Deactive
  (bind _trigerobject (Variables|Default|GetTrigerObject))
  (if (not (Variables|Default|GetbClear))
    (Variables|Default|SetbActive false)
    (bind _light_value (Timeline|Turn%20Light Reverse)
      (:Update
        (Rendering|Material|SetScalarParameterValue (Variables|머티리얼|GetMaterialInstatance) "Fade Amount" _light_value :!class /Script/Engine.MaterialInstanceDynamic)
        (if (and (Variables|Default|GetbActive) (>= (Components|Timeline|GetPlaybackPosition (Variables|Default|GetTurn%20Light)) 2.8))
          (Utilities|IsValid (Utilities|ToObject(Interface) _trigerobject)
            (:Is%20Valid
              (CallFunction|LogicComplete)
              (Default|Trigeron _trigerobject))
            (:Is%20Not%20Valid
              (Development|PrintString "TrigerObject가 할당되지 않았습니다."))))))))

(event Custom|LogicComplete
  (bind _trigerobject (Variables|Default|GetTrigerObject))
  (Variables|Default|SetbClear true)
  (bind _light_value (Timeline|Turn%20Light Stop)
    (:Update
      (Rendering|Material|SetScalarParameterValue (Variables|머티리얼|GetMaterialInstatance) "Fade Amount" _light_value :!class /Script/Engine.MaterialInstanceDynamic)
      (if (and (Variables|Default|GetbActive) (>= (Components|Timeline|GetPlaybackPosition (Variables|Default|GetTurn%20Light)) 2.8))
        (Utilities|IsValid (Utilities|ToObject(Interface) _trigerobject)
          (:Is%20Valid
            (CallFunction|LogicComplete)
            (Default|Trigeron _trigerobject))
          (:Is%20Not%20Valid
            (Development|PrintString "TrigerObject가 할당되지 않았습니다.")))))))

(event EventBeginPlay
  (bind _returnvalue (Rendering|Material|CreateDynamicMaterialInstance (Variables|Default|GetFire) 0 (select (Variables|Default|GetbForLight) (Variables|Material|GetMaterialAsset_Light) (Variables|머티리얼|GetMaterialAsset_Dark)) "None" :!class /Script/Engine.PrimitiveComponent))
  (bind _output_get (Variables|머티리얼|SetMaterialInstatance _returnvalue))
  (Rendering|Material|SetScalarParameterValue _output_get "Fade Amount" 1.0 :!class /Script/Engine.MaterialInstanceDynamic))

(event Collision|EventActorBeginOverlap
  (params (OtherActor :type Actor%20Object%20Reference)))

(event EventTick
  (params (DeltaSeconds :type Float%20%28single-precision%29))
  (if (not (Variables|Default|GetbClear))
    (if true
      ;[1 1 1] Inner Timer
      (if (> (Variables|Time|GetInnerTimer) 0.0)
        (Variables|Time|SetInnerTimer (- (Variables|Time|GetInnerTimer) DeltaSeconds))
        (else
          (Variables|Time|SetInnerTimer 0.0)))
      (if (not (> (Variables|Time|GetInnerTimer) 0.0))
        (CallFunction|Deactive)))))

(event EventReact
  (params (bLightCharacter :type Boolean) (Location :type Vector :default "0, 0, 0"))
  (bind _trigerobject (Variables|Default|GetTrigerObject))
  (if (not (Variables|Default|GetbClear))
    (if (Math|Boolean|Equal(Boolean) bLightCharacter (Variables|Default|GetbForLight))
      (Variables|Default|SetbActive true)
      (Variables|Time|SetInnerTimer (Variables|Time|GetInputTime))
      (bind _light_value (Timeline|Turn%20Light Play)
        (:Update
          (Rendering|Material|SetScalarParameterValue (Variables|머티리얼|GetMaterialInstatance) "Fade Amount" _light_value :!class /Script/Engine.MaterialInstanceDynamic)
          (if (and (Variables|Default|GetbActive) (>= (Components|Timeline|GetPlaybackPosition (Variables|Default|GetTurn%20Light)) 2.8))
            (Utilities|IsValid (Utilities|ToObject(Interface) _trigerobject)
              (:Is%20Valid
                (CallFunction|LogicComplete)
                (Default|Trigeron _trigerobject))
              (:Is%20Not%20Valid
                (Development|PrintString "TrigerObject가 할당되지 않았습니다.")))))))))

(fn ConstructionScript)