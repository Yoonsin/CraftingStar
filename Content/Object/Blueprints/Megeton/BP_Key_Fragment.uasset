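; BP_Key_Fragment is a collectible key fragment pickup that advances game progress.
; The Fragment component spins around its yaw axis on Tick.
; When a Character overlaps BoxCollision, it increments ProgressLevel in the CraftingStarGS game state's ProgressData, switching the quest ID to EMegetonGetKey when the level reaches four.
; It then destroys itself and prints a pickup message.
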(event OnComponentBeginOverlap(BoxCollision)
  (params (OverlappedComponent :type Primitive%20Component%20Object%20Reference) (OtherActor :type Actor%20Object%20Reference) (OtherComp :type Primitive%20Component%20Object%20Reference) (OtherBodyIndex :type Integer) (bFromSweep :type Boolean) (SweepResult :type Hit%20Result%20Structure%20%28by%20ref%29))
  (Utilities|Casting|CastToCharacter OtherActor)
  (bind _ascrafting_star_gs (Utilities|Casting|CastToCraftingStarGS (Game|GetGameState)))
  (if (== (+ (.progresslevel (Variables|/Script/CraftingStar.CraftingStarGS|GetProgressData _ascrafting_star_gs)) 1) 4)
    (Variables|/Script/CraftingStar.CraftingStarGS|SetProgressData _ascrafting_star_gs (Utilities|Struct|MakeProgressData (.nowmapname (Variables|/Script/CraftingStar.CraftingStarGS|GetProgressData _ascrafting_star_gs)) (.hostplayerpos (Variables|/Script/CraftingStar.CraftingStarGS|GetProgressData _ascrafting_star_gs)) (.guestplayerpos (Variables|/Script/CraftingStar.CraftingStarGS|GetProgressData _ascrafting_star_gs)) (+ (.progresslevel (Variables|/Script/CraftingStar.CraftingStarGS|GetProgressData _ascrafting_star_gs)) 1) "EMegetonGetKey" 0 0))
    (else
      (Variables|/Script/CraftingStar.CraftingStarGS|SetProgressData _ascrafting_star_gs (Utilities|Struct|MakeProgressData (.nowmapname (Variables|/Script/CraftingStar.CraftingStarGS|GetProgressData _ascrafting_star_gs)) (.hostplayerpos (Variables|/Script/CraftingStar.CraftingStarGS|GetProgressData _ascrafting_star_gs)) (.guestplayerpos (Variables|/Script/CraftingStar.CraftingStarGS|GetProgressData _ascrafting_star_gs)) (+ (.progresslevel (Variables|/Script/CraftingStar.CraftingStarGS|GetProgressData _ascrafting_star_gs)) 1) (.questid (Variables|/Script/CraftingStar.CraftingStarGS|GetProgressData _ascrafting_star_gs)) 0 0))))
  (Actor|DestroyActor)
  (Development|PrintString "Get Item"))

(event EventBeginPlay)

(event Collision|EventActorBeginOverlap
  (params (OtherActor :type Actor%20Object%20Reference)))

(event EventTick
  (params (DeltaSeconds :type Float%20%28single-precision%29))
  (Transformation|AddRelativeRotation (Variables|Default|GetFragment) (* "0.000000,100.000000,0.000000" DeltaSeconds) false false))

(fn ConstructionScript)