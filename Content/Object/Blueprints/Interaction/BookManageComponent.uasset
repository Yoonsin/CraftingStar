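; Interaction component for a readable book that shows an array of page images in a UI widget.
; On interaction it pauses the player, sets the interaction state, switches to UI-only input with cursor and binds the widget's Prev, Next and Exit events.
; Page turns update the image, hide arrows at the first and last pages and print the index.
; Exit unbinds and removes the widget, then restores idle state and game input.
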(event Custom|ReadPrevPage
  (bind _bookwidget (Variables|위젯|GetBookWidget))
  (bind _result (Math|Integer|DecrementInt (Variables|이미지|GetNowPageNum))
    (:%20%20
      (bind _output_get (Variables|이미지|SetNowPageNum (Math|Integer|%(Integer) (+ _result (Variables|이미지|GetMaxPageSize)) (Variables|이미지|GetMaxPageSize))))
      (Development|PrintString (Utilities|String|ToString(Integer) _output_get))
      (Default|SetImage (Variables|위젯|GetBookWidget) (Utilities|Array|Get(acopy) (Variables|이미지|GetImageArray) _output_get))
      (Default|SetVisibilityNextButton (Variables|위젯|GetBookWidget) "Visible")
      (if (== (Variables|이미지|GetNowPageNum) 0)
        (Default|SetVisibilityPrevButton _bookwidget "Collapsed")
        (else
          (Default|SetVisibilityPrevButton _bookwidget "Visible"))))))

(event Custom|Quit
  (bind _playercharacter (Variables|캐릭터|GetplayerCharacter))
  (bind _bookwidget (Variables|위젯|GetBookWidget))
  (bind _returnvalue (Pawn|GetController _playercharacter))
  (bind _asplayer_controller (Utilities|Casting|CastToPlayerController _returnvalue))
  (Class|CraftingStarCharacter|UpdatePlayerGMState (Variables|캐릭터|GetplayerCharacter) "EIdle")
  (EventDispatchers|UnbindEventfromNext _bookwidget (delegate Custom|ReadNextPage))
  (EventDispatchers|UnbindEventfromPrev _bookwidget (delegate Custom|ReadPrevPage))
  (EventDispatchers|UnbindEventfromExit _bookwidget (delegate Custom|Quit))
  (Widget|RemovefromParent (Variables|위젯|GetBookWidget))
  (Input|SetInputModeGameOnly _asplayer_controller)
  (Variables|/Script/Engine.PlayerController|SetbShowMouseCursor _asplayer_controller false)
  (Class|CraftingStarCharacter|SetPause (Variables|캐릭터|GetplayerCharacter) false))

(event Custom|ReadNextPage
  (bind _bookwidget (Variables|위젯|GetBookWidget))
  (bind _result (Math|Integer|IncrementInt (Variables|이미지|GetNowPageNum))
    (:%20%20
      (bind _output_get (Variables|이미지|SetNowPageNum (Math|Integer|%(Integer) _result (Variables|이미지|GetMaxPageSize))))
      (Development|PrintString (Utilities|String|ToString(Integer) _output_get))
      (Default|SetImage (Variables|위젯|GetBookWidget) (Utilities|Array|Get(acopy) (Variables|이미지|GetImageArray) _output_get))
      (Default|SetVisibilityPrevButton (Variables|위젯|GetBookWidget) "Visible")
      (if (== (Variables|이미지|GetNowPageNum) (- (Variables|이미지|GetMaxPageSize) 1))
        (Default|SetVisibilityNextButton _bookwidget "Collapsed")
        (else
          (Default|SetVisibilityNextButton _bookwidget "Visible"))))))

(event EventBeginPlay
  (Variables|이미지|SetMaxPageSize (Utilities|Array|Length (Variables|이미지|GetImageArray))))

(event EventTick
  (params (DeltaSeconds :type Float%20%28single-precision%29)))

(event EventOnInteraction
  (params (PlayerCharacter :type Crafting%20Star%20Character%20Object%20Reference))
  (bind _output_get (Variables|캐릭터|SetplayerCharacter PlayerCharacter))
  (Class|CraftingStarCharacter|SetPause _output_get true)
  (Class|CraftingStarCharacter|UpdatePlayerGMState PlayerCharacter "EInteraction")
  (Input|SetInputModeUIOnly (.AsPlayer%20Controller (Utilities|Casting|CastToPlayerController (Pawn|GetController _output_get))) 0 "DoNotLock")
  (Variables|/Script/Engine.PlayerController|SetbShowMouseCursor (.AsPlayer%20Controller (Utilities|Casting|CastToPlayerController (Pawn|GetController _output_get))) true)
  (bind _returnvalue (UserInterface|CreateWidget "/Game/Object/Blueprints/Interaction/BookWidget.BookWidget_C" (.AsPlayer%20Controller (Utilities|Casting|CastToPlayerController (Pawn|GetController _output_get)))))
  (UserInterface|Viewport|AddtoViewport _returnvalue 0)
  (bind _output_get_2 (Variables|위젯|SetBookWidget _returnvalue))
  (Default|SetImage _output_get_2 (Utilities|Array|Get(acopy) (Variables|이미지|GetImageArray)))
  (EventDispatchers|BindEventtoPrev (Variables|위젯|GetBookWidget) (delegate Custom|ReadPrevPage))
  (EventDispatchers|BindEventtoNext (Variables|위젯|GetBookWidget) (delegate Custom|ReadNextPage))
  (EventDispatchers|BindEventtoExit (Variables|위젯|GetBookWidget) (delegate Custom|Quit))
  (Variables|이미지|SetNowPageNum 0)
  (if (> (Variables|이미지|GetMaxPageSize) 1)
    (Default|SetVisibilityPrevButton (Variables|위젯|GetBookWidget) "Collapsed")
    (else
      (Default|SetVisibilityNextButton (Variables|위젯|GetBookWidget) "Collapsed")
      (Default|SetVisibilityPrevButton (Variables|위젯|GetBookWidget) "Collapsed"))))

(fn GetInteractionType
  (return "NewEnumerator0"))

(fn GetMultiState
  (return "NewEnumerator1"))