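; DoorManageComponent is an interactable door Blueprint whose open/close logic is currently disconnected.
; OnInteraction is empty, leaving orphaned nodes that would play a door sound, toggle IsOpened, save state and rotate the Door through a rotator lerp.
; GetInteractionType and GetMultiState each return a fixed enum value to describe the interaction.
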(event EventBeginPlay)

(event EventTick
  (params (DeltaSeconds :type Float%20%28single-precision%29)))

(event EventOnInteraction
  (params (PlayerCharacter :type Crafting%20Star%20Character%20Object%20Reference)))

(fn GetInteractionType
  (return "NewEnumerator1"))

(fn GetMultiState
  (return "NewEnumerator1"))