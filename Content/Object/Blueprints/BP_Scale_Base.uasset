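; BP_Scale_Base is a balance scale that tips toward whichever basket holds more weight.
; Basket overlap events add or subtract each BP_ScaleForObject's weight from left and right totals, printing the result.
; Tick compares totals, stepping the beam's pitch while counter-rotating both baskets, or stepping back toward level when equal.
; Steps ignore delta time, and past the tilt limit RotateScale blocks movement in both directions.
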(event OnComponentBeginOverlap(inBasketRight)
  (params (OverlappedComponent :type Primitive%20Component%20Object%20Reference) (OtherActor :type Actor%20Object%20Reference) (OtherComp :type Primitive%20Component%20Object%20Reference) (OtherBodyIndex :type Integer) (bFromSweep :type Boolean) (SweepResult :type Hit%20Result%20Structure%20%28by%20ref%29))
  (bind _asbp_scale_for_object (Utilities|Casting|CastToBP_ScaleForObject OtherActor))
  (bind _object_weight (Default|GetWeight _asbp_scale_for_object))
  (bind _output_get (Variables|Default|SetRightWeight (+ (Variables|Default|GetRightWeight) _object_weight)))
  (Development|PrintString (Utilities|String|ToString(Integer) _output_get)))

(event OnComponentBeginOverlap(inBasketLeft)
  (params (OverlappedComponent :type Primitive%20Component%20Object%20Reference) (OtherActor :type Actor%20Object%20Reference) (OtherComp :type Primitive%20Component%20Object%20Reference) (OtherBodyIndex :type Integer) (bFromSweep :type Boolean) (SweepResult :type Hit%20Result%20Structure%20%28by%20ref%29))
  (bind _asbp_scale_for_object (Utilities|Casting|CastToBP_ScaleForObject OtherActor))
  (bind _object_weight (Default|GetWeight _asbp_scale_for_object))
  (bind _output_get (Variables|Default|SetLeftWeight (+ (Variables|Default|GetLeftWeight) _object_weight)))
  (Development|PrintString (Utilities|String|ToString(Integer) _output_get)))

(event OnComponentEndOverlap(inBasketLeft)
  (params (OverlappedComponent :type Primitive%20Component%20Object%20Reference) (OtherActor :type Actor%20Object%20Reference) (OtherComp :type Primitive%20Component%20Object%20Reference) (OtherBodyIndex :type Integer))
  (bind _asbp_scale_for_object (Utilities|Casting|CastToBP_ScaleForObject OtherActor))
  (bind _object_weight (Default|GetWeight _asbp_scale_for_object))
  (bind _output_get (Variables|Default|SetLeftWeight (- (Variables|Default|GetLeftWeight) _object_weight)))
  (Development|PrintString (Utilities|String|ToString(Integer) _output_get)))

(event OnComponentEndOverlap(inBasketRight)
  (params (OverlappedComponent :type Primitive%20Component%20Object%20Reference) (OtherActor :type Actor%20Object%20Reference) (OtherComp :type Primitive%20Component%20Object%20Reference) (OtherBodyIndex :type Integer))
  (bind _asbp_scale_for_object (Utilities|Casting|CastToBP_ScaleForObject OtherActor))
  (bind _object_weight (Default|GetWeight _asbp_scale_for_object))
  (bind _output_get (Variables|Default|SetRightWeight (- (Variables|Default|GetRightWeight) _object_weight)))
  (Development|PrintString (Utilities|String|ToString(Integer) _output_get)))

(event EventBeginPlay)

(event Collision|EventActorBeginOverlap
  (params (OtherActor :type Actor%20Object%20Reference)))

(event EventTick
  (params (DeltaSeconds :type Float%20%28single-precision%29))
  (CallFunction|CheckScale))

(fn ConstructionScript)

(fn CheckScale
  (bind _rightweight (Variables|Default|GetRightWeight))
  (bind _leftweight (Variables|Default|GetLeftWeight))
  (if (== _leftweight _rightweight)
    (CallFunction|RestoreScale)
    (else
      (CallFunction|RotateScale (select (> _leftweight _rightweight) 0.1 -0.1)))))

(fn RotateScale
  (params (Rotate%20Amount :type Float%20%28single-precision%29))
  (bind _returnvalue (* Rotate%20Amount -1.0))
  (if (< (Math|Float|Absolute(Float) (.pitch (Variables|/Script/Engine.SceneComponent|GetRelativeRotation (Variables|Default|GetScaleRoot)))) 2e+01)
    (Transformation|AddLocalRotation (Variables|Default|GetScaleRoot) (Math|Rotator|MakeRotator 0.0 Rotate%20Amount 0.0) false false)
    (Transformation|AddLocalRotation (Variables|Default|GetBasketLeft) (Math|Rotator|MakeRotator 0.0 _returnvalue 0.0) false false)
    (Transformation|AddLocalRotation (Variables|Default|GetBasketRight) (Math|Rotator|MakeRotator 0.0 _returnvalue 0.0) false false)
    (else
      (return))))

(fn RestoreScale
  (bind _scaleroot (Variables|Default|GetScaleRoot))
  (bind _relativerotation (Variables|/Script/Engine.SceneComponent|GetRelativeRotation _scaleroot))
  (bind _returnvalue (Math|Float|Sign(Float) (.pitch _relativerotation)))
  (bind _returnvalue_2 (* _returnvalue -0.1))
  (bind _returnvalue_3 (* _returnvalue_2 -1.0))
  (Transformation|AddLocalRotation (Variables|Default|GetScaleRoot) (Math|Rotator|MakeRotator 0.0 _returnvalue_2 0.0) false false)
  (Transformation|AddLocalRotation (Variables|Default|GetBasketLeft) (Math|Rotator|MakeRotator 0.0 _returnvalue_3 0.0) false false)
  (Transformation|AddLocalRotation (Variables|Default|GetBasketRight) (Math|Rotator|MakeRotator 0.0 _returnvalue_3 0.0) false false))