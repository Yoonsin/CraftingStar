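; Rotatable puzzle stone in Incendies that turns in response to a matching light character and tracks whether it faces its answer angle.
; React starts a countdown when the character matches ForLight, and Tick yaws the mesh at constant speed until it expires.
; While turning, a wrap-safe angle tolerance test sets Clear and particle visibility.
; Construction applies the starting yaw and Clear state and passes ForLight to the child symbol actor.
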(event EventBeginPlay)

(event Collision|EventActorBeginOverlap
  (params (OtherActor :type Actor%20Object%20Reference)))

(event EventTick
  (params (DeltaSeconds :type Float%20%28single-precision%29))
  (bind _staticmesh (Variables|Default|GetStaticMesh))
  (bind _output_get (Variables|Default|SetDelta%20Seconds DeltaSeconds))
  (if (> (Variables|Game|GetInnerTimer) 0.0)
    (Variables|Game|SetInnerTimer (- (Variables|Game|GetInnerTimer) _output_get))
    (Transformation|AddRelativeRotation _staticmesh (Math|Rotator|MakeRotator 0.0 0.0 (* (Variables|Default|GetDelta%20Seconds) 75.0)) false false)
    (bind _output_get_2 (Variables|Game|SetDegree (.Yaw (Math|Rotator|BreakRotator (Variables|/Script/Engine.SceneComponent|GetRelativeRotation _staticmesh)))))
    (bind _output_get_3 (Variables|Game|SetbClear (< (Math|Float|Absolute(Float) (Math|Rotator|NormalizeAxis (- _output_get_2 (Variables|Game|GetAnswer)))) (Variables|Default|GetToleranceAmount))))
    (Rendering|SetVisibility (Variables|Default|GetParticleSystem) _output_get_3 false)))

(event EventReact
  (params (bLightCharacter :type Boolean) (Location :type Vector :default "0, 0, 0"))
  (if (Math|Boolean|Equal(Boolean) bLightCharacter (Variables|Game|GetForLight))
    (|QuestCheck
      (:then
        _)
      (:NotQuest
        _))
    (Variables|Game|SetInnerTimer (Variables|Game|GetInputTime))))

(fn ConstructionScript
  (bind _asbp_eject_symbol (Utilities|Casting|CastToBP_Eject_Symbol (Variables|/Script/Engine.ChildActorComponent|GetChildActor (Variables|Default|GetChildActor))))
  (Variables|/Game/Object/BP_Eject_Symbol.BP_Eject_Symbol_C|SetbForLight _asbp_eject_symbol (Variables|Game|GetForLight))
  (Transformation|SetActorRotation (Math|Rotator|MakeRotator 0.0 0.0 (Variables|Game|GetDegree)))
  (bind _output_get (Variables|Game|SetbClear (< (Math|Float|Absolute(Float) (Math|Rotator|NormalizeAxis (- (Variables|Game|GetDegree) (Variables|Game|GetAnswer)))) (Variables|Default|GetToleranceAmount))))
  (Rendering|SetVisibility (Variables|Default|GetParticleSystem) _output_get false))