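; BP_ResqueTriggerBox is an interactable trigger object that plays its assigned Sequence through the game state's multicast when interacted with.
; It then records its ID in the game state's progress WorldObjects and saves, and LoadState destroys the actor.
; The construction script generates a GUID when ID is empty, getters report interaction type, multi state and ID, and OffCollision disables its collision.
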(event Custom|OffCollision
  (Collision|SetCollisionEnabled (Variables|Default|GetCollisionComponent) "NoCollision"))

(event EventBeginPlay)

(event EventTick
  (params (DeltaSeconds :type Float%20%28single-precision%29)))

(event EventSaveState
  (bind _ascrafting_star_gs (Utilities|Casting|CastToCraftingStarGS (Game|GetGameState)))
  (Utilities|Array|AddUnique (.WorldObjects (Utilities|Struct|BreakProgressData (Variables|/Script/CraftingStar.CraftingStarGS|GetProgressData _ascrafting_star_gs))) (Variables|세이브|GetID))
  (Class|UtilityFunction|Save (Game|GetGameInstance)))

(event EventLoadState
  (Actor|DestroyActor))

(event EventOnInteraction
  (params (PlayerCharacter :type Crafting%20Star%20Character%20Object%20Reference))
  (bind _asbp_crafting_star_gs (Utilities|Casting|CastToBP_CraftingStarGS (Game|GetGameState)))
  (Default|MultiCastPlaySequence _asbp_crafting_star_gs (Variables|시퀀스재생|GetSequence))
  (CallFunction|SaveState))

(fn ConstructionScript
  (if (Utilities|Enum|Equal(Enum) (Variables|세이브|GetID) "")
    (Variables|세이브|SetID (Guid|ToString(Guid) (Guid|NewGuid)))))

(fn GetInteractionType
  (return "NewEnumerator5"))

(fn GetMultiState
  (return "NewEnumerator1"))

(fn GetObjectID
  (return (Variables|세이브|GetID)))