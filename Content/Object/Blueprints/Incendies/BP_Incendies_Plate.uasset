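; Incendies puzzle plate that ends a sequence of play once four linked trigger objects, apparently light rotation stones, are all active.
; BeginPlay prints a warning if any of the four references is unset.
; On authority, Tick polls their Active flags and has BP_CraftingStarGS multicast the Farewell sequence.
; No latch guards this, so the call repeats every tick while all four stay active.
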(event EventBeginPlay
  (Utilities|IsValid (Variables|Default|GetTriggerObject1)
    (:Is%20Valid
      (Utilities|IsValid (Variables|Default|GetTriggerObject2)
        (:Is%20Valid
          (Utilities|IsValid (Variables|Default|GetTriggerObject3)
            (:Is%20Valid
              (Utilities|IsValid (Variables|Default|GetTriggerObject4)
                (:Is%20Not%20Valid
                  _)))
            (:Is%20Not%20Valid
              _)))
        (:Is%20Not%20Valid
          _)))
    (:Is%20Not%20Valid
      _))
  (Development|PrintString "Need Light Rotation Stone "))

(event Collision|EventActorBeginOverlap
  (params (OtherActor :type Actor%20Object%20Reference)))

(event EventTick
  (params (DeltaSeconds :type Float%20%28single-precision%29))
  (Networking|SwitchHasAuthority
    (:Authority
      (if (Variables|/Game/Object/Blueprints/Incendies/BP_LightRotationStone.BP_LightRotationStone_C|GetbActive (Variables|Default|GetTriggerObject1))
        (if (Variables|/Game/Object/Blueprints/Incendies/BP_LightRotationStone.BP_LightRotationStone_C|GetbActive (Variables|Default|GetTriggerObject2))
          (if (Variables|/Game/Object/Blueprints/Incendies/BP_LightRotationStone.BP_LightRotationStone_C|GetbActive (Variables|Default|GetTriggerObject3))
            (if (Variables|/Game/Object/Blueprints/Incendies/BP_LightRotationStone.BP_LightRotationStone_C|GetbActive (Variables|Default|GetTriggerObject4))
              (Development|PrintString "End")
              (bind _asbp_crafting_star_gs (Utilities|Casting|CastToBP_CraftingStarGS (Game|GetGameState)))
              (Default|MultiCastPlaySequence _asbp_crafting_star_gs "/Game/Cinematics/Incendies/farewell.farewell"))))))))

(fn ConstructionScript)