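; BP_Key_F is an interactable key object that is picked up on interaction.
; Interacting casts the game state to BP_CraftingStarGS, multicasts the GetKey sequence, calls SaveState and destroys the actor.
; LoadState hides the static mesh, while SaveState has no logic in this graph.
; Overrides return fixed interaction type and multi-state enumerators and an empty object ID.
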(event EventOnInteraction
  (params (PlayerCharacter :type Crafting%20Star%20Character%20Object%20Reference))
  (bind _asbp_crafting_star_gs (Utilities|Casting|CastToBP_CraftingStarGS (Game|GetGameState)))
  (Default|MultiCastPlaySequence _asbp_crafting_star_gs "/Game/Cinematics/Incendies/GetKey.GetKey")
  (CallFunction|SaveState)
  (Actor|DestroyActor))

(event EventSaveState)

(event EventLoadState
  (Rendering|SetVisibility (Variables|Debug|GetStaticMeshComponent) false false))

(fn ConstructionScript)

(fn GetInteractionType
  (return "NewEnumerator4"))

(fn GetMultiState
  (return "NewEnumerator1"))

(fn GetObjectID
  (return ""))