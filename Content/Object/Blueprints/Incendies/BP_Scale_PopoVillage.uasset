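; Balance-scale puzzle actor for Popo Village that tilts by basket weight and fires a linked trigger when balanced.
; Basket overlaps sum BP_ScaleForObject1 weights per side; Tick tilts the beam within a limit, counter-rotating the cable-hung baskets.
; Equal weights ease it back and, once pitch drops below threshold, authority calls TriggerOn, sinks the scale on a timeline and destroys it.
; The Sample flag bypasses the one-time clear guard.
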(event OnComponentBeginOverlap(inBasketRight)
  (params (OverlappedComponent :type Primitive%20Component%20Object%20Reference) (OtherActor :type Actor%20Object%20Reference) (OtherComp :type Primitive%20Component%20Object%20Reference) (OtherBodyIndex :type Integer) (bFromSweep :type Boolean) (SweepResult :type Hit%20Result%20Structure%20%28by%20ref%29))
  (bind _asbp_scale_for_object_1 (Utilities|Casting|CastToBP_ScaleForObject1 OtherActor))
  (bind _object_weight (Default|GetWeight _asbp_scale_for_object_1))
  (bind _output_get (Variables|Puzzle|SetRightWeight (+ (Variables|Puzzle|GetRightWeight) _object_weight)))
  (Development|PrintString (Utilities|String|ToString(Integer) _output_get)))

(event OnComponentBeginOverlap(inBasketLeft)
  (params (OverlappedComponent :type Primitive%20Component%20Object%20Reference) (OtherActor :type Actor%20Object%20Reference) (OtherComp :type Primitive%20Component%20Object%20Reference) (OtherBodyIndex :type Integer) (bFromSweep :type Boolean) (SweepResult :type Hit%20Result%20Structure%20%28by%20ref%29))
  (bind _asbp_scale_for_object_1 (Utilities|Casting|CastToBP_ScaleForObject1 OtherActor))
  (bind _object_weight (Default|GetWeight _asbp_scale_for_object_1))
  (bind _output_get (Variables|Puzzle|SetLeftWeight (+ (Variables|Puzzle|GetLeftWeight) _object_weight)))
  (Development|PrintString (Utilities|String|ToString(Integer) _output_get))
  (Development|PrintString "Siiisisisisi"))

(event OnComponentEndOverlap(inBasketLeft)
  (params (OverlappedComponent :type Primitive%20Component%20Object%20Reference) (OtherActor :type Actor%20Object%20Reference) (OtherComp :type Primitive%20Component%20Object%20Reference) (OtherBodyIndex :type Integer))
  (bind _asbp_scale_for_object_1 (Utilities|Casting|CastToBP_ScaleForObject1 OtherActor))
  (bind _object_weight (Default|GetWeight _asbp_scale_for_object_1))
  (bind _output_get (Variables|Puzzle|SetLeftWeight (- (Variables|Puzzle|GetLeftWeight) _object_weight)))
  (Development|PrintString (Utilities|String|ToString(Integer) _output_get))
  (Development|PrintString "Aiiaiaiaiai"))

(event OnComponentEndOverlap(inBasketRight)
  (params (OverlappedComponent :type Primitive%20Component%20Object%20Reference) (OtherActor :type Actor%20Object%20Reference) (OtherComp :type Primitive%20Component%20Object%20Reference) (OtherBodyIndex :type Integer))
  (bind _asbp_scale_for_object_1 (Utilities|Casting|CastToBP_ScaleForObject1 OtherActor))
  (bind _object_weight (Default|GetWeight _asbp_scale_for_object_1))
  (bind _output_get (Variables|Puzzle|SetRightWeight (- (Variables|Puzzle|GetRightWeight) _object_weight)))
  (Development|PrintString (Utilities|String|ToString(Integer) _output_get)))

(event Custom|Perform
  (if (not (and (not (Variables|Default|GetbSample)) (Variables|Puzzle|GetbIsClear)))
    (Networking|SwitchHasAuthority
      (:Authority
        (Variables|Puzzle|SetbIsClear true)
        (bind _astriger_object (Utilities|Casting|CastToTrigerObject (Variables|Puzzle|GetTriggerObject)))
        (Default|Trigeron _astriger_object)
        (Variables|Default|SetActorLocation (Transformation|GetActorLocation))
        (bind _새_트랙_0 (Timeline|Down Play)
          (:Update
            (Transformation|SetActorLocation (Math|Vector|Lerp(Vector) (Variables|Default|GetActorLocation) (Math|Vector|MakeVector (.X (Math|Vector|BreakVector (Variables|Default|GetActorLocation))) (.Y (Math|Vector|BreakVector (Variables|Default|GetActorLocation))) (- (.Z (Math|Vector|BreakVector (Variables|Default|GetActorLocation))) 5e+02)) _새_트랙_0) false false))
          (:Finished
            (Actor|DestroyActor)))))))

(event EventBeginPlay
  (|AttachCableSocket))

(event Collision|EventActorBeginOverlap
  (params (OtherActor :type Actor%20Object%20Reference)))

(event EventTick
  (params (DeltaSeconds :type Float%20%28single-precision%29))
  (if (Variables|Default|GetbSample)
    (CallFunction|CheckScale :!label _label)
    (elif (not (Variables|Puzzle|GetbIsClear))
      (goto _label))))

(fn ConstructionScript
  (Class|CableComponent|SetAttachEndtoComponent (Variables|Default|GetCable) (Variables|Default|GetSM_SocketLeft) "EndPoint")
  (Class|CableComponent|SetAttachEndtoComponent (Variables|Default|GetCable2) (Variables|Default|GetSM_SocketRight) "EndPoint"))

(fn CheckScale
  (bind _rightweight (Variables|Puzzle|GetRightWeight))
  (bind _leftweight (Variables|Puzzle|GetLeftWeight))
  (if (== _leftweight _rightweight)
    (CallFunction|RestoreScale)
    (else
      (CallFunction|RotateScale (select (> _leftweight _rightweight) 0.1 -0.1)))))

(fn RotateScale
  (params (Rotate%20Amount :type Float%20%28single-precision%29))
  (bind _returnvalue (* Rotate%20Amount -1.0))
  (if (< (Math|Float|Absolute(Float) (.pitch (Variables|/Script/Engine.SceneComponent|GetRelativeRotation (Variables|Default|GetScaleRoot)))) 2e+01)
    (Transformation|AddLocalRotation (Variables|Default|GetScaleRoot) (Math|Rotator|MakeRotator 0.0 Rotate%20Amount 0.0) false false)
    (Transformation|AddLocalRotation (Variables|Default|GetBasketLeft) (Math|Rotator|MakeRotator _returnvalue 0.0 0.0) false false)
    (Transformation|AddLocalRotation (Variables|Default|GetBasketRight) (Math|Rotator|MakeRotator _returnvalue 0.0 0.0) false false)
    (else
      (return))))

(fn RestoreScale
  (bind _scaleroot (Variables|Default|GetScaleRoot))
  (bind _relativerotation (Variables|/Script/Engine.SceneComponent|GetRelativeRotation _scaleroot))
  (bind _returnvalue (Math|Float|Sign(Float) (.pitch _relativerotation)))
  (bind _returnvalue_2 (* _returnvalue -0.1))
  (bind _returnvalue_3 (* _returnvalue_2 -1.0))
  (Transformation|AddLocalRotation (Variables|Default|GetScaleRoot) (Math|Rotator|MakeRotator 0.0 _returnvalue_2 0.0) false false)
  (Transformation|AddLocalRotation (Variables|Default|GetBasketLeft) (Math|Rotator|MakeRotator _returnvalue_3 0.0 0.0) false false)
  (Transformation|AddLocalRotation (Variables|Default|GetBasketRight) (Math|Rotator|MakeRotator _returnvalue_3 0.0 0.0) false false)
  (if (< (.pitch (Variables|/Script/Engine.SceneComponent|GetRelativeRotation (Variables|Default|GetScaleRoot))) 0.1)
    (CallFunction|Perform))
  (return))