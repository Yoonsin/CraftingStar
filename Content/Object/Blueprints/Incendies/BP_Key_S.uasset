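; BP_Key_S is an interactable key object that advances game progress when used.
; On interaction it sets the progress level in the game state's ProgressData, saves through the crafting star game instance, then destroys itself.
; It reports a fixed interaction type and multi-state with an empty object ID, and its LoadState event is empty.
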(event EventOnInteraction
  (params (PlayerCharacter :type Crafting%20Star%20Character%20Object%20Reference))
  (bind _asbp_crafting_star_gs (Utilities|Casting|CastToBP_CraftingStarGS (Game|GetGameState)))
  (Utilities|Struct|SetmembersinProgressData (Variables|/Script/CraftingStar.CraftingStarGS|GetProgressData _asbp_crafting_star_gs) 1)
  (CallFunction|SaveState)
  (Actor|DestroyActor))

(event EventSaveState
  (bind _asbp_crafting_star_game_instance (Utilities|Casting|CastToBP_CraftingStarGameInstance (Game|GetGameInstance)))
  (Class|UtilityFunction|Save _asbp_crafting_star_game_instance))

(event EventLoadState)

(fn ConstructionScript)

(fn GetInteractionType
  (return "NewEnumerator4"))

(fn GetMultiState
  (return "NewEnumerator1"))

(fn GetObjectID
  (return ""))