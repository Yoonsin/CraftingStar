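; Guardian route actor that carries a controller's pawn along a spline and fires a trigger at the end.
; While IsOn, server-side Tick advances Distance by Speed and sets the pawn's transform directly from the spline, drawing a debug point.
; Nearing the last spline point within a small tolerance calls TrigerOn on TriggerObject once, guarded by IsEnded.
; An alternative that feeds the controller a Destination is left disconnected.
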(event EventBeginPlay)

(event Collision|EventActorBeginOverlap
  (params (OtherActor :type Actor%20Object%20Reference)))

(event EventTick
  (params (DeltaSeconds :type Float%20%28single-precision%29))
  (Networking|SwitchHasAuthority
    (:Authority
      (CallFunction|Moveon DeltaSeconds (Variables|Default|GetbIsOn)))))

(fn ConstructionScript)

(fn Moveon
  (params (Delta%20Sec :type Float%20%28single-precision%29) (Condition :type Boolean))
  (bind _spline (Variables|Default|GetSpline))
  (if Condition
    (bind _output_get (Variables|Default|SetDistance (+ (* Delta%20Sec (Variables|Default|GetSpeed)) (Variables|Default|GetDistance))))
    (Rendering|Debug|DrawDebugPoint (.Location (Math|Transform|BreakTransform (Spline|GetTransformatDistanceAlongSpline (Variables|Default|GetSpline) _output_get "World" false))) 5e+01 "(R=1.000000,G=0.000000,B=0.058562,A=1.000000)" 0.1)
    (Transformation|SetActorTransform (Pawn|GetControlledPawn (Variables|Default|GetGuadianController)) (Spline|GetTransformatDistanceAlongSpline (Variables|Default|GetSpline) _output_get "World" false))
    (if (and (Math|Float|NearlyEqual(Float) (Spline|GetDistanceAlongSplineatSplinePoint _spline (- (Spline|GetNumberOfSplinePoints _spline) 1)) (Variables|Default|GetDistance) 1e+01) (not (Variables|Default|GetbIsEnded)))
      ;[1 1 1] 이 부분에 Trigger
      (Development|PrintString "Spline ENd")
      (Variables|Default|SetbIsEnded true)
      (Default|Trigeron (Variables|Default|GetTrigger%20Object)))))