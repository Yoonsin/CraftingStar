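; Spawner actor that creates a BP_FlameGaudian AI at its own location when SpawnFrameGaudian is called.
; The spawned guardian is activated with this spawner's Route.
; It then receives as TriggerObject the first BP_SignInForest in the level whose object name contains "BP_SignInForest".
; BeginPlay, overlap and Tick are empty, so nothing in this Blueprint starts the spawn by itself.
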(event Custom|SpawnFrameGaudian
  (bind _returnvalue (AI|SpawnAIFromClass "/Game/NPC/Monster/Blueprint/BP_FlameGaudian.BP_FlameGaudian_C" 0 (Transformation|GetActorLocation) "0, 0, 0" false 0))
  (bind _asbp_flame_gaudian (Utilities|Casting|CastToBP_FlameGaudian _returnvalue))
  (Default|ActivateFlameGaudian _asbp_flame_gaudian (Variables|Default|GetRoute))
  (bind _outactors (Actor|GetAllActorsOfClass "/Game/Object/Blueprints/Incendies/BP_SignInForest.BP_SignInForest_C"))
  (bind _array_element (Utilities|Array|ForEachLoopwithBreak _outactors :!label _label)
    (:LoopBody
      (if (Utilities|String|Contains (Utilities|GetObjectName _array_element) "BP_SignInForest")
        (Variables|/Game/NPC/Monster/Blueprint/BP_FlameGaudian.BP_FlameGaudian_C|SetTrigger%20Object _asbp_flame_gaudian _array_element)
        (goto _label Break)))))

(event EventBeginPlay)

(event Collision|EventActorBeginOverlap
  (params (OtherActor :type Actor%20Object%20Reference)))

(event EventTick
  (params (DeltaSeconds :type Float%20%28single-precision%29)))

(fn ConstructionScript)