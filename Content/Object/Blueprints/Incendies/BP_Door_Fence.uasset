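; BP_Door_Fence is a fence door object that reports its interaction type and lock state through getter functions.
; It returns fixed enum values for interaction type and multi-state, passes through its IsLocked and LockMessage variables, and gives an empty object ID.
; IsLocked has an empty OnRep handler, and the event graph and construction script hold no logic, so no opening behavior is defined here.
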(event EventBeginPlay)

(event Collision|EventActorBeginOverlap
  (params (OtherActor :type Actor%20Object%20Reference)))

(event EventTick
  (params (DeltaSeconds :type Float%20%28single-precision%29)))

(fn ConstructionScript)

(fn OnRepIsLocked)

(fn GetInteractionType
  (return "NewEnumerator1"))

(fn GetIsLocked
  (return (Variables|Default|GetisLocked)))

(fn GetLockMessage
  (return (Variables|Default|GetlockMessage)))

(fn GetMultiState
  (return "NewEnumerator1"))

(fn GetObjectID
  (return ""))