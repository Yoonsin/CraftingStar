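; Interactable prison gate in Incendies that handles entering and leaving the Flame Guardian's prison.
; On interaction, IsInPrison selects which sequence the game state multicasts.
; The exit branch also finds the Brother Penguin Glacier NPC by object name, moves host and guest to either side of it and updates progress data for the Flame Guardian rescue quest.
; Interface getters expose interaction type, lock state and lock message.
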(event Collision|EventActorBeginOverlap
  (params (OtherActor :type Actor%20Object%20Reference)))

(event EventTick
  (params (DeltaSeconds :type Float%20%28single-precision%29)))

(event EventOnInteraction
  (params (PlayerCharacter :type Crafting%20Star%20Character%20Object%20Reference))
  (bind _asbp_crafting_star_gs (Utilities|Casting|CastToBP_CraftingStarGS (Game|GetGameState)))
  (if (Variables|문상호작용|GetisInPrison)
    ;[1 1 1] 감옥에 들어갈 때
    (Default|MultiCastPlaySequence _asbp_crafting_star_gs "/Game/Cinematics/Incendies/EnterFlameGuardianPrison.EnterFlameGuardianPrison")
    (else
      ;[1 1 1] 감옥에 나갈 때
      (Default|MultiCastPlaySequence _asbp_crafting_star_gs "/Game/Cinematics/Incendies/visitGLwithFlameGuardian.visitGLwithFlameGuardian")
      (bind _outactors (Actor|GetAllActorsOfClass "/Game/NPC/BP_NPC_Glacier.BP_NPC_Glacier_C"))
      (bind _array_element (Utilities|Array|ForEachLoopwithBreak _outactors)
        (:LoopBody
          (if (Utilities|String|Contains (Utilities|GetObjectName _array_element) "Brother_Penguin_C_PhysicsAsset")
            (Default|MoveCharacter _asbp_crafting_star_gs (Math|Transform|MakeTransform (+ (.location (Transformation|GetActorTransform _array_element)) "-150.000000, 0, 0") (.rotation (Transformation|GetActorTransform _array_element)) (.scale (Transformation|GetActorTransform _array_element))) (Math|Transform|MakeTransform (+ (.location (Transformation|GetActorTransform _array_element)) "150.000000, 0, 0") (.rotation (Transformation|GetActorTransform _array_element)) (.scale (Transformation|GetActorTransform _array_element))))
            (Utilities|Struct|SetmembersinProgressData (Variables|/Script/CraftingStar.CraftingStarGS|GetProgressData _asbp_crafting_star_gs) "EIncendieRescueFrameGuardian")))))))

(event EventBeginPlay)

(fn ConstructionScript)

(fn OnRepIsLocked)

(fn OnRepNewVar0)

(fn GetInteractionType
  (return "NewEnumerator1"))

(fn GetIsLocked
  (return (Variables|문상호작용|GetisLocked)))

(fn GetLockMessage
  (return (Variables|문상호작용|GetMessage)))

(fn GetMultiState
  (return "NewEnumerator1"))

(fn GetObjectID
  (return ""))