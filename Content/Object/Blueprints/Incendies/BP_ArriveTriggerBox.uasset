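; BP_ArriveTriggerBox is a server-authoritative overlap trigger that reacts when a flame guardian arrives.
; For the prison guardian, it unlocks the first prison gate door whose object name contains "prisonGate2".
; For the regular guardian, it sets the quest ID in the CraftingStar GameState's progress data to mark arrival at the forest's end, the Incendie rescue site.
; Both branches print a debug arrival message.
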(event EventBeginPlay)

(event Collision|EventActorBeginOverlap
  (params (OtherActor :type Actor%20Object%20Reference))
  (Networking|SwitchHasAuthority
    (:Authority
      (Utilities|Casting|CastToBP_FlameGuadian_InPrison OtherActor
        (:then
          (Development|PrintString "불꽃 수호자 도착")
          (bind _outactors (Actor|GetAllActorsOfClass "/Game/Object/Blueprints/Incendies/BP_Door_prisonGate.BP_Door_prisonGate_C"))
          (bind _array_element (Utilities|Array|ForEachLoopwithBreak _outactors :!label _label)
            (:LoopBody
              (if (Utilities|String|Contains (Utilities|GetObjectName _array_element) "prisonGate2")
                (Variables|/Game/Object/Blueprints/Incendies/BP_Door_prisonGate.BP_Door_prisonGate_C|SetisLocked _array_element false)
                (goto _label Break)))))
        (:CastFailed
          (Utilities|Casting|CastToBP_FlameGaudian OtherActor)
          (Development|PrintString "불꽃 수호자 도착" true true "(R=0.000000,G=0.660000,B=1.000000,A=1.000000)" 3e+01)
          ;[1 1 1] 앙상디 구출장소에 불꽃수호자 도착으로 퀘스트 ID 설정
          (bind _ascrafting_star_gs (Utilities|Casting|CastToCraftingStarGS (Game|GetGameState)))
          (Utilities|Struct|SetmembersinProgressData (Variables|/Script/CraftingStar.CraftingStarGS|GetProgressData _ascrafting_star_gs) "EIncendieArriveTheEndOfForest"))))))

(event EventTick
  (params (DeltaSeconds :type Float%20%28single-precision%29)))

(fn ConstructionScript)