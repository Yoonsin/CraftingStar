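; BP_DestroyPopo is an overlap trigger that removes the Popo character from the level once a specific village house door is unlocked.
; On any actor overlap, it searches all BP_Door_VillageHouse actors for one whose display name contains "BP_Door_VillageHouse_G" and checks its IsLocked flag.
; If that door is unlocked, it finds BP_Popo by the same name-matching technique, destroys it, then destroys itself.
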(event EventBeginPlay)

(event Collision|EventActorBeginOverlap
  (params (OtherActor :type Actor%20Object%20Reference))
  ;[1 1 1] 레벨의 잠긴 문 액터 찾기
  (bind _outactors (Actor|GetAllActorsOfClass "/Game/Object/Blueprints/Incendies/BP_Door_VillageHouse.BP_Door_VillageHouse_C"))
  (for _array_element _outactors
    (if (Utilities|String|Contains (Utilities|GetDisplayName _array_element) (Utilities|String|MakeLiteralString "BP_Door_VillageHouse_G"))
      ;[1 1 1] 문 열렸는지 확인
      (bind _asbp_door_village_house (Utilities|Casting|CastToBP_Door_VillageHouse _array_element))
      (if (not (Variables|/Game/Object/Blueprints/Incendies/BP_Door_VillageHouse.BP_Door_VillageHouse_C|GetbIsLocked _asbp_door_village_house))
        ;[1 1 1] 레벨의 포포 캐릭터 찾기
        (bind _outactors_2 (Actor|GetAllActorsOfClass "/Game/NPC/Monster/Blueprint/Popo/BP_Popo.BP_Popo_C"))
        (for _array_element_2 _outactors_2
          (if (Utilities|String|Contains (Utilities|GetDisplayName _array_element_2) (Utilities|String|MakeLiteralString "Popo"))
            ;[1 1 1] 포포 숨기기
            (bind _asbp_popo (Utilities|Casting|CastToBP_Popo _array_element_2))
            (bind _output_get (Variables|Default|SetPopoChar _asbp_popo))
            (Actor|DestroyActor _output_get)
            (Actor|DestroyActor)))))))

(event EventTick
  (params (DeltaSeconds :type Float%20%28single-precision%29)))

(fn ConstructionScript)