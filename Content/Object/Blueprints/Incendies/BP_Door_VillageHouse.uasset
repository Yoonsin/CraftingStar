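; BP_Door_VillageHouse is an interactable village house door that can be locked and toggles open or closed.
; When unlocked, OnInteraction plays a multicast sound and runs the DoorManage timeline forward or in reverse to rotate the door, saving state when it finishes.
; Trigeron clears the lock.
; The construction script assigns a GUID as the object ID if empty, exposed alongside interaction-type and multi-state getters.
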(event Custom|Server_PlayEffects
  (params (Sound :type Sound%20Base%20Object%20Reference) (Location :type Vector))
  ;[1 1 1] 음향 효과 리플리케이트
  (CallFunction|MulticastPlayEffects Sound Location))

(event Custom|Multicast_PlayEffects
  (params (Sound :type Sound%20Base%20Object%20Reference) (Location :type Vector))
  ;[1 1 1] 음향 효과 리플리케이트
  (Audio|PlaySoundatLocation Sound Location "0, 0, 0" 1.0 1.0 0.0 0 0 0))

(event EventTrigeron
  (Variables|Default|SetbIsLocked false))

(event EventOnInteraction
  (params (PlayerCharacter :type Crafting%20Star%20Character%20Object%20Reference))
  ;[1 1 1] 문이 잠겨있는지 확인
  (if (not (Variables|Default|GetbIsLocked))
    ;[1 1 1] 문 여는 소리 재생
    (CallFunction|MulticastPlayEffects "/Game/Assets/Sound/OpenDoor.OpenDoor" (Transformation|GetActorLocation))
    ;[1 1 1] 문이 열린 상태인지 확인
    (if (Variables|Default|GetbIsOpened)
      (Variables|Default|SetbIsOpened false)
      ;[1 1 1] 문 열기 타임라인 재생 후 저장
      (bind _새_트랙_0 (Timeline|DoorManage Reverse)
        (:Update
          (Transformation|SetRelativeRotation (Variables|Default|GetDoor) (Math|Rotator|Lerp(Rotator) "0, 0, 0" "0.000000,100.000000,0.000000" _새_트랙_0) false false))
        (:Finished
          (CallFunction|SaveState)))
      (else
        (Variables|Default|SetbIsOpened true)
        (Timeline|DoorManage Play)))))

(fn ConstructionScript
  (if (Utilities|Enum|Equal(Enum) (Variables|Default|GetID) "")
    (Variables|Default|SetID (Guid|ToString(Guid) (Guid|NewGuid)))))

(fn OnRepBIsLocked)

(fn GetInteractionType
  (return "NewEnumerator1"))

(fn GetMultiState
  (return "NewEnumerator1"))

(fn GetObjectID
  (return (Variables|Default|GetID)))